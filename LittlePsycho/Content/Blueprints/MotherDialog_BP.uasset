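; NPC dialog actor for a grieving mother's apparition, running a branching Polish conversation about her dying daughter.
; Overlap swaps the main character's input for a cursor-driven DialogInterface6 widget; leaving restores control.
; Three answer events share one nested-branch state machine, where HeaderIndex and ArrayIndex select the reply and next options from construction-script strings.
; Late choices adjust the player's Points and set moral flags, and the final choices close the dialog.
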(event `self.ReceiveActorBeginOverlap`
  (params (OtherActor :type "Actor Object Reference"))
  ;[1 1 1] Handle input and camera
  (bind _asmain_character (cast `MainCharacter` OtherActor))
  (bind _returnvalue (`self.setMainCharacter` _asmain_character))
  (bind _returnvalue_2 (`GameplayStatics.GetPlayerController` _returnvalue))
  (`self.DisableInput` _returnvalue _returnvalue_2)
  (bind _returnvalue_3 (`|CreateWidget` "/Game/Dialog/DialogInterface6.DialogInterface6_C" _returnvalue_2))
  (bind _output_get (set `self.DialogInterface` _returnvalue_3))
  (`TextBlock.SetText` (`/Game/Dialog/DialogInterface6.Text_Block_1` _output_get) (`self.Header Start`))
  (set `self.ButtonText` (select `int` (`self.ArrayIndex`) :`0` (`|MakeArray` (`self.Odp 0.1`) (`self.Odp 0.2`) (`self.Odp 0.3`)) :`1` (`|MakeArray` (`self.Odp 1.1`) (`self.Odp 1.2`) (`self.Odp 1.3`)) :`2` (`|MakeArray` (`self.Odp 3.1`) (`self.Odp 3.2`) (`self.Odp 3.3`)) :`3` (`|MakeArray` (`self.Odp 6.1`) (`self.Odp 6.2`) (`self.Odp 6.3`)) :`4` (`|MakeArray` (`self.Odp 10.1`) (`self.Odp 10.2`) (`self.Odp 10.3`)) :`5` (`|MakeArray` (`self.Odp 13.1`) (`self.Odp 13.2`) (`self.Odp 13.3`)) :`6` (`|MakeArray` (`self.Odp 14.1`) (`self.Odp 14.2`) (`self.Odp 14.3`))))
  (`UserWidget.AddToViewport` _output_get 0)
  (set `PlayerController.bShowMouseCursor` true _returnvalue_2))

(event `self.ReceiveActorEndOverlap`
  (params (OtherActor :type "Actor Object Reference"))
  (bind _returnvalue (`GameplayStatics.GetPlayerController` 0))
  ;[1 1 1] Handle input and camera
  (`Widget.RemoveFromParent` (`self.DialogInterface`) :!label _label)
  (bind _returnvalue_2 (`self.getMainCharacter`))
  (`self.EnableInput` _returnvalue_2 _returnvalue)
  (set `PlayerController.bShowMouseCursor` false _returnvalue))

(event `Leave`
  ;[1 1 1] Handle input and camera
  (`self.endDialog`)
  (goto _label))

(event `Answer1`
  (`self.setChosenNumber` 0)
  (if (== (`self.HeaderIndex`) 0) :!label _label_2
    (bind _returnvalue (`self.isDialogDataAccurate` 0))
    (if _returnvalue
      (bind _returnvalue_2 (`self.setHeaderIndex` 1))
      (set `self.HeaderIndex` _returnvalue_2)
      (bind _returnvalue_3 (`self.setArrayIndex` 1))
      (set `self.ArrayIndex` _returnvalue_3)
      (set `self.ButtonText` (select `int` (`self.ArrayIndex`) :`0` (`|MakeArray` (`self.Odp 0.1`) (`self.Odp 0.2`) (`self.Odp 0.3`)) :`1` (`|MakeArray` (`self.Odp 1.1`) (`self.Odp 1.2`) (`self.Odp 1.3`)) :`2` (`|MakeArray` (`self.Odp 3.1`) (`self.Odp 3.2`) (`self.Odp 3.3`)) :`3` (`|MakeArray` (`self.Odp 6.1`) (`self.Odp 6.2`) (`self.Odp 6.3`)) :`4` (`|MakeArray` (`self.Odp 10.1`) (`self.Odp 10.2`) (`self.Odp 10.3`)) :`5` (`|MakeArray` (`self.Odp 13.1`) (`self.Odp 13.2`) (`self.Odp 13.3`)) :`6` (`|MakeArray` (`self.Odp 14.1`) (`self.Odp 14.2`) (`self.Odp 14.3`))) :!label _label_3)
      (set `self.CurrentNPCResponse` (select `int` (`self.HeaderIndex`) :`0` (`self.Header Start`) :`1` (`self.Header 1`) :`2` (`self.Header 2`) :`3` (`self.Header 3`) :`4` (`self.Header 6`) :`5` (`self.Header 10`) :`6` (`self.Header 13`) :`7` (`self.Header 14`) :`8` (`self.Header 15`)))
      (else
        (bind _returnvalue_4 (`self.isDialogDataAccurate` 1))
        (if _returnvalue_4
          (bind _returnvalue_5 (`self.setHeaderIndex` 2))
          (set `self.HeaderIndex` _returnvalue_5)
          (bind _returnvalue_6 (`self.setArrayIndex` 1))
          (set `self.ArrayIndex` _returnvalue_6)
          (goto _label_3)
          (else
            (bind _returnvalue_7 (`self.isDialogDataAccurate` 2))
            (if _returnvalue_7
              (bind _returnvalue_8 (`self.setHeaderIndex` 3))
              (set `self.HeaderIndex` _returnvalue_8)
              (bind _returnvalue_9 (`self.setArrayIndex` 2))
              (set `self.ArrayIndex` _returnvalue_9)
              (goto _label_3))))))
    (elif (== (`self.HeaderIndex`) 1)
      (bind _returnvalue_10 (`self.isDialogDataAccurate` 0))
      (if _returnvalue_10
        (bind _returnvalue_11 (`self.setHeaderIndex` 4))
        (set `self.HeaderIndex` _returnvalue_11)
        (bind _returnvalue_12 (`self.setArrayIndex` 3))
        (set `self.ArrayIndex` _returnvalue_12)
        (goto _label_3)
        (else
          (bind _returnvalue_13 (`self.isDialogDataAccurate` 1))
          (if _returnvalue_13
            (bind _returnvalue_14 (`self.setHeaderIndex` 4))
            (set `self.HeaderIndex` _returnvalue_14)
            (bind _returnvalue_15 (`self.setArrayIndex` 3))
            (set `self.ArrayIndex` _returnvalue_15)
            (goto _label_3)
            (else
              (bind _returnvalue_16 (`self.isDialogDataAccurate` 2))
              (if _returnvalue_16
                (bind _returnvalue_17 (`self.setHeaderIndex` 4))
                (set `self.HeaderIndex` _returnvalue_17)
                (bind _returnvalue_18 (`self.setArrayIndex` 3))
                (set `self.ArrayIndex` _returnvalue_18)
                (goto _label_3))))))
      (elif (== (`self.HeaderIndex`) 2)
        (bind _returnvalue_19 (`self.isDialogDataAccurate` 0))
        (if _returnvalue_19
          (bind _returnvalue_20 (`self.setHeaderIndex` 4))
          (set `self.HeaderIndex` _returnvalue_20)
          (bind _returnvalue_21 (`self.setArrayIndex` 3))
          (set `self.ArrayIndex` _returnvalue_21)
          (goto _label_3)
          (else
            (bind _returnvalue_22 (`self.isDialogDataAccurate` 1))
            (if _returnvalue_22
              (bind _returnvalue_23 (`self.setHeaderIndex` 4))
              (set `self.HeaderIndex` _returnvalue_23)
              (bind _returnvalue_24 (`self.setArrayIndex` 3))
              (set `self.ArrayIndex` _returnvalue_24)
              (goto _label_3)
              (else
                (bind _returnvalue_25 (`self.isDialogDataAccurate` 2))
                (if _returnvalue_25
                  (bind _returnvalue_26 (`self.setHeaderIndex` 4))
                  (set `self.HeaderIndex` _returnvalue_26)
                  (bind _returnvalue_27 (`self.setArrayIndex` 3))
                  (set `self.ArrayIndex` _returnvalue_27)
                  (goto _label_3))))))
        (elif (== (`self.HeaderIndex`) 3)
          (bind _returnvalue_28 (`self.isDialogDataAccurate` 0))
          (if _returnvalue_28
            (bind _returnvalue_29 (`self.setHeaderIndex` 4))
            (set `self.HeaderIndex` _returnvalue_29)
            (bind _returnvalue_30 (`self.setArrayIndex` 3))
            (set `self.ArrayIndex` _returnvalue_30)
            (goto _label_3)
            (else
              (bind _returnvalue_31 (`self.isDialogDataAccurate` 1))
              (if _returnvalue_31
                (bind _returnvalue_32 (`self.setHeaderIndex` 4))
                (set `self.HeaderIndex` _returnvalue_32)
                (bind _returnvalue_33 (`self.setArrayIndex` 3))
                (set `self.ArrayIndex` _returnvalue_33)
                (goto _label_3)
                (else
                  (bind _returnvalue_34 (`self.isDialogDataAccurate` 2))
                  (if _returnvalue_34
                    (bind _returnvalue_35 (`self.setHeaderIndex` 4))
                    (set `self.HeaderIndex` _returnvalue_35)
                    (bind _returnvalue_36 (`self.setArrayIndex` 3))
                    (set `self.ArrayIndex` _returnvalue_36)
                    (goto _label_3))))))
          (elif (== (`self.HeaderIndex`) 4)
            (bind _returnvalue_37 (`self.isDialogDataAccurate` 0))
            (if _returnvalue_37
              (bind _returnvalue_38 (`self.setHeaderIndex` 5))
              (set `self.HeaderIndex` _returnvalue_38)
              (bind _returnvalue_39 (`self.setArrayIndex` 4))
              (set `self.ArrayIndex` _returnvalue_39)
              (goto _label_3)
              (else
                (bind _returnvalue_40 (`self.isDialogDataAccurate` 1))
                (if _returnvalue_40
                  (bind _returnvalue_41 (`self.setHeaderIndex` 5))
                  (set `self.HeaderIndex` _returnvalue_41)
                  (bind _returnvalue_42 (`self.setArrayIndex` 4))
                  (set `self.ArrayIndex` _returnvalue_42)
                  (goto _label_3)
                  (else
                    (bind _returnvalue_43 (`self.isDialogDataAccurate` 2))
                    (if _returnvalue_43
                      (bind _returnvalue_44 (`self.setHeaderIndex` 5))
                      (set `self.HeaderIndex` _returnvalue_44)
                      (bind _returnvalue_45 (`self.setArrayIndex` 4))
                      (set `self.ArrayIndex` _returnvalue_45)
                      (goto _label_3))))))
            (elif (== (`self.HeaderIndex`) 5)
              (bind _returnvalue_46 (`self.isDialogDataAccurate` 0))
              (if _returnvalue_46
                (bind _returnvalue_47 (`self.setHeaderIndex` 6))
                (set `self.HeaderIndex` _returnvalue_47)
                (bind _returnvalue_48 (`self.setArrayIndex` 5))
                (set `self.ArrayIndex` _returnvalue_48)
                (goto _label_3)
                (else
                  (bind _returnvalue_49 (`self.isDialogDataAccurate` 1))
                  (if _returnvalue_49
                    (bind _returnvalue_50 (`self.setHeaderIndex` 7))
                    (set `self.HeaderIndex` _returnvalue_50)
                    (bind _returnvalue_51 (`self.setArrayIndex` 6))
                    (set `self.ArrayIndex` _returnvalue_51)
                    (bind _returnvalue_52 (`self.getMainCharacter`))
                    (set `MainCharacter.bWontWasteTime` true _returnvalue_52)
                    (set `MainCharacter.Points` (- (`MainCharacter.Points` _returnvalue_52) 43) _returnvalue_52)
                    (goto _label_3)
                    (else
                      (bind _returnvalue_53 (`self.isDialogDataAccurate` 2))
                      (if _returnvalue_53
                        (bind _returnvalue_54 (`self.setHeaderIndex` 8))
                        (set `self.HeaderIndex` _returnvalue_54)
                        (bind _returnvalue_55 (`self.setArrayIndex` 5))
                        (set `self.ArrayIndex` _returnvalue_55)
                        (bind _returnvalue_56 (`self.getMainCharacter`))
                        (set `MainCharacter.bWantToHappy` true _returnvalue_56)
                        (set `MainCharacter.Points` (+ (`MainCharacter.Points` _returnvalue_56) 43) _returnvalue_56)
                        (goto _label_3))))))
              (elif (== (`self.HeaderIndex`) 6)
                (bind _returnvalue_57 (`self.isDialogDataAccurate` 0))
                (if _returnvalue_57
                  (`self.Leave`)
                  (else
                    (bind _returnvalue_58 (`self.isDialogDataAccurate` 1))
                    (if _returnvalue_58
                      (bind _returnvalue_59 (`self.getMainCharacter`))
                      (set `MainCharacter.bWantToAchievePurpose` true _returnvalue_59)
                      (set `MainCharacter.Points` (+ (`MainCharacter.Points` _returnvalue_59) 50) _returnvalue_59)
                      (`self.Leave`)
                      (else
                        (bind _returnvalue_60 (`self.isDialogDataAccurate` 2))
                        (if _returnvalue_60
                          (bind _returnvalue_61 (`self.getMainCharacter`))
                          (set `MainCharacter.Points` (- (`MainCharacter.Points` _returnvalue_61) 50) _returnvalue_61)
                          (set `MainCharacter.bWantToDie` true _returnvalue_61)
                          (`self.Leave`))))))
                (elif (== (`self.HeaderIndex`) 7)
                  (bind _returnvalue_62 (`self.isDialogDataAccurate` 0))
                  (if _returnvalue_62
                    (`self.Leave`)
                    (else
                      (bind _returnvalue_63 (`self.isDialogDataAccurate` 1))
                      (if _returnvalue_63
                        (bind _returnvalue_64 (`self.getMainCharacter`))
                        (set `MainCharacter.bWantToBeImportant` true _returnvalue_64)
                        (`self.Leave`)
                        (else
                          (bind _returnvalue_65 (`self.isDialogDataAccurate` 2))
                          (if _returnvalue_65
                            (`self.Leave`))))))
                  (elif (== (`self.HeaderIndex`) 8)
                    (bind _returnvalue_66 (`self.isDialogDataAccurate` 0))
                    (if _returnvalue_66
                      (`self.Leave`)
                      (else
                        (bind _returnvalue_67 (`self.isDialogDataAccurate` 1))
                        (if _returnvalue_67
                          (bind _returnvalue_68 (`self.getMainCharacter`))
                          (set `MainCharacter.bWantToAchievePurpose` true _returnvalue_68)
                          (set `MainCharacter.Points` (+ (`MainCharacter.Points` _returnvalue_68) 50) _returnvalue_68)
                          (`self.Leave`)
                          (else
                            (bind _returnvalue_69 (`self.isDialogDataAccurate` 2))
                            (if _returnvalue_69
                              (bind _returnvalue_70 (`self.getMainCharacter`))
                              (set `MainCharacter.Points` (- (`MainCharacter.Points` _returnvalue_70) 50) _returnvalue_70)
                              (set `MainCharacter.bWantToDie` true _returnvalue_70)
                              (`self.Leave`))))))))))))))))

(event `Answer2`
  (`self.setChosenNumber` 1)
  (goto _label_2))

(event `Answer3`
  (`self.setChosenNumber` 2)
  (goto _label_2))

(fn `UserConstructionScript`
  ;[1 1 1] Header Configuration
  (bind _output_get (set `self.Header Start` "Spójrz na mnie! Cała we krwi! Cała!"))
  (set `self.Header 1` "Pomóż! Pomóż!")
  (set `self.Header 2` "Odsuń się?! Odsuń?! Nie mów tak do mnie!")
  (set `self.Header 3` "Czemu? Co? Moje serce! Serce mi krwawi!")
  (set `self.Header 6` "Co byś zrobił, gdybyś musiał wybierać między swoim życiem, a życiem swojego dziecka?")
  (set `self.Header 10` "Ale nie w tym sensie! Wybrałbyś opiekę nad córką, o któej i tak wiesz, że umrze... Czy może wolałbyś skazać ją na śmierć i nie marnować swojego czasu?")
  (set `self.Header 13` "Widzisz jakie to ciężkie brzemię?! Widzisz?! A ona odchodzi! Muszę patrzeć, jak gaśnie coraz mocniej i mocniej. Aż zgaśnie całkowicie. Nawet nie wiesz! Opiekujesz się, pielęgnujesz, dbasz, cieszysz się z sukcesów i smucisz się z porażek... A ona ma czelność po prostu odejść!")
  (set `self.Header 14` "Okrutnik! Jak możesz! Jak?! Moja mała córeczka... Taka biedna, taka kochana! Musi odejść, musi!")
  (set `self.Header 15` "Ja też! Ja też!! Widzisz jakie to ciężkie brzemię?! Widzisz?! A ona odchodzi! Muszę patrzeć, jak gaśnie coraz mocniej i mocniej. Aż zgaśnie całkowicie. Nawet nie wiesz! Opiekujesz się, pielęgnujesz, dbasz, cieszysz się z sukcesów i smucisz się z porażek... A ona ma czelność po prostu odejść!")
  (set `self.CurrentNPCResponse` _output_get)
  ;[1 1 1] Dialog Data Configuration
  (set `self.Odp 0.1` "Mogę Ci jakoś pomóc?")
  (set `self.Odp 0.2` "Odsuń się, bo mnie ochlapiesz!")
  (set `self.Odp 0.3` "C-Co się stało?! Czemu krwawisz?")
  (set `self.Odp 1.1` "Jak się tu znalazłaś? Co się wydarzyło, że tak bardzo cierpisz?")
  (set `self.Odp 1.2` "Jesteś tylko zjawą, nic Ci nie jest")
  (set `self.Odp 1.3` "Jak Ci niby mam pomóc?")
  (set `self.Odp 3.1` "Czemu krwawi Ci serce?")
  (set `self.Odp 3.2` "Jesteś obłąkana!")
  (set `self.Odp 3.3` "Mogę Ci pomóc?")
  (set `self.Odp 6.1` "Wybrałbym siebie")
  (set `self.Odp 6.2` "Wybrałbym dziecko")
  (set `self.Odp 6.3` "Nie byłbym w stanie podjąć decyzji")
  (set `self.Odp 10.1` "Czemu pytasz mnie o takie rzeczy?")
  (set `self.Odp 10.2` "Wolałbym nie marnować swojego czasu")
  (set `self.Odp 10.3` "Wolałbym uszczęśliwić córkę, nawet jeśli żyłaby krótko")
  (set `self.Odp 13.1` "[Odsuń się i wymiń zjawę]")
  (set `self.Odp 13.2` "Jesteś obłąkana... [Odejdź]")
  (set `self.Odp 13.3` "Zawsze lepiej jest nie poświęcać się dla innych [Odejdź]")
  (set `self.Odp 14.1` "[Odsuń się i wymiń zjawę]")
  (set `self.Odp 14.2` "Jesteś obłąkana...[Odejdź]")
  (set `self.Odp 14.3` "Zawsze lepiej nie poświęcać się dla innych[Odejdź]")
  (set `self.HeaderIndex` 0)
  (set `self.ArrayIndex` 0))