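; Branching Polish dialogue for the father apparition, who judges the player's earlier choice about the sick rabbits.
; Overlap disables player input and shows a DialogInterface7 widget; Leave or end overlap removes it and restores input.
; Three Answer events share a nested branch chain that moves HeaderIndex and ArrayIndex, splitting on MainCharacter's KilledIll and LeaveAlone flags.
; Those indices select the NPC line and button texts defined in the Construction Script; final-stage answers call Leave.
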(event `self.ReceiveActorBeginOverlap`
  (params (OtherActor :type "Actor Object Reference"))
  ;[1 1 1] Handle input and camera
  (bind _asmain_character (cast `MainCharacter` OtherActor))
  (bind _returnvalue (`self.setMainCharacter` _asmain_character))
  (bind _returnvalue_2 (`GameplayStatics.GetPlayerController` _returnvalue))
  (`self.DisableInput` _returnvalue _returnvalue_2)
  (bind _returnvalue_3 (`|CreateWidget` "/Game/Dialog/DialogInterface7.DialogInterface7_C" _returnvalue_2))
  (bind _output_get (set `self.DialogInterface` _returnvalue_3))
  (`TextBlock.SetText` (`/Game/Dialog/DialogInterface7.Text_Block_1` _output_get) (`self.HeaderStart`))
  (set `self.ButtonText` (select `int` (`self.ArrayIndex`) :`0` (`|MakeArray` (`self.Odp0.1`) (`self.Odp0.2`) (`self.Odp0.3`)) :`1` (`|MakeArray` (`self.Odp1.1a`) (`self.Odp1.2a`) (`self.Odp1.3a`)) :`2` (`|MakeArray` (`self.Odp1.1b`) (`self.Odp1.2b`) (`self.Odp1.3b`)) :`3` (`|MakeArray` (`self.Odp1.1c`) (`self.Odp1.2c`) (`self.Odp1.3c`)) :`4` (`|MakeArray` (`self.Odp4.1a`) (`self.Odp4.2a`) (`self.Odp4.3a`)) :`5` (`|MakeArray` (`self.Odp4.1b`) (`self.Odp4.2b`) (`self.Odp4.3b`)) :`6` (`|MakeArray` (`self.Odp4.1c`) (`self.Odp4.2c`) (`self.Odp4.3c`))))
  (`UserWidget.AddToViewport` _output_get 0)
  (set `PlayerController.bShowMouseCursor` true _returnvalue_2))

(event `self.ReceiveActorEndOverlap`
  (params (OtherActor :type "Actor Object Reference"))
  (bind _returnvalue (`GameplayStatics.GetPlayerController` 0))
  ;[1 1 1] Handle input and camera
  (`Widget.RemoveFromParent` (`self.DialogInterface`) :!label _label)
  (bind _returnvalue_2 (`self.getMainCharacter`))
  (`self.EnableInput` _returnvalue_2 _returnvalue)
  (set `PlayerController.bShowMouseCursor` false _returnvalue))

(event `Leave`
  ;[1 1 1] Handle input and camera
  (`self.endDialog`)
  (goto _label))

(event `Answer1`
  (`self.setChosenNumber` 0)
  (if (== (`self.HeaderIndex`) 0) :!label _label_2
    (bind _returnvalue (`self.isDialogDataAccurate` 0))
    (if _returnvalue
      (bind _returnvalue_2 (`self.getMainCharacter`))
      (if (`MainCharacter.bKilledIll` _returnvalue_2)
        (bind _returnvalue_3 (`self.setHeaderIndex` 1))
        (set `self.HeaderIndex` _returnvalue_3)
        (bind _returnvalue_4 (`self.setArrayIndex` 1))
        (set `self.ArrayIndex` _returnvalue_4)
        (elif (`MainCharacter.bLeaveAlone` _returnvalue_2)
          (bind _returnvalue_5 (`self.setHeaderIndex` 4))
          (set `self.HeaderIndex` _returnvalue_5)
          (bind _returnvalue_6 (`self.setArrayIndex` 2))
          (set `self.ArrayIndex` _returnvalue_6)
          (else
            (bind _returnvalue_7 (`self.setHeaderIndex` 7))
            (set `self.HeaderIndex` _returnvalue_7)
            (bind _returnvalue_8 (`self.setArrayIndex` 3))
            (set `self.ArrayIndex` _returnvalue_8))))
      (set `self.ButtonText` (select `int` (`self.ArrayIndex`) :`0` (`|MakeArray` (`self.Odp0.1`) (`self.Odp0.2`) (`self.Odp0.3`)) :`1` (`|MakeArray` (`self.Odp1.1a`) (`self.Odp1.2a`) (`self.Odp1.3a`)) :`2` (`|MakeArray` (`self.Odp1.1b`) (`self.Odp1.2b`) (`self.Odp1.3b`)) :`3` (`|MakeArray` (`self.Odp1.1c`) (`self.Odp1.2c`) (`self.Odp1.3c`)) :`4` (`|MakeArray` (`self.Odp4.1a`) (`self.Odp4.2a`) (`self.Odp4.3a`)) :`5` (`|MakeArray` (`self.Odp4.1b`) (`self.Odp4.2b`) (`self.Odp4.3b`)) :`6` (`|MakeArray` (`self.Odp4.1c`) (`self.Odp4.2c`) (`self.Odp4.3c`))) :!label _label_3)
      (set `self.CurrentNPCResponse` (select `int` (`self.HeaderIndex`) :`0` (`self.HeaderStart`) :`1` (`self.Header1a`) :`2` (`self.Header2a`) :`3` (`self.Header3a`) :`4` (`self.Header 1b`) :`5` (`self.Header 2b`) :`6` (`self.Header 3b`) :`7` (`self.Header 1c`) :`8` (`self.Header 2c`) :`9` (`self.Header 3c`) :`10` (`self.Header4a`) :`11` (`self.Header5a`) :`12` (`self.Header6a`) :`13` (`self.Header4b`) :`14` (`self.Header5b`) :`15` (`self.Header6b`) :`16` (`self.Header4c`) :`17` (`self.Header5c`) :`18` (`self.Header6c`)))
      (else
        (bind _returnvalue_9 (`self.isDialogDataAccurate` 1))
        (if _returnvalue_9
          (bind _returnvalue_10 (`self.getMainCharacter`))
          (if (`MainCharacter.bKilledIll` _returnvalue_10)
            (bind _returnvalue_11 (`self.setHeaderIndex` 2))
            (set `self.HeaderIndex` _returnvalue_11)
            (bind _returnvalue_12 (`self.setArrayIndex` 1))
            (set `self.ArrayIndex` _returnvalue_12)
            (goto _label_3)
            (elif (`MainCharacter.bLeaveAlone` _returnvalue_10)
              (bind _returnvalue_13 (`self.setHeaderIndex` 5))
              (set `self.HeaderIndex` _returnvalue_13)
              (bind _returnvalue_14 (`self.setArrayIndex` 2))
              (set `self.ArrayIndex` _returnvalue_14)
              (goto _label_3)
              (else
                (bind _returnvalue_15 (`self.setHeaderIndex` 8))
                (set `self.HeaderIndex` _returnvalue_15)
                (bind _returnvalue_16 (`self.setArrayIndex` 3))
                (set `self.ArrayIndex` _returnvalue_16)
                (goto _label_3))))
          (else
            (bind _returnvalue_17 (`self.isDialogDataAccurate` 2))
            (if _returnvalue_17
              (bind _returnvalue_18 (`self.getMainCharacter`))
              (if (`MainCharacter.bKilledIll` _returnvalue_18)
                (bind _returnvalue_19 (`self.setHeaderIndex` 3))
                (set `self.HeaderIndex` _returnvalue_19)
                (bind _returnvalue_20 (`self.setArrayIndex` 1))
                (set `self.ArrayIndex` _returnvalue_20)
                (goto _label_3)
                (elif (`MainCharacter.bLeaveAlone` _returnvalue_18)
                  (bind _returnvalue_21 (`self.setHeaderIndex` 6))
                  (set `self.HeaderIndex` _returnvalue_21)
                  (bind _returnvalue_22 (`self.setArrayIndex` 2))
                  (set `self.ArrayIndex` _returnvalue_22)
                  (goto _label_3)
                  (else
                    (bind _returnvalue_23 (`self.setHeaderIndex` 9))
                    (set `self.HeaderIndex` _returnvalue_23)
                    (bind _returnvalue_24 (`self.setArrayIndex` 3))
                    (set `self.ArrayIndex` _returnvalue_24)
                    (goto _label_3)))))))))
    (elif (== (`self.HeaderIndex`) 1)
      (bind _returnvalue_25 (`self.isDialogDataAccurate` 0))
      (if _returnvalue_25
        (bind _returnvalue_26 (`self.setHeaderIndex` 10))
        (set `self.HeaderIndex` _returnvalue_26)
        (bind _returnvalue_27 (`self.setArrayIndex` 4))
        (set `self.ArrayIndex` _returnvalue_27)
        (goto _label_3)
        (else
          (bind _returnvalue_28 (`self.isDialogDataAccurate` 1))
          (if _returnvalue_28
            (bind _returnvalue_29 (`self.setHeaderIndex` 11))
            (set `self.HeaderIndex` _returnvalue_29)
            (bind _returnvalue_30 (`self.setArrayIndex` 4))
            (set `self.ArrayIndex` _returnvalue_30)
            (goto _label_3)
            (else
              (bind _returnvalue_31 (`self.isDialogDataAccurate` 2))
              (if _returnvalue_31
                (bind _returnvalue_32 (`self.setHeaderIndex` 12))
                (set `self.HeaderIndex` _returnvalue_32)
                (bind _returnvalue_33 (`self.setArrayIndex` 4))
                (set `self.ArrayIndex` _returnvalue_33)
                (goto _label_3))))))
      (elif (== (`self.HeaderIndex`) 2)
        (bind _returnvalue_34 (`self.isDialogDataAccurate` 0))
        (if _returnvalue_34
          (bind _returnvalue_35 (`self.setHeaderIndex` 10))
          (set `self.HeaderIndex` _returnvalue_35)
          (bind _returnvalue_36 (`self.setArrayIndex` 4))
          (set `self.ArrayIndex` _returnvalue_36)
          (goto _label_3)
          (else
            (bind _returnvalue_37 (`self.isDialogDataAccurate` 1))
            (if _returnvalue_37
              (bind _returnvalue_38 (`self.setHeaderIndex` 11))
              (set `self.HeaderIndex` _returnvalue_38)
              (bind _returnvalue_39 (`self.setArrayIndex` 4))
              (set `self.ArrayIndex` _returnvalue_39)
              (goto _label_3)
              (else
                (bind _returnvalue_40 (`self.isDialogDataAccurate` 2))
                (if _returnvalue_40
                  (bind _returnvalue_41 (`self.setHeaderIndex` 12))
                  (set `self.HeaderIndex` _returnvalue_41)
                  (bind _returnvalue_42 (`self.setArrayIndex` 4))
                  (set `self.ArrayIndex` _returnvalue_42)
                  (goto _label_3))))))
        (elif (== (`self.HeaderIndex`) 3)
          (bind _returnvalue_43 (`self.isDialogDataAccurate` 0))
          (if _returnvalue_43
            (bind _returnvalue_44 (`self.setHeaderIndex` 10))
            (set `self.HeaderIndex` _returnvalue_44)
            (bind _returnvalue_45 (`self.setArrayIndex` 4))
            (set `self.ArrayIndex` _returnvalue_45)
            (goto _label_3)
            (else
              (bind _returnvalue_46 (`self.isDialogDataAccurate` 1))
              (if _returnvalue_46
                (bind _returnvalue_47 (`self.setHeaderIndex` 11))
                (set `self.HeaderIndex` _returnvalue_47)
                (bind _returnvalue_48 (`self.setArrayIndex` 4))
                (set `self.ArrayIndex` _returnvalue_48)
                (goto _label_3)
                (else
                  (bind _returnvalue_49 (`self.isDialogDataAccurate` 2))
                  (if _returnvalue_49
                    (bind _returnvalue_50 (`self.setHeaderIndex` 12))
                    (set `self.HeaderIndex` _returnvalue_50)
                    (bind _returnvalue_51 (`self.setArrayIndex` 4))
                    (set `self.ArrayIndex` _returnvalue_51)
                    (goto _label_3))))))
          (elif (== (`self.HeaderIndex`) 4)
            (bind _returnvalue_52 (`self.isDialogDataAccurate` 0))
            (if _returnvalue_52
              (bind _returnvalue_53 (`self.setHeaderIndex` 13))
              (set `self.HeaderIndex` _returnvalue_53)
              (bind _returnvalue_54 (`self.setArrayIndex` 5))
              (set `self.ArrayIndex` _returnvalue_54)
              (goto _label_3)
              (else
                (bind _returnvalue_55 (`self.isDialogDataAccurate` 1))
                (if _returnvalue_55
                  (bind _returnvalue_56 (`self.setHeaderIndex` 14))
                  (set `self.HeaderIndex` _returnvalue_56)
                  (bind _returnvalue_57 (`self.setArrayIndex` 5))
                  (set `self.ArrayIndex` _returnvalue_57)
                  (goto _label_3)
                  (else
                    (bind _returnvalue_58 (`self.isDialogDataAccurate` 2))
                    (if _returnvalue_58
                      (bind _returnvalue_59 (`self.setHeaderIndex` 15))
                      (set `self.HeaderIndex` _returnvalue_59)
                      (bind _returnvalue_60 (`self.setArrayIndex` 5))
                      (set `self.ArrayIndex` _returnvalue_60)
                      (goto _label_3))))))
            (elif (== (`self.HeaderIndex`) 5)
              (bind _returnvalue_61 (`self.isDialogDataAccurate` 0))
              (if _returnvalue_61
                (bind _returnvalue_62 (`self.setHeaderIndex` 13))
                (set `self.HeaderIndex` _returnvalue_62)
                (bind _returnvalue_63 (`self.setArrayIndex` 5))
                (set `self.ArrayIndex` _returnvalue_63)
                (goto _label_3)
                (else
                  (bind _returnvalue_64 (`self.isDialogDataAccurate` 1))
                  (if _returnvalue_64
                    (bind _returnvalue_65 (`self.setHeaderIndex` 14))
                    (set `self.HeaderIndex` _returnvalue_65)
                    (bind _returnvalue_66 (`self.setArrayIndex` 5))
                    (set `self.ArrayIndex` _returnvalue_66)
                    (goto _label_3)
                    (else
                      (bind _returnvalue_67 (`self.isDialogDataAccurate` 2))
                      (if _returnvalue_67
                        (bind _returnvalue_68 (`self.setHeaderIndex` 15))
                        (set `self.HeaderIndex` _returnvalue_68)
                        (bind _returnvalue_69 (`self.setArrayIndex` 5))
                        (set `self.ArrayIndex` _returnvalue_69)
                        (goto _label_3))))))
              (elif (== (`self.HeaderIndex`) 6)
                (bind _returnvalue_70 (`self.isDialogDataAccurate` 0))
                (if _returnvalue_70
                  (bind _returnvalue_71 (`self.setHeaderIndex` 13))
                  (set `self.HeaderIndex` _returnvalue_71)
                  (bind _returnvalue_72 (`self.setArrayIndex` 5))
                  (set `self.ArrayIndex` _returnvalue_72)
                  (goto _label_3)
                  (else
                    (bind _returnvalue_73 (`self.isDialogDataAccurate` 1))
                    (if _returnvalue_73
                      (bind _returnvalue_74 (`self.setHeaderIndex` 14))
                      (set `self.HeaderIndex` _returnvalue_74)
                      (bind _returnvalue_75 (`self.setArrayIndex` 5))
                      (set `self.ArrayIndex` _returnvalue_75)
                      (goto _label_3)
                      (else
                        (bind _returnvalue_76 (`self.isDialogDataAccurate` 2))
                        (if _returnvalue_76
                          (bind _returnvalue_77 (`self.setHeaderIndex` 15))
                          (set `self.HeaderIndex` _returnvalue_77)
                          (bind _returnvalue_78 (`self.setArrayIndex` 5))
                          (set `self.ArrayIndex` _returnvalue_78)
                          (goto _label_3))))))
                (elif (== (`self.HeaderIndex`) 7)
                  (bind _returnvalue_79 (`self.isDialogDataAccurate` 0))
                  (if _returnvalue_79
                    (bind _returnvalue_80 (`self.setHeaderIndex` 16))
                    (set `self.HeaderIndex` _returnvalue_80)
                    (bind _returnvalue_81 (`self.setArrayIndex` 6))
                    (set `self.ArrayIndex` _returnvalue_81)
                    (goto _label_3)
                    (else
                      (bind _returnvalue_82 (`self.isDialogDataAccurate` 1))
                      (if _returnvalue_82
                        (bind _returnvalue_83 (`self.setHeaderIndex` 17))
                        (set `self.HeaderIndex` _returnvalue_83)
                        (bind _returnvalue_84 (`self.setArrayIndex` 6))
                        (set `self.ArrayIndex` _returnvalue_84)
                        (goto _label_3)
                        (else
                          (bind _returnvalue_85 (`self.isDialogDataAccurate` 2))
                          (if _returnvalue_85
                            (bind _returnvalue_86 (`self.setHeaderIndex` 18))
                            (set `self.HeaderIndex` _returnvalue_86)
                            (bind _returnvalue_87 (`self.setArrayIndex` 6))
                            (set `self.ArrayIndex` _returnvalue_87)
                            (goto _label_3))))))
                  (elif (== (`self.HeaderIndex`) 8)
                    (bind _returnvalue_88 (`self.isDialogDataAccurate` 0))
                    (if _returnvalue_88
                      (bind _returnvalue_89 (`self.setHeaderIndex` 16))
                      (set `self.HeaderIndex` _returnvalue_89)
                      (bind _returnvalue_90 (`self.setArrayIndex` 6))
                      (set `self.ArrayIndex` _returnvalue_90)
                      (goto _label_3)
                      (else
                        (bind _returnvalue_91 (`self.isDialogDataAccurate` 1))
                        (if _returnvalue_91
                          (bind _returnvalue_92 (`self.setHeaderIndex` 17))
                          (set `self.HeaderIndex` _returnvalue_92)
                          (bind _returnvalue_93 (`self.setArrayIndex` 6))
                          (set `self.ArrayIndex` _returnvalue_93)
                          (goto _label_3)
                          (else
                            (bind _returnvalue_94 (`self.isDialogDataAccurate` 2))
                            (if _returnvalue_94
                              (bind _returnvalue_95 (`self.setHeaderIndex` 18))
                              (set `self.HeaderIndex` _returnvalue_95)
                              (bind _returnvalue_96 (`self.setArrayIndex` 6))
                              (set `self.ArrayIndex` _returnvalue_96)
                              (goto _label_3))))))
                    (elif (== (`self.HeaderIndex`) 9)
                      (bind _returnvalue_97 (`self.isDialogDataAccurate` 0))
                      (if _returnvalue_97
                        (bind _returnvalue_98 (`self.setHeaderIndex` 16))
                        (set `self.HeaderIndex` _returnvalue_98)
                        (bind _returnvalue_99 (`self.setArrayIndex` 6))
                        (set `self.ArrayIndex` _returnvalue_99)
                        (goto _label_3)
                        (else
                          (bind _returnvalue_100 (`self.isDialogDataAccurate` 1))
                          (if _returnvalue_100
                            (bind _returnvalue_101 (`self.setHeaderIndex` 17))
                            (set `self.HeaderIndex` _returnvalue_101)
                            (bind _returnvalue_102 (`self.setArrayIndex` 6))
                            (set `self.ArrayIndex` _returnvalue_102)
                            (goto _label_3)
                            (else
                              (bind _returnvalue_103 (`self.isDialogDataAccurate` 2))
                              (if _returnvalue_103
                                (bind _returnvalue_104 (`self.setHeaderIndex` 18))
                                (set `self.HeaderIndex` _returnvalue_104)
                                (bind _returnvalue_105 (`self.setArrayIndex` 6))
                                (set `self.ArrayIndex` _returnvalue_105)
                                (goto _label_3))))))
                      (elif (== (`self.HeaderIndex`) 10)
                        (bind _returnvalue_106 (`self.isDialogDataAccurate` 0))
                        (if _returnvalue_106
                          (`self.Leave`)
                          (else
                            (bind _returnvalue_107 (`self.isDialogDataAccurate` 1))
                            (if _returnvalue_107
                              (`self.Leave`)
                              (else
                                (bind _returnvalue_108 (`self.isDialogDataAccurate` 2))
                                (if _returnvalue_108
                                  (`self.Leave`))))))
                        (elif (== (`self.HeaderIndex`) 11)
                          (bind _returnvalue_109 (`self.isDialogDataAccurate` 0))
                          (if _returnvalue_109
                            (`self.Leave`)
                            (else
                              (bind _returnvalue_110 (`self.isDialogDataAccurate` 1))
                              (if _returnvalue_110
                                (`self.Leave`)
                                (else
                                  (bind _returnvalue_111 (`self.isDialogDataAccurate` 2))
                                  (if _returnvalue_111
                                    (`self.Leave`))))))
                          (elif (== (`self.HeaderIndex`) 12)
                            (bind _returnvalue_112 (`self.isDialogDataAccurate` 0))
                            (if _returnvalue_112
                              (`self.Leave`)
                              (else
                                (bind _returnvalue_113 (`self.isDialogDataAccurate` 1))
                                (if _returnvalue_113
                                  (`self.Leave`)
                                  (else
                                    (bind _returnvalue_114 (`self.isDialogDataAccurate` 2))
                                    (if _returnvalue_114
                                      (`self.Leave`))))))
                            (elif (== (`self.HeaderIndex`) 13)
                              (bind _returnvalue_115 (`self.isDialogDataAccurate` 0))
                              (if _returnvalue_115
                                (`self.Leave`)
                                (else
                                  (bind _returnvalue_116 (`self.isDialogDataAccurate` 1))
                                  (if _returnvalue_116
                                    (`self.Leave`)
                                    (else
                                      (bind _returnvalue_117 (`self.isDialogDataAccurate` 2))
                                      (if _returnvalue_117
                                        (`self.Leave`))))))
                              (elif (== (`self.HeaderIndex`) 14)
                                (bind _returnvalue_118 (`self.isDialogDataAccurate` 0))
                                (if _returnvalue_118
                                  (`self.Leave`)
                                  (else
                                    (bind _returnvalue_119 (`self.isDialogDataAccurate` 1))
                                    (if _returnvalue_119
                                      (`self.Leave`)
                                      (else
                                        (bind _returnvalue_120 (`self.isDialogDataAccurate` 2))
                                        (if _returnvalue_120
                                          (`self.Leave`))))))
                                (elif (== (`self.HeaderIndex`) 15)
                                  (bind _returnvalue_121 (`self.isDialogDataAccurate` 0))
                                  (if _returnvalue_121
                                    (`self.Leave`)
                                    (else
                                      (bind _returnvalue_122 (`self.isDialogDataAccurate` 1))
                                      (if _returnvalue_122
                                        (`self.Leave`)
                                        (else
                                          (bind _returnvalue_123 (`self.isDialogDataAccurate` 2))
                                          (if _returnvalue_123
                                            (`self.Leave`))))))
                                  (elif (== (`self.HeaderIndex`) 16)
                                    (bind _returnvalue_124 (`self.isDialogDataAccurate` 0))
                                    (if _returnvalue_124
                                      (`self.Leave`)
                                      (else
                                        (bind _returnvalue_125 (`self.isDialogDataAccurate` 1))
                                        (if _returnvalue_125
                                          (`self.Leave`)
                                          (else
                                            (bind _returnvalue_126 (`self.isDialogDataAccurate` 2))
                                            (if _returnvalue_126
                                              (`self.Leave`))))))
                                    (elif (== (`self.HeaderIndex`) 17)
                                      (bind _returnvalue_127 (`self.isDialogDataAccurate` 0))
                                      (if _returnvalue_127
                                        (`self.Leave`)
                                        (else
                                          (bind _returnvalue_128 (`self.isDialogDataAccurate` 1))
                                          (if _returnvalue_128
                                            (`self.Leave`)
                                            (else
                                              (bind _returnvalue_129 (`self.isDialogDataAccurate` 2))
                                              (if _returnvalue_129
                                                (`self.Leave`))))))
                                      (elif (== (`self.HeaderIndex`) 18)
                                        (bind _returnvalue_130 (`self.isDialogDataAccurate` 0))
                                        (if _returnvalue_130
                                          (`self.Leave`)
                                          (else
                                            (bind _returnvalue_131 (`self.isDialogDataAccurate` 1))
                                            (if _returnvalue_131
                                              (`self.Leave`)
                                              (else
                                                (bind _returnvalue_132 (`self.isDialogDataAccurate` 2))
                                                (if _returnvalue_132
                                                  (`self.Leave`))))))))))))))))))))))))))

(event `Answer2`
  (`self.setChosenNumber` 1)
  (goto _label_2))

(event `Answer3`
  (`self.setChosenNumber` 2)
  (goto _label_2))

(fn `UserConstructionScript`
  ;[1 1 1] Header Configuration
  (bind _output_get (set `self.HeaderStart` "Och, to Ty... Jestem kolejną próbą."))
  (set `self.Header1a` "Na pytaniu. Chcę zrozumieć. Dlaczego zabiłeś chore króliki?")
  (set `self.Header2a` "Tak... I nie. Wszyscy Cię widzą, obserwują. Dlaczego zabiłeś chore króliki?")
  (set `self.Header3a` "Dlaczego zabiłeś chore króliki?")
  (set `self.Header 1b` "Na pytaniu. Chcę zrozumieć. Dlaczego skazałeś na śmierć wszystkie króliki?")
  (set `self.Header 2b` "Tak... I nie. Wszyscy Cię widzą, obserwują. Dlaczego skazałeś na śmierć wszystkie króliki?")
  (set `self.Header 3b` "Dlaczego skazałeś na śmierć wszystkie króliki?")
  (set `self.Header 1c` "Na pytaniu. Chcę zrozumieć. Dlaczego przekonałeś opiekuna, by jednak zajął się podopiecznymi?")
  (set `self.Header 2c` "Tak... I nie. Wszyscy Cię widzą, obserwują. Dlaczego przekonałeś opiekuna, by jednak zajął się podopiecznymi?")
  (set `self.Header 3c` "Dlaczego przekonałeś opiekuna, by jednak zajął się podopiecznymi?")
  (set `self.Header4a` "Niewątpliwie, jednakże musiało istnieć jakieś inne rozwiązanie tego problemu. Zawiodłem się, synu.")
  (set `self.Header5a` "To nie sen! Ten wybór miał wpływ na nasz świat. Synu, zawiodłem się Tobą jeszcze bardziej.")
  (set `self.Header6a` "Nie wiesz, czy by umarły. Poszedłeś na skróty. Zawiodłem się, synu.")
  (set `self.Header4b` "Mogłeś zrobić cokolwiek. Bezczynność jest najgorsza. Zawiodłem się, synu.")
  (set `self.Header5b` "To nie nauczka! Straciły życie istoty z krwi i kości. Nie wzrusza Cię to?")
  (set `self.Header6b` "To nie sen! Ten wybór miał wpływ na nasz świat. Synu, zawodzę się Tobą coraz bardziej.")
  (set `self.Header4c` "To prawda. Postąpiłeś słusznie.")
  (set `self.Header5c` "A zatem jesteś na wskroś dobry. Dobrze, bardzo mi się to podoba.")
  (set `self.Header6c` "I było najlepsze. Efektów nie zobaczysz, ale zaufaj mi, postąpiłeś słusznie.")
  (set `self.CurrentNPCResponse` _output_get)
  ;[1 1 1] Dialog Data Configuration
  (set `self.Odp0.1` "I... na czym polega ta próba?")
  (set `self.Odp0.2` "Spotkaliśmy się już, że jesteś taki niechętny?")
  (set `self.Odp0.3` "Jestem gotowy na twoją próbę.")
  (set `self.Odp1.1a` "Stwarzały zagrożenie dla reszty stada.")
  (set `self.Odp1.2a` "To tylko sen, czemu miałbym się nimi przejmować?")
  (set `self.Odp1.3a` "I tak by umarły, skróciłem ich cierpienia.")
  (set `self.Odp1.1b` "Właścicielka nie chciała podjąć żadnych działań, więc ja również ich nie podjąłem.")
  (set `self.Odp1.2b` "Właścicielka ma nauczkę, by w przyszłości podejmować działania.")
  (set `self.Odp1.3b` "To tylko sen, czemu miałbym się nimi przejmować?")
  (set `self.Odp1.1c` "Nie musiały umierać. Wystarczyło tylko poświęcić im trochę czasu.")
  (set `self.Odp1.2c` "Doradziłem, by zrobić to, co sam bym zrobił w takiej sytuacji.")
  (set `self.Odp1.3c` "Wydawało mi się, że to najlepsze rozwiązanie. Nie byłbym w stanie odebrać komuś życia.")
  (set `self.Odp4.1a` "Musiało czy nie, obrałem taką drogę [Odejdź]")
  (set `self.Odp4.2a` "[Przebiegnij przez zjawę]")
  (set `self.Odp4.3a` "Próbujesz mi tylko namącić w głowie, jak reszta zjaw. [Odejdź]")
  (set `self.Odp4.1b` "Może i najgorsza, ale według mnie nie powinienem się mieszać .[Odejdź]")
  (set `self.Odp4.2b` "To nie była bezczynność, tylko nauka na przyszłość. [Odejdź]")
  (set `self.Odp4.3b` "Ty również mnie wiele razy zawiodłeś, ale nie słuchałeś. [Odejdź]")
  (set `self.Odp4.1c` "Dziękuję. [Odejdź]")
  (set `self.Odp4.2c` "[Odejdź]")
  (set `self.Odp4.3c` "[Przebiegnij przez zjawę]")
  (set `self.HeaderIndex` 0)
  (set `self.ArrayIndex` 0))