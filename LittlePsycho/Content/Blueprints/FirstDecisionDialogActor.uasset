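; Overlap-triggered NPC dialog actor that runs a branching first-decision conversation with the player.
; On overlap it shows a DialogInterface2 widget with cursor and input, and resets and removes it on exit.
; Answer events branch on a state index (UpdateArray) to set the NPC line and next reply texts.
; Final choices may set MainCharacter's FlowersWasTaken or ForcedToTakeCare flags, then close and destroy the actor.
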(event `self.ReceiveActorBeginOverlap`
  (params (OtherActor :type "Actor Object Reference"))
  ;[1 1 1] begin and end overlap
  (`self.EnableInput` (`GameplayStatics.GetPlayerController` 0))
  (bind _returnvalue (`|CreateWidget` "/Game/Dialog/DialogInterface2.DialogInterface2_C" (`GameplayStatics.GetPlayerController` 0)))
  (bind _output_get (set `self.DialogInterface` _returnvalue))
  (bind _output_get_2 (set `self.CurrentNPCResponse` (`self.Start`)))
  (`TextBlock.SetText` (`/Game/Dialog/DialogInterface2.Text_Block_1` _output_get) _output_get_2)
  (`UserWidget.AddToViewport` (`self.DialogInterface`) 0)
  (set `PlayerController.bShowMouseCursor` true (`GameplayStatics.GetPlayerController` 0))
  (set `self.ButtonText` (`|MakeArray` (`self.Question 0 - 1`) (`self.Question 0 - 2`) (`self.Question 0 - 3`))))

(event `self.ReceiveActorEndOverlap`
  (params (OtherActor :type "Actor Object Reference"))
  ;[1 1 1] begin and end overlap
  (`self.DisableInput` (`GameplayStatics.GetPlayerController` 0) :!label _label)
  (bind _output_get (set `self.CurrentNPCResponse` (`self.End`)))
  (`TextBlock.SetText` (`/Game/Dialog/DialogInterface2.Text_Block_1` (stale `self.ReceiveActorBeginOverlap` _output_get)) _output_get)
  (set `self.UpdateArray` 0)
  (`Widget.RemoveFromParent` (`self.DialogInterface`))
  (set `PlayerController.bShowMouseCursor` false (`GameplayStatics.GetPlayerController` 0)))

(event `Leaving`
  ;[1 1 1] begin and end overlap
  (goto _label))

(event `Answer1`
  (bind _int (`self.int`))
  (bind _int_2 (`self.int`))
  (bind _int_3 (`self.int`))
  (bind _int_4 (`self.int`))
  (bind _int_5 (`self.int`))
  (bind _int_6 (`self.int`))
  (bind _int_7 (`self.int`))
  (bind _int_8 (`self.int`))
  (bind _text_block_1 (`/Game/Dialog/DialogInterface2.Text_Block_1` (`self.DialogInterface`)))
  ;[1 1 1] Answers Setup
  (set `self.int` 0)
  (if (== (`self.UpdateArray`) 0) :!label _label_2
    (if (== _int_7 0)
      (bind _output_get (set `self.CurrentNPCResponse` (`self.NPC0-1`)))
      (`TextBlock.SetText` (`/Game/Dialog/DialogInterface2.Text_Block_1` (`self.DialogInterface`)) _output_get)
      (set `self.UpdateArray` 1)
      (bind _asmain_character (cast `MainCharacter` (`GameplayStatics.GetPlayerPawn` 0)))
      (set `self.ButtonText` (select `int` (`self.UpdateArray`) :`0` (`|MakeArray` (`self.Question 0 - 1`) (`self.Question 0 - 2`) (`self.Question 0 - 3`)) :`1` (`|MakeArray` (`self.Question 1- 1`) (`self.Question 1- 2`) (`self.Question 1 - 3`)) :`2` (`|MakeArray` (`self.Question 2 - 1`) (`self.Question 2 - 2`) (`self.Question 2 - 3`)) :`3` (`|MakeArray` (`self.Question 3 - 1`) (`self.Question 3 - 2`) (`self.Question 3 - 3`)) :`4` (`|MakeArray` (`self.Question 4 - 1`) (`self.Question 4 - 2`) (`self.Question 4 - 3`)) :`5` (`|MakeArray` (`self.Question 5 - 1`) (`self.Question 5 -2`) (`self.Question 5 - 3`)) :`6` (`|MakeArray` (`self.Question 6 - 1`) (`self.Question 6 - 2`) (`self.Question 6 - 3`)) :`7` (`|MakeArray` (`self.Question 7 - 1`) (`self.Question 7 - 2`) (`self.Question 7 - 3`)) :`8` (`|MakeArray` (`self.Question 8 - 1`) (`self.Question 8 - 2`) (`self.Question 8 - 3`)) :`9` (`|MakeArray` (`self.Question 9 - 1`) (`self.Question 9 - 2`) (`self.Question 9 - 3`))) :!label _label_3)
      (elif (== _int_7 1)
        (bind _output_get_2 (set `self.CurrentNPCResponse` (`self.NPC0-2`)))
        (`TextBlock.SetText` (`/Game/Dialog/DialogInterface2.Text_Block_1` (`self.DialogInterface`)) _output_get_2)
        (set `self.UpdateArray` 4)
        (bind _asmain_character_2 (cast `MainCharacter` (`GameplayStatics.GetPlayerPawn` 0)))
        (goto _label_3)
        (elif (== _int_7 2)
          (bind _output_get_3 (set `self.CurrentNPCResponse` (`self.NPC0-1`)))
          (`TextBlock.SetText` (`/Game/Dialog/DialogInterface2.Text_Block_1` (`self.DialogInterface`)) _output_get_3)
          (set `self.UpdateArray` 1)
          (goto _label_3))))
    (elif (== (`self.UpdateArray`) 1)
      (if (== _int_8 0)
        (bind _output_get_4 (set `self.CurrentNPCResponse` (`self.npc04`)))
        (`TextBlock.SetText` (`/Game/Dialog/DialogInterface2.Text_Block_1` (`self.DialogInterface`)) _output_get_4)
        (set `self.UpdateArray` 1)
        (goto _label_3)
        (elif (== _int_8 1)
          (bind _output_get_5 (set `self.CurrentNPCResponse` (`self.npc05`)))
          (`TextBlock.SetText` (`/Game/Dialog/DialogInterface2.Text_Block_1` (`self.DialogInterface`)) _output_get_5)
          (set `self.UpdateArray` 4)
          (goto _label_3)
          (elif (== _int_8 2)
            (bind _output_get_6 (set `self.CurrentNPCResponse` (`self.npc06`)))
            (`TextBlock.SetText` (`/Game/Dialog/DialogInterface2.Text_Block_1` (`self.DialogInterface`)) _output_get_6)
            (set `self.UpdateArray` 6)
            (goto _label_3))))
      (elif (== (`self.UpdateArray`) 2)
        (if (== _int_2 0)
          (bind _output_get_7 (set `self.CurrentNPCResponse` (`self.npc7`)))
          (`TextBlock.SetText` (`/Game/Dialog/DialogInterface2.Text_Block_1` (`self.DialogInterface`)) _output_get_7)
          (set `self.UpdateArray` 7)
          (goto _label_3)
          (elif (== _int_2 1)
            (bind _output_get_8 (set `self.CurrentNPCResponse` (`self.npc8`)))
            (`TextBlock.SetText` (`/Game/Dialog/DialogInterface2.Text_Block_1` (`self.DialogInterface`)) _output_get_8)
            (set `self.UpdateArray` 8)
            (goto _label_3)
            (elif (== _int_2 2)
              (bind _output_get_9 (set `self.CurrentNPCResponse` (`self.npc9`)))
              (`TextBlock.SetText` (`/Game/Dialog/DialogInterface2.Text_Block_1` (`self.DialogInterface`)) _output_get_9)
              (set `self.UpdateArray` 9)
              (goto _label_3))))
        (elif (== (`self.UpdateArray`) 3)
          _
          (elif (== (`self.UpdateArray`) 4)
            (if (== _int 0)
              (`TextBlock.SetText` _text_block_1 "Jesteś pewny? To według Ciebie jedyne wyjście? Może to da się rozwiązać inaczej?")
              (set `self.UpdateArray` 9)
              (goto _label_3)
              (elif (== _int 1)
                (`TextBlock.SetText` _text_block_1 "Więc co proponujesz? ")
                (set `self.UpdateArray` 8)
                (goto _label_3)
                (elif (== _int 2)
                  (`TextBlock.SetText` _text_block_1 "To dodatkowy czas, który muszę poświęcić na opiekę nad nimi. Muszę pójść, zająć się nimi, wrócić i dopilnować reszty stada, by nie dopadła ich zaraza. To bardzo ciężka praca.")
                  (set `self.UpdateArray` 7)
                  (goto _label_3))))
            (elif (== (`self.UpdateArray`) 5)
              _
              (elif (== (`self.UpdateArray`) 6)
                (if (== _int_3 0)
                  (bind _asmain_character_3 (cast `MainCharacter` (`GameplayStatics.GetPlayerPawn` 0)))
                  (set `MainCharacter.bFlowersWasTaken` true _asmain_character_3)
                  (`self.Leaving`)
                  (`self.K2_DestroyActor`)
                  (elif (== _int_3 1)
                    (bind _asmain_character_4 (cast `MainCharacter` (`GameplayStatics.GetPlayerPawn` 0)))
                    (set `MainCharacter.bForcedToTakeCare` true _asmain_character_4)
                    (`self.Leaving`)
                    (`self.K2_DestroyActor`)
                    (elif (== _int_3 2)
                      (bind _asmain_character_5 (cast `MainCharacter` (`GameplayStatics.GetPlayerPawn` 0)))
                      (`self.Leaving`)
                      (`self.K2_DestroyActor`))))
                (elif (== (`self.UpdateArray`) 7)
                  (if (== _int_6 0)
                    (bind _asmain_character_6 (cast `MainCharacter` (`GameplayStatics.GetPlayerPawn` 0)))
                    (set `MainCharacter.bForcedToTakeCare` true _asmain_character_6)
                    (`self.Leaving`)
                    (`self.K2_DestroyActor`)
                    (elif (== _int_6 1)
                      (bind _asmain_character_7 (cast `MainCharacter` (`GameplayStatics.GetPlayerPawn` 0)))
                      (set `MainCharacter.bFlowersWasTaken` true _asmain_character_7)
                      (`self.Leaving`)
                      (`self.K2_DestroyActor`)
                      (elif (== _int_6 2)
                        (bind _asmain_character_8 (cast `MainCharacter` (`GameplayStatics.GetPlayerPawn` 0)))
                        (`self.Leaving`)
                        (`self.K2_DestroyActor`))))
                  (elif (== (`self.UpdateArray`) 8)
                    (if (== _int_5 0)
                      (bind _asmain_character_9 (cast `MainCharacter` (`GameplayStatics.GetPlayerPawn` 0)))
                      (set `MainCharacter.bFlowersWasTaken` true _asmain_character_9)
                      (`self.Leaving`)
                      (`self.K2_DestroyActor`)
                      (elif (== _int_5 1)
                        (bind _asmain_character_10 (cast `MainCharacter` (`GameplayStatics.GetPlayerPawn` 0)))
                        (`self.Leaving`)
                        (`self.K2_DestroyActor`)
                        (elif (== _int_5 2)
                          (bind _asmain_character_11 (cast `MainCharacter` (`GameplayStatics.GetPlayerPawn` 0)))
                          (`self.Leaving`)
                          (`self.K2_DestroyActor`))))
                    (elif (== (`self.UpdateArray`) 9)
                      (if (== _int_4 0)
                        (bind _asmain_character_12 (cast `MainCharacter` (`GameplayStatics.GetPlayerPawn` 0)))
                        (`self.Leaving`)
                        (`self.K2_DestroyActor`)
                        (elif (== _int_4 1)
                          (bind _asmain_character_13 (cast `MainCharacter` (`GameplayStatics.GetPlayerPawn` 0)))
                          (`self.Leaving`)
                          (`self.K2_DestroyActor`)
                          (elif (== _int_4 2)
                            (bind _asmain_character_14 (cast `MainCharacter` (`GameplayStatics.GetPlayerPawn` 0)))
                            (set `MainCharacter.bFlowersWasTaken` true _asmain_character_14)
                            (`self.Leaving`)
                            (`self.K2_DestroyActor`)))))))))))))))

(event `Answer2`
  ;[1 1 1] Answers Setup
  (set `self.int` 1)
  (goto _label_2))

(event `Answer3`
  ;[1 1 1] Answers Setup
  (set `self.int` 2)
  (goto _label_2))

(event `Answer4`
  ;[1 1 1] Answers Setup
  (`self.Leaving`)
  (`self.K2_DestroyActor`))

(fn `UserConstructionScript`)