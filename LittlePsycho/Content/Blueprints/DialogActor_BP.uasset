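; Trigger actor for a branching Polish conversation with a ghostly Dreamland guardian, who explains the trials for saving the player's sister.
; Overlap disables player input and opens a three-answer DialogInterface widget with mouse cursor.
; Answers feed a hardcoded nested-branch state machine on HeaderIndex, selecting the NPC line and reply set from text defined in the Construction Script.
; Certain choices set character flags or adjust Points; leaving restores input and removes the widget.
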(event `self.ReceiveActorBeginOverlap`
  (params (OtherActor :type "Actor Object Reference"))
  ;[1 1 1] Handle input and camera
  (bind _asmain_character (cast `MainCharacter` OtherActor))
  (bind _returnvalue (`self.setMainCharacter` _asmain_character))
  (bind _returnvalue_2 (`GameplayStatics.GetPlayerController` _returnvalue))
  (`self.DisableInput` _returnvalue _returnvalue_2)
  (bind _output_get (set `self.ButtonText` (`|MakeArray` (`self.Odp0.1`) (`self.Odp0.2`) (`self.Odp0.3`))))
  (bind _returnvalue_3 (`|CreateWidget` "/Game/Dialog/DialogInterface.DialogInterface_C" _returnvalue_2))
  (bind _output_get_2 (set `self.DialogInterface` _returnvalue_3))
  (`TextBlock.SetText` (`/Game/Dialog/DialogInterface.TextBlock_1` _output_get_2) (`KismetArrayLibrary.Array_Get` _output_get))
  (`TextBlock.SetText` (`/Game/Dialog/DialogInterface.TextBlock_2` _output_get_2) (`KismetArrayLibrary.Array_Get` _output_get 1))
  (`TextBlock.SetText` (`/Game/Dialog/DialogInterface.TextBlock_3` _output_get_2) (`KismetArrayLibrary.Array_Get` _output_get 2))
  (`UserWidget.AddToViewport` _output_get_2 0)
  (set `PlayerController.bShowMouseCursor` true _returnvalue_2))

(event `self.ReceiveActorEndOverlap`
  (params (OtherActor :type "Actor Object Reference"))
  (bind _returnvalue (`GameplayStatics.GetPlayerController` 0))
  ;[1 1 1] Handle input and camera
  (`Widget.RemoveFromParent` (`self.DialogInterface`) :!label _label)
  (bind _returnvalue_2 (`self.getMainCharacter`))
  (`self.EnableInput` _returnvalue_2 _returnvalue)
  (set `PlayerController.bShowMouseCursor` false _returnvalue))

(event `Leave`
  ;[1 1 1] Handle input and camera
  (`self.endDialog`)
  (goto _label))

(event `Answer1`
  (`self.setChosenNumber` 0)
  (if (== (`self.HeaderIndex`) 0) :!label _label_2
    (bind _returnvalue (`self.isDialogDataAccurate` 0))
    (if _returnvalue
      (bind _returnvalue_2 (`self.setHeaderIndex` 1))
      (set `self.HeaderIndex` _returnvalue_2)
      (bind _returnvalue_3 (`self.setArrayIndex` 1))
      (set `self.ArrayIndex` _returnvalue_3)
      (set `self.ButtonText` (select `int` (`self.ArrayIndex`) :`0` (`|MakeArray` (`self.Odp0.1`) (`self.Odp0.2`) (`self.Odp0.3`)) :`1` (`|MakeArray` (`self.Odp1.1`) (`self.Odp1.2`) (`self.Odp1.3`)) :`2` (`|MakeArray` (`self.Odp2.1`) (`self.Odp2.2`) (`self.Odp2.3`)) :`3` (`|MakeArray` (`self.Odp3.1`) (`self.Odp3.2`) (`self.Odp3.3`)) :`4` (`|MakeArray` (`self.Odp4.1`) (`self.Odp4.2`) (`self.Odp4.3`)) :`5` (`|MakeArray` (`self.Odp6.1`) (`self.Odp6.2`) (`self.Odp6.3`)) :`6` (`|MakeArray` (`self.Odp11.1`) (`self.Odp11.2`) (`self.Odp11.3`)) :`7` (`|MakeArray` (`self.Odp13.1`) (`self.Odp13.2`) (`self.Odp13.3`)) :`8` (`|MakeArray` (`self.Odp16.1`) (`self.Odp16.2`) (`self.Odp16.3`))) :!label _label_3)
      (set `self.CurrentNPCResponse` (select `int` (`self.HeaderIndex`) :`0` (`self.HeaderStart`) :`1` (`self.Header1`) :`2` (`self.Header2`) :`3` (`self.Header3`) :`4` (`self.Header4`) :`5` (`self.Header5`) :`6` (`self.Header6`) :`7` (`self.Header7`) :`8` (`self.Header8`) :`9` (`self.Header11`) :`10` (`self.Header13`) :`11` (`self.Header16`) :`12` (`self.Header18`) :`13` (`self.Header22`)))
      (else
        (bind _returnvalue_4 (`self.isDialogDataAccurate` 1))
        (if _returnvalue_4
          (bind _returnvalue_5 (`self.setHeaderIndex` 2))
          (set `self.HeaderIndex` _returnvalue_5)
          (bind _returnvalue_6 (`self.setArrayIndex` 2))
          (set `self.ArrayIndex` _returnvalue_6)
          (goto _label_3)
          (else
            (bind _returnvalue_7 (`self.isDialogDataAccurate` 2))
            (if _returnvalue_7
              (bind _returnvalue_8 (`self.setHeaderIndex` 3))
              (set `self.HeaderIndex` _returnvalue_8)
              (bind _returnvalue_9 (`self.setArrayIndex` 3))
              (set `self.ArrayIndex` _returnvalue_9)
              (goto _label_3))))))
    (elif (== (`self.HeaderIndex`) 1)
      (bind _returnvalue_10 (`self.isDialogDataAccurate` 0))
      (if _returnvalue_10
        (bind _returnvalue_11 (`self.setHeaderIndex` 8))
        (set `self.HeaderIndex` _returnvalue_11)
        (bind _returnvalue_12 (`self.setArrayIndex` 4))
        (set `self.ArrayIndex` _returnvalue_12)
        (goto _label_3)
        (else
          (bind _returnvalue_13 (`self.isDialogDataAccurate` 1))
          (if _returnvalue_13
            (bind _returnvalue_14 (`self.setHeaderIndex` 9))
            (set `self.HeaderIndex` _returnvalue_14)
            (bind _returnvalue_15 (`self.setArrayIndex` 6))
            (set `self.ArrayIndex` _returnvalue_15)
            (goto _label_3)
            (else
              (bind _returnvalue_16 (`self.isDialogDataAccurate` 2))
              (if _returnvalue_16
                (bind _returnvalue_17 (`self.setHeaderIndex` 7))
                (set `self.HeaderIndex` _returnvalue_17)
                (bind _returnvalue_18 (`self.setArrayIndex` 4))
                (set `self.ArrayIndex` _returnvalue_18)
                (goto _label_3))))))
      (elif (== (`self.HeaderIndex`) 2)
        (bind _returnvalue_19 (`self.isDialogDataAccurate` 0))
        (if _returnvalue_19
          (bind _returnvalue_20 (`self.setHeaderIndex` 6))
          (set `self.HeaderIndex` _returnvalue_20)
          (bind _returnvalue_21 (`self.setArrayIndex` 5))
          (set `self.ArrayIndex` _returnvalue_21)
          (goto _label_3)
          (else
            (bind _returnvalue_22 (`self.isDialogDataAccurate` 1))
            (if _returnvalue_22
              (bind _returnvalue_23 (`self.setHeaderIndex` 8))
              (set `self.HeaderIndex` _returnvalue_23)
              (bind _returnvalue_24 (`self.setArrayIndex` 4))
              (set `self.ArrayIndex` _returnvalue_24)
              (goto _label_3)
              (else
                (bind _returnvalue_25 (`self.isDialogDataAccurate` 2))
                (if _returnvalue_25
                  (bind _returnvalue_26 (`self.setHeaderIndex` 7))
                  (set `self.HeaderIndex` _returnvalue_26)
                  (bind _returnvalue_27 (`self.setArrayIndex` 4))
                  (set `self.ArrayIndex` _returnvalue_27)
                  (goto _label_3))))))
        (elif (== (`self.HeaderIndex`) 3)
          (bind _returnvalue_28 (`self.isDialogDataAccurate` 0))
          (if _returnvalue_28
            (bind _returnvalue_29 (`self.setHeaderIndex` 4))
            (set `self.HeaderIndex` _returnvalue_29)
            (bind _returnvalue_30 (`self.setArrayIndex` 4))
            (set `self.ArrayIndex` _returnvalue_30)
            (goto _label_3)
            (else
              (bind _returnvalue_31 (`self.isDialogDataAccurate` 1))
              (if _returnvalue_31
                (bind _returnvalue_32 (`self.setHeaderIndex` 5))
                (set `self.HeaderIndex` _returnvalue_32)
                (bind _returnvalue_33 (`self.setArrayIndex` 4))
                (set `self.ArrayIndex` _returnvalue_33)
                (goto _label_3)
                (else
                  (bind _returnvalue_34 (`self.isDialogDataAccurate` 2))
                  (if _returnvalue_34
                    (bind _returnvalue_35 (`self.setHeaderIndex` 6))
                    (set `self.HeaderIndex` _returnvalue_35)
                    (bind _returnvalue_36 (`self.setArrayIndex` 5))
                    (set `self.ArrayIndex` _returnvalue_36)
                    (goto _label_3))))))
          (elif (== (`self.HeaderIndex`) 4)
            (bind _returnvalue_37 (`self.isDialogDataAccurate` 0))
            (if _returnvalue_37
              (bind _returnvalue_38 (`self.setHeaderIndex` 10))
              (set `self.HeaderIndex` _returnvalue_38)
              (bind _returnvalue_39 (`self.setArrayIndex` 7))
              (set `self.ArrayIndex` _returnvalue_39)
              (goto _label_3)
              (else
                (bind _returnvalue_40 (`self.isDialogDataAccurate` 1))
                (if _returnvalue_40
                  (bind _returnvalue_41 (`self.setHeaderIndex` 10))
                  (set `self.HeaderIndex` _returnvalue_41)
                  (bind _returnvalue_42 (`self.setArrayIndex` 7))
                  (set `self.ArrayIndex` _returnvalue_42)
                  (goto _label_3)
                  (else
                    (bind _returnvalue_43 (`self.isDialogDataAccurate` 2))
                    (if _returnvalue_43
                      (bind _returnvalue_44 (`self.setHeaderIndex` 10))
                      (set `self.HeaderIndex` _returnvalue_44)
                      (bind _returnvalue_45 (`self.setArrayIndex` 7))
                      (set `self.ArrayIndex` _returnvalue_45)
                      (goto _label_3))))))
            (elif (== (`self.HeaderIndex`) 5)
              (bind _returnvalue_46 (`self.isDialogDataAccurate` 0))
              (if _returnvalue_46
                (bind _returnvalue_47 (`self.setHeaderIndex` 10))
                (set `self.HeaderIndex` _returnvalue_47)
                (bind _returnvalue_48 (`self.setArrayIndex` 7))
                (set `self.ArrayIndex` _returnvalue_48)
                (goto _label_3)
                (else
                  (bind _returnvalue_49 (`self.isDialogDataAccurate` 1))
                  (if _returnvalue_49
                    (bind _returnvalue_50 (`self.setHeaderIndex` 10))
                    (set `self.HeaderIndex` _returnvalue_50)
                    (bind _returnvalue_51 (`self.setArrayIndex` 7))
                    (set `self.ArrayIndex` _returnvalue_51)
                    (goto _label_3)
                    (else
                      (bind _returnvalue_52 (`self.isDialogDataAccurate` 2))
                      (if _returnvalue_52
                        (bind _returnvalue_53 (`self.setHeaderIndex` 10))
                        (set `self.HeaderIndex` _returnvalue_53)
                        (bind _returnvalue_54 (`self.setArrayIndex` 7))
                        (set `self.ArrayIndex` _returnvalue_54)
                        (goto _label_3))))))
              (elif (== (`self.HeaderIndex`) 6)
                (bind _returnvalue_55 (`self.isDialogDataAccurate` 0))
                (if _returnvalue_55
                  (bind _returnvalue_56 (`self.setHeaderIndex` 8))
                  (set `self.HeaderIndex` _returnvalue_56)
                  (bind _returnvalue_57 (`self.setArrayIndex` 4))
                  (set `self.ArrayIndex` _returnvalue_57)
                  (goto _label_3)
                  (else
                    (bind _returnvalue_58 (`self.isDialogDataAccurate` 1))
                    (if _returnvalue_58
                      (bind _returnvalue_59 (`self.setHeaderIndex` 12))
                      (set `self.HeaderIndex` _returnvalue_59)
                      (bind _returnvalue_60 (`self.setArrayIndex` 4))
                      (set `self.ArrayIndex` _returnvalue_60)
                      (bind _returnvalue_61 (`self.getMainCharacter`))
                      (set `MainCharacter.bWasCurious` true _returnvalue_61)
                      (goto _label_3)
                      (else
                        (bind _returnvalue_62 (`self.isDialogDataAccurate` 2))
                        (if _returnvalue_62
                          (bind _returnvalue_63 (`self.setHeaderIndex` 4))
                          (set `self.HeaderIndex` _returnvalue_63)
                          (bind _returnvalue_64 (`self.setArrayIndex` 4))
                          (set `self.ArrayIndex` _returnvalue_64)
                          (goto _label_3))))))
                (elif (== (`self.HeaderIndex`) 7)
                  (bind _returnvalue_65 (`self.isDialogDataAccurate` 0))
                  (if _returnvalue_65
                    (bind _returnvalue_66 (`self.setHeaderIndex` 10))
                    (set `self.HeaderIndex` _returnvalue_66)
                    (bind _returnvalue_67 (`self.setArrayIndex` 7))
                    (set `self.ArrayIndex` _returnvalue_67)
                    (goto _label_3)
                    (else
                      (bind _returnvalue_68 (`self.isDialogDataAccurate` 1))
                      (if _returnvalue_68
                        (bind _returnvalue_69 (`self.setHeaderIndex` 10))
                        (set `self.HeaderIndex` _returnvalue_69)
                        (bind _returnvalue_70 (`self.setArrayIndex` 7))
                        (set `self.ArrayIndex` _returnvalue_70)
                        (goto _label_3)
                        (else
                          (bind _returnvalue_71 (`self.isDialogDataAccurate` 2))
                          (if _returnvalue_71
                            (bind _returnvalue_72 (`self.setHeaderIndex` 10))
                            (set `self.HeaderIndex` _returnvalue_72)
                            (bind _returnvalue_73 (`self.setArrayIndex` 7))
                            (set `self.ArrayIndex` _returnvalue_73)
                            (goto _label_3))))))
                  (elif (== (`self.HeaderIndex`) 8)
                    (bind _returnvalue_74 (`self.isDialogDataAccurate` 0))
                    (if _returnvalue_74
                      (bind _returnvalue_75 (`self.setHeaderIndex` 10))
                      (set `self.HeaderIndex` _returnvalue_75)
                      (bind _returnvalue_76 (`self.setArrayIndex` 7))
                      (set `self.ArrayIndex` _returnvalue_76)
                      (goto _label_3)
                      (else
                        (bind _returnvalue_77 (`self.isDialogDataAccurate` 1))
                        (if _returnvalue_77
                          (bind _returnvalue_78 (`self.setHeaderIndex` 10))
                          (set `self.HeaderIndex` _returnvalue_78)
                          (bind _returnvalue_79 (`self.setArrayIndex` 7))
                          (set `self.ArrayIndex` _returnvalue_79)
                          (goto _label_3)
                          (else
                            (bind _returnvalue_80 (`self.isDialogDataAccurate` 2))
                            (if _returnvalue_80
                              (bind _returnvalue_81 (`self.setHeaderIndex` 10))
                              (set `self.HeaderIndex` _returnvalue_81)
                              (bind _returnvalue_82 (`self.setArrayIndex` 7))
                              (set `self.ArrayIndex` _returnvalue_82)
                              (goto _label_3))))))
                    (elif (== (`self.HeaderIndex`) 9)
                      (bind _returnvalue_83 (`self.isDialogDataAccurate` 0))
                      (if _returnvalue_83
                        (bind _returnvalue_84 (`self.setHeaderIndex` 13))
                        (set `self.HeaderIndex` _returnvalue_84)
                        (bind _returnvalue_85 (`self.setArrayIndex` 4))
                        (set `self.ArrayIndex` _returnvalue_85)
                        (goto _label_3)
                        (else
                          (bind _returnvalue_86 (`self.isDialogDataAccurate` 1))
                          (if _returnvalue_86
                            (bind _returnvalue_87 (`self.setHeaderIndex` 8))
                            (set `self.HeaderIndex` _returnvalue_87)
                            (bind _returnvalue_88 (`self.setArrayIndex` 4))
                            (set `self.ArrayIndex` _returnvalue_88)
                            (goto _label_3)
                            (else
                              (bind _returnvalue_89 (`self.isDialogDataAccurate` 2))
                              (if _returnvalue_89
                                (bind _returnvalue_90 (`self.setHeaderIndex` 8))
                                (set `self.HeaderIndex` _returnvalue_90)
                                (bind _returnvalue_91 (`self.setArrayIndex` 4))
                                (set `self.ArrayIndex` _returnvalue_91)
                                (goto _label_3))))))
                      (elif (== (`self.HeaderIndex`) 10)
                        (bind _returnvalue_92 (`self.isDialogDataAccurate` 0))
                        (if _returnvalue_92
                          (bind _returnvalue_93 (`self.setHeaderIndex` 11))
                          (set `self.HeaderIndex` _returnvalue_93)
                          (bind _returnvalue_94 (`self.setArrayIndex` 8))
                          (set `self.ArrayIndex` _returnvalue_94)
                          (goto _label_3)
                          (else
                            (bind _returnvalue_95 (`self.isDialogDataAccurate` 1))
                            (if _returnvalue_95
                              (`self.Leave`)
                              (else
                                (bind _returnvalue_96 (`self.isDialogDataAccurate` 2))
                                (if _returnvalue_96
                                  (bind _returnvalue_97 (`self.getMainCharacter`))
                                  (set `MainCharacter.bWantSacrifice` true _returnvalue_97)
                                  (set `MainCharacter.Points` (+ (`MainCharacter.Points` _returnvalue_97) 10) _returnvalue_97)
                                  (`self.Leave`))))))
                        (elif (== (`self.HeaderIndex`) 11)
                          (bind _returnvalue_98 (`self.isDialogDataAccurate` 0))
                          (if _returnvalue_98
                            (`self.Leave`)
                            (else
                              (bind _returnvalue_99 (`self.isDialogDataAccurate` 1))
                              (if _returnvalue_99
                                (`self.Leave`)
                                (else
                                  (bind _returnvalue_100 (`self.isDialogDataAccurate` 2))
                                  (if _returnvalue_100
                                    (bind _returnvalue_101 (`self.getMainCharacter`))
                                    (set `MainCharacter.Points` (- (`MainCharacter.Points` _returnvalue_101) 3) _returnvalue_101)
                                    (set `MainCharacter.bWalkThroughFirst` false _returnvalue_101)
                                    (`self.Leave`))))))
                          (elif (== (`self.HeaderIndex`) 12)
                            (bind _returnvalue_102 (`self.isDialogDataAccurate` 0))
                            (if _returnvalue_102
                              (bind _returnvalue_103 (`self.setHeaderIndex` 10))
                              (set `self.HeaderIndex` _returnvalue_103)
                              (bind _returnvalue_104 (`self.setArrayIndex` 7))
                              (set `self.ArrayIndex` _returnvalue_104)
                              (goto _label_3)
                              (else
                                (bind _returnvalue_105 (`self.isDialogDataAccurate` 1))
                                (if _returnvalue_105
                                  (bind _returnvalue_106 (`self.setHeaderIndex` 10))
                                  (set `self.HeaderIndex` _returnvalue_106)
                                  (bind _returnvalue_107 (`self.setArrayIndex` 7))
                                  (set `self.ArrayIndex` _returnvalue_107)
                                  (goto _label_3)
                                  (else
                                    (bind _returnvalue_108 (`self.isDialogDataAccurate` 2))
                                    (if _returnvalue_108
                                      (bind _returnvalue_109 (`self.setHeaderIndex` 10))
                                      (set `self.HeaderIndex` _returnvalue_109)
                                      (bind _returnvalue_110 (`self.setArrayIndex` 7))
                                      (set `self.ArrayIndex` _returnvalue_110)
                                      (goto _label_3))))))
                            (elif (== (`self.HeaderIndex`) 13)
                              (bind _returnvalue_111 (`self.isDialogDataAccurate` 0))
                              (if _returnvalue_111
                                (bind _returnvalue_112 (`self.setHeaderIndex` 10))
                                (set `self.HeaderIndex` _returnvalue_112)
                                (bind _returnvalue_113 (`self.setArrayIndex` 7))
                                (set `self.ArrayIndex` _returnvalue_113)
                                (goto _label_3)
                                (else
                                  (bind _returnvalue_114 (`self.isDialogDataAccurate` 1))
                                  (if _returnvalue_114
                                    (bind _returnvalue_115 (`self.setHeaderIndex` 10))
                                    (set `self.HeaderIndex` _returnvalue_115)
                                    (bind _returnvalue_116 (`self.setArrayIndex` 7))
                                    (set `self.ArrayIndex` _returnvalue_116)
                                    (goto _label_3)
                                    (else
                                      (bind _returnvalue_117 (`self.isDialogDataAccurate` 2))
                                      (if _returnvalue_117
                                        (bind _returnvalue_118 (`self.setHeaderIndex` 10))
                                        (set `self.HeaderIndex` _returnvalue_118)
                                        (bind _returnvalue_119 (`self.setArrayIndex` 7))
                                        (set `self.ArrayIndex` _returnvalue_119)
                                        (goto _label_3)))))))))))))))))))))

(event `Answer2`
  (`self.setChosenNumber` 1)
  (goto _label_2))

(event `Answer3`
  (`self.setChosenNumber` 2)
  (goto _label_2))

(fn `UserConstructionScript`
  ;[1 1 1] Header configuration
  (bind _output_get (set `self.HeaderStart` "Och, tu jesteś! Wszędzie Cię szukałam!"))
  (set `self.Header1` "Och, oczywiście, na pewno masz wiele pytań Jesteś w Krainie Marzeń. My - opiekunowie tego miejsca, nasłuchujemy \"wołań\" - próśb, błagań, skrytych pragnień -  ludzi. A tych, którzy mają czyste serce oraz szczere zamiary, zapraszamy do naszego świata. Dlatego się tu znalazłeś.")
  (set `self.Header2` "Absurd! W Krainie Marzeń nie odczuwa się głodu, ani zimna, czy bólu. My - opiekunowie tego miejsca, nie jesteśmy zdolni do odczuwania takich rzeczy... Już nie. Nasłuchujemy jednakże \"wołań\" - próśb, błagań, skrytych pragnień - ludzi. A tych, którzy mają czyste serce oraz szczere zamiary, zapraszamy do naszego świata. Dlatego się tu znalazłeś.")
  (set `self.Header3` "Rozumiem, spokojnie, cofam się, widzisz? Już zapomniałam, co to strach, dezorientacja... Przepraszam. Jestem jednym z wielu opiekunów tego miejsca. Naszym celem jest nasłuchiwanie \"wołań\" - próśb, błagań, skrytych pragnień - ludzi. A tych, którzy mają czyste serce oraz szczere zamiary, zapraszamy do Krainy Marzeń, naszego świata. Dlatego się tu znalazłeś.")
  (set `self.Header4` "Racja, czas jest w Twojej sytuacji kluczowy, wybacz mój nietakt. My już zrobiliśmy wszystko, co w naszej mocy. Teraz musisz wziąć sprawy w swoje ręce. Powiem więc krótko - jeśli zależy Ci na siostrze, musisz pokazać Drzewu Mądrości, że naprawdę masz szczere intencje.")
  (set `self.Header5` "My już zrobiliśmy wszystko, co w naszej mocy. Teraz musisz wziąć sprawy w swoje ręce. Powiem wprost - nie będzie łatwo. Będziesz poddany przeróżnym próbom, które będą testować Twój charakter, intencje... Strażnicy będą Cię kusić i prowokować. Jeśli zależy Ci na siostrze, musisz pokazać Drzewu Mądrości, że naprawdę masz szczere intencje. ")
  (set `self.Header6` "Nie. Wszyscy mieszkańcy tego świata byli kiedyś ludźmi, takimi jak Ty. Każdy z nas ma własną historię, każdy z nas chciał rozpaczliwie spełnić swoje życzenie. Niektórzy z nas nie mieli po co wracać do świata żywych, inni zostali ukarani, nieliczni postradali zmysły i zostali tu zamknięci, by nie czynić żywym krzywdy. Pieczę nad nami sprawuje Drzewo Mądrości.")
  (set `self.Header7` "Racja, czas w Twojej sytuacji jest kluczowy, wybacz mój nietakt. Zrobiłam wszystko, co mogłam. Musisz teraz wziąć sprawy w swoje ręce. Nie będzie łatwo, bo będziesz wystawiany na wiele różnych prób. Jeśli zależy Ci na siostrze, musisz pokazać Drzewu Mądrości, że masz naprawdę szczere intencje.")
  (set `self.Header8` "Zrobiłam wszystko, co mogłam. Musisz wziąć sprawy w swoje ręce. Nie będzie łatwo, bo będziesz wystawiony na wiele różnych prób. Jeśli zależy Ci na siostrze, musisz pokazać Drzewu Mądrości, że masz naprawdę szczere intencje.")
  (set `self.Header11` "Absurd! To, co teraz widzisz jest REALNE. Nie znalazłeś się tu bez powodu. My, istoty żyjące w Krainie Marzeń, istniejemy po to, by słuchać \"wołań\" - próśb, błagań, skrytych pragnień -  ludzi. A tych, którzy mają czyste serce oraz szczere intencje, sprowadzamy do naszego domu i poddajmy próbom, nie słuchałeś? Tym razem to Twojej prośby wysłuchaliśmy. Nie kpij z tego!")
  (set `self.Header13` "Będziesz zbierał do słoja zbierał kryształy. Kolorowe, jeśli inne istoty uznają, że przeszedłeś próbę. Czarne w przeciwnym przypadku. Jeśli nie przejdziesz próby, część Twoich już zebranych kolorowych kryształów zczernieje. Zanieś wypełniony słój do Drzewa Mądrości.Zapomniałabym... Za wykorzystanie życzenia... Musisz zapłacić swoim życiem.")
  (set `self.Header16` "Niektórym ta cena nieodpowiada i po prostu rezygnują z życzenia. Inni uważają, że to odpowiednia cena. Tak czy siak, musisz się dostać do Drzewa Mądrości, bo tylko ono jest w stanie Cię stąd wypuścić.")
  (set `self.Header18` "Jest esencją tego miejsca. Bez niego to miejsce umrze. Nie wiem skąd się tu wzięło i chyba nikt nie wie. Jesteś zbyt dociekliwy, a czasu coraz mniej. Bierz się do roboty. Niebawem inni opiekunowie poddadzą Cię próbom. Nie będzie łatwo, ale jeśli Ci zależy na siostrze, na pewno dasz radę udowodnić swoje szczere intencje.")
  (set `self.Header22` "Nie. Słuchaj, zrobiłam wszystko, co mogłam. Musisz wziąć sprawy w swoje ręce. Nie będzie łatwo, bo będziesz wystawiony na wiele różnych prób. Jeśli zależy Ci na siostrze, musisz pokazać Drzewu Mądrości, że masz naprawdę szczere intencje. ")
  (set `self.CurrentNPCResponse` _output_get)
  ;[1 1 1] Dialog Data configuration
  (set `self.Odp0.1` "Szukałaś mnie? Kim jesteś? Gdzie ja jestem?")
  (set `self.Odp0.2` "Co za dziwnie realistyczny sen... Czy tylko mi się wydaje, że strasznie tu zimno?")
  (set `self.Odp0.3` "Odsuń się, zjawo! Masz natychmiast mi wyjaśnić co się dzieje!")
  (set `self.Odp1.1` "A więc mama miała rację...? Wyleczysz moją siostrę?")
  (set `self.Odp1.2` "A jaka jest zapłata za wyleczenie siostry?")
  (set `self.Odp1.3` "A tak konkretniej? Co muszę zrobić, żeby wyleczyć siostrę?")
  (set `self.Odp2.1` "\"Już nie odczuwacie takich rzeczy\"...? To nie od zawsze jesteście zjawami?")
  (set `self.Odp2.2` "Skoro to nie sen... To znaczy, że mama miała rację. Uleczysz moją siostrę?")
  (set `self.Odp2.3` "Cudownie, więc tu utknąłem? Może chociaż przejdziemy do konkretów i uleczysz moją siostrę?")
  (set `self.Odp3.1` "Przejdźmy do konkretów: moja siostra umiera. Czy możecie ją wyleczyć?")
  (set `self.Odp3.2` "A więc mama miała rację... Wyleczycie moją siostrę? Proszę, ona umiera!")
  (set `self.Odp3.3` "\"Już zapomniałam\"? To nie od zawsze jesteś zjawą?")
  (set `self.Odp4.1` "Czy ten słoik, który mam na plecach będzie mi do czegoś potrzebny?")
  (set `self.Odp4.2` "Ten słoik na moich plecach jest strasznie lekki jak na tak duży słoik")
  (set `self.Odp4.3` "Po co mi ten słój na plecach?")
  (set `self.Odp6.1` "To kto może uratować moją siostrę?")
  (set `self.Odp6.2` "To Drzewo Mądrości...")
  (set `self.Odp6.3` "Dosyć pogaduszek. Powiedz mi, jak mam uratować siostrę.")
  (set `self.Odp11.1` "W ogóle nie masz poczucia humoru. Nigdy się nie śmiejecie?")
  (set `self.Odp11.2` "Przepraszam, tylko się droczyłem. Powiesz mi, jak uratować siostrę?")
  (set `self.Odp11.3` "Powtarzasz się, nudziaro. Będę kpił, z czego będę chciał. Ulecz mi siostrę, zamiast gadać.")
  (set `self.Odp13.1` "I ludzie się na to godzą?!")
  (set `self.Odp13.2` "O! A więc to jest sposób, by się stąd wydostać? Trzeba TYLKO umrzeć [Odejdź]")
  (set `self.Odp13.3` "Myślę, że to jest cena, którą jestem gotów zapłacić. [Odejdź]")
  (set `self.Odp16.1` "[Przytaknij i odejdź]")
  (set `self.Odp16.2` "[Odejdź]")
  (set `self.Odp16.3` "[Przebiegnij dla zabawy przez zjawę]")
  (bind _returnvalue (`self.setHeaderIndex` 0))
  (bind _output_get_2 (set `self.HeaderIndex` _returnvalue))
  (bind _returnvalue_2 (`self.setArrayIndex` _output_get_2))
  (set `self.ArrayIndex` _returnvalue_2))