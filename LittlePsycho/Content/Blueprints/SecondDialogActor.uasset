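; NPC dialogue actor that runs a branching conversation, with partly hard-coded Polish lines, while overlapped.
; Overlap opens a DialogInterface3 widget with input and cursor; ending overlap closes it and resets the conversation.
; Answer1–3 share a nested branch on the UpdateArray state, setting the NPC reply and selecting the next ButtonText set.
; Answer4, or any answer in the farewell state (2), closes the dialogue and destroys the actor.
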(event `self.ReceiveActorBeginOverlap`
  (params (OtherActor :type "Actor Object Reference"))
  ;[1 1 1] begin and end overlap
  (`self.EnableInput` (`GameplayStatics.GetPlayerController` 0))
  (bind _returnvalue (`|CreateWidget` "/Game/Dialog/DialogInterface3.DialogInterface3_C" (`GameplayStatics.GetPlayerController` 0)))
  (bind _output_get (set `self.DialogInterface` _returnvalue))
  (bind _output_get_2 (set `self.CurrentNPCResponse` (`self.Start`)))
  (`TextBlock.SetText` (`/Game/Dialog/DialogInterface3.Text_Block_1` _output_get) _output_get_2)
  (`UserWidget.AddToViewport` (`self.DialogInterface`) 0)
  (set `PlayerController.bShowMouseCursor` true (`GameplayStatics.GetPlayerController` 0))
  (set `self.ButtonText` (select `int` (`self.UpdateArray`) :`0` (`|MakeArray` (`self.Question 0 - 1`) (`self.Question 0 - 2`) (`self.Question 0 - 3`)) :`1` (`|MakeArray` (`self.Question 1- 1`) (`self.Question 1- 2`) (`self.Question 1 - 3`)) :`2` (`|MakeArray` (`self.Question 2 - 1`) (`self.Question 2 - 2`) (`self.Question 2 - 3`)) :`3` (`|MakeArray` (`self.Question 3 - 1`) (`self.Question 3 - 2`) (`self.Question 3 - 3`)) :`4` (`|MakeArray` (`self.Question 4 - 1`) (`self.Question 4 - 2`) (`self.Question 4 - 3`)) :`5` (`|MakeArray` (`self.Question 5 - 1`) (`self.Question 5 -2`) (`self.Question 5 - 3`)) :`6` (`|MakeArray` (`self.Question 6 - 1`) (`self.Question 6 - 2`) (`self.Question 6 - 3`)) :`7` (`|MakeArray` (`self.Question 7 - 1`) (`self.Question 7 - 2`) (`self.Question 7 - 3`)) :`8` (`|MakeArray` (`self.Question 8 - 1`) (`self.Question 8 - 2`) (`self.Question 8 - 3`)) :`9` (`|MakeArray` (`self.Question 9 - 1`) (`self.Question 9 - 2`) (`self.Question 9 - 3`)))))

(event `self.ReceiveActorEndOverlap`
  (params (OtherActor :type "Actor Object Reference"))
  ;[1 1 1] begin and end overlap
  (`self.DisableInput` (`GameplayStatics.GetPlayerController` 0) :!label _label)
  (bind _output_get (set `self.CurrentNPCResponse` (`self.End`)))
  (`TextBlock.SetText` (`/Game/Dialog/DialogInterface3.Text_Block_1` (stale `self.ReceiveActorBeginOverlap` _output_get)) _output_get)
  (set `self.UpdateArray` 0)
  (`Widget.RemoveFromParent` (`self.DialogInterface`))
  (set `PlayerController.bShowMouseCursor` false (`GameplayStatics.GetPlayerController` 0)))

(event `Leaving`
  ;[1 1 1] begin and end overlap
  (goto _label))

(event `Answer1`
  (bind _int (`self.Int`))
  (bind _int_2 (`self.int`))
  (bind _int_3 (`self.int`))
  (bind _int_4 (`self.int`))
  (bind _int_5 (`self.int`))
  (bind _int_6 (`self.int`))
  ;[1 1 1] Answers Setup
  (set `self.Int` 0)
  (if (== (`self.UpdateArray`) 0) :!label _label_2
    (if (== _int 0)
      (bind _output_get (set `self.CurrentNPCResponse` (`self.NPC0-1`)))
      (`TextBlock.SetText` (`/Game/Dialog/DialogInterface3.Text_Block_1` (`self.DialogInterface`)) _output_get)
      (set `self.UpdateArray` 1)
      (set `self.ButtonText` (select `int` (`self.UpdateArray`) :`0` (`|MakeArray` (`self.Question 0 - 1`) (`self.Question 0 - 2`) (`self.Question 0 - 3`)) :`1` (`|MakeArray` (`self.Question 1- 1`) (`self.Question 1- 2`) (`self.Question 1 - 3`)) :`2` (`|MakeArray` (`self.Question 2 - 1`) (`self.Question 2 - 2`) (`self.Question 2 - 3`)) :`3` (`|MakeArray` (`self.Question 3 - 1`) (`self.Question 3 - 2`) (`self.Question 3 - 3`)) :`4` (`|MakeArray` (`self.Question 4 - 1`) (`self.Question 4 - 2`) (`self.Question 4 - 3`)) :`5` (`|MakeArray` (`self.Question 5 - 1`) (`self.Question 5 -2`) (`self.Question 5 - 3`)) :`6` (`|MakeArray` (`self.Question 6 - 1`) (`self.Question 6 - 2`) (`self.Question 6 - 3`)) :`7` (`|MakeArray` (`self.Question 7 - 1`) (`self.Question 7 - 2`) (`self.Question 7 - 3`)) :`8` (`|MakeArray` (`self.Question 8 - 1`) (`self.Question 8 - 2`) (`self.Question 8 - 3`)) :`9` (`|MakeArray` (`self.Question 9 - 1`) (`self.Question 9 - 2`) (`self.Question 9 - 3`))) :!label _label_3)
      (elif (== _int 1)
        (bind _output_get_2 (set `self.CurrentNPCResponse` (`self.NPC0-2`)))
        (`TextBlock.SetText` (`/Game/Dialog/DialogInterface3.Text_Block_1` (`self.DialogInterface`)) _output_get_2)
        (set `self.UpdateArray` 1)
        (goto _label_3)
        (elif (== _int 2)
          (bind _output_get_3 (set `self.CurrentNPCResponse` (`self.NPC0-1`)))
          (`TextBlock.SetText` (`/Game/Dialog/DialogInterface3.Text_Block_1` (`self.DialogInterface`)) _output_get_3)
          (set `self.UpdateArray` 1)
          (goto _label_3))))
    (elif (== (`self.UpdateArray`) 1)
      (if (== _int_3 0)
        (bind _output_get_4 (set `self.CurrentNPCResponse` "Tak! Tak! Haha! I co dalej?"))
        (`TextBlock.SetText` (`/Game/Dialog/DialogInterface3.Text_Block_1` (`self.DialogInterface`)) _output_get_4)
        (set `self.UpdateArray` 3)
        (goto _label_3)
        (elif (== _int_3 1)
          (bind _output_get_5 (set `self.CurrentNPCResponse` "Haha! Wydostać się chcesz, hm? Jak?"))
          (`TextBlock.SetText` (`/Game/Dialog/DialogInterface3.Text_Block_1` (`self.DialogInterface`)) _output_get_5)
          (set `self.UpdateArray` 4)
          (goto _label_3)
          (elif (== _int_3 2)
            (bind _output_get_6 (set `self.CurrentNPCResponse` "Tak! Haha! Sen... Sen? O czym lubisz śnić?"))
            (`TextBlock.SetText` (`/Game/Dialog/DialogInterface3.Text_Block_1` (`self.DialogInterface`)) _output_get_6)
            (set `self.UpdateArray` 5)
            (goto _label_3))))
      (elif (== (`self.UpdateArray`) 2)
        (if (== _int_4 0)
          (cast `MainCharacter` (`GameplayStatics.GetPlayerPawn` 0))
          (`self.Leaving`)
          (`self.K2_DestroyActor`)
          (elif (== _int_4 1)
            (cast `MainCharacter` (`GameplayStatics.GetPlayerPawn` 0))
            (`self.Leaving`)
            (`self.K2_DestroyActor`)
            (elif (== _int_4 2)
              (cast `MainCharacter` (`GameplayStatics.GetPlayerPawn` 0))
              (`self.Leaving`)
              (`self.K2_DestroyActor`))))
        (elif (== (`self.UpdateArray`) 3)
          (if (== _int_5 0)
            (bind _output_get_7 (set `self.CurrentNPCResponse` "Taki... Miłe... Taki.e... Słodkie... Ohyda! Fuj! Może już znikniesz?"))
            (`TextBlock.SetText` (`/Game/Dialog/DialogInterface3.Text_Block_1` (`self.DialogInterface`)) _output_get_7)
            (set `self.UpdateArray` 2)
            (goto _label_3)
            (elif (== _int_5 1)
              (bind _output_get_8 (set `self.CurrentNPCResponse` "Samolubne! Haha! Podoba mi się, podoba, bardzo mi się podoba! Idź już,. Inne złośliwce już na Ciebie czekają."))
              (`TextBlock.SetText` (`/Game/Dialog/DialogInterface3.Text_Block_1` (`self.DialogInterface`)) _output_get_8)
              (set `self.UpdateArray` 2)
              (goto _label_3)
              (elif (== _int_5 2)
                (bind _output_get_9 (set `self.CurrentNPCResponse` "Samolubne! Haha! Podoba mi się, podoba, bardzo mi się podoba! Idź już,. Inne złośliwce już na Ciebie czekają."))
                (`TextBlock.SetText` (`/Game/Dialog/DialogInterface3.Text_Block_1` (`self.DialogInterface`)) _output_get_9)
                (set `self.UpdateArray` 2)
                (goto _label_3))))
          (elif (== (`self.UpdateArray`) 4)
            (if (== _int_6 0)
              (bind _output_get_10 (set `self.CurrentNPCResponse` "Tak, tak, rozumiesz! Pytasz! Ciekawość, ciekawość! Bądź ciekawy następnym razem. Idź już, znikaj!"))
              (`TextBlock.SetText` (`/Game/Dialog/DialogInterface3.Text_Block_1` (`self.DialogInterface`)) _output_get_10)
              (set `self.UpdateArray` 2)
              (goto _label_3)
              (elif (== _int_6 1)
                (bind _output_get_11 (set `self.CurrentNPCResponse` "Władza! Haha! Podoba mi się, podoba, bardzo mi się podoba! Idź już,. Inne złośliwce już na Ciebie czekają."))
                (`TextBlock.SetText` (`/Game/Dialog/DialogInterface3.Text_Block_1` (`self.DialogInterface`)) _output_get_11)
                (set `self.UpdateArray` 2)
                (goto _label_3)
                (elif (== _int_6 2)
                  (bind _output_get_12 (set `self.CurrentNPCResponse` "Samolubne! Haha! Podoba mi się, podoba, bardzo mi się podoba! Idź już,. Inne złośliwce już na Ciebie czekają."))
                  (`TextBlock.SetText` (`/Game/Dialog/DialogInterface3.Text_Block_1` (`self.DialogInterface`)) _output_get_12)
                  (set `self.UpdateArray` 2)
                  (goto _label_3))))
            (elif (== (`self.UpdateArray`) 5)
              (if (== _int_2 0)
                (bind _output_get_13 (set `self.CurrentNPCResponse` "Taki... Miłe... Taki.e... Słodkie... Ohyda! Fuj! Może już znikniesz?"))
                (`TextBlock.SetText` (`/Game/Dialog/DialogInterface3.Text_Block_1` (`self.DialogInterface`)) _output_get_13)
                (set `self.UpdateArray` 2)
                (goto _label_3)
                (elif (== _int_2 1)
                  (bind _output_get_14 (set `self.CurrentNPCResponse` "Samolubne! Haha! Podoba mi się, podoba, bardzo mi się podoba! Idź już,. Inne złośliwce już na Ciebie czekają."))
                  (`TextBlock.SetText` (`/Game/Dialog/DialogInterface3.Text_Block_1` (`self.DialogInterface`)) _output_get_14)
                  (set `self.UpdateArray` 2)
                  (goto _label_3)
                  (elif (== _int_2 2)
                    (bind _output_get_15 (set `self.CurrentNPCResponse` "Bo mogę, haha! Może już sobie pójdziesz?"))
                    (`TextBlock.SetText` (`/Game/Dialog/DialogInterface3.Text_Block_1` (`self.DialogInterface`)) _output_get_15)
                    (set `self.UpdateArray` 2)
                    (goto _label_3)))))))))))

(event `Answer2`
  ;[1 1 1] Answers Setup
  (set `self.Int` 1)
  (goto _label_2))

(event `Answer3`
  ;[1 1 1] Answers Setup
  (set `self.Int` 2)
  (goto _label_2))

(event `Answer4`
  ;[1 1 1] Answers Setup
  (`self.Leaving`)
  (`self.K2_DestroyActor`))

(fn `UserConstructionScript`)