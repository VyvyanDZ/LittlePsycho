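; Final-judgement NPC, the Tree of Wisdom, which reviews the player's deeds in Polish dialogue and triggers one of three endings.
; Overlap disables player input and opens a dialog widget.
; GetNext steps HeaderIndex through a nested branch chain over MainCharacter's points and choice flags, selecting verdict lines set in the Construction Script.
; A decision widget then branches on ArrayIndex about surrendering the jar and the wish, showing an Outro before quitting.
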(event `self.ReceiveActorBeginOverlap`
  (params (OtherActor :type "Actor Object Reference"))
  ;[1 1 1] Handle input and camera
  (bind _asmain_character (cast `MainCharacter` OtherActor))
  (bind _returnvalue (`self.setMainCharacter` _asmain_character))
  (bind _returnvalue_2 (`GameplayStatics.GetPlayerController` _returnvalue))
  (`self.DisableInput` _returnvalue _returnvalue_2)
  (bind _returnvalue_3 (`|CreateWidget` "/Game/Dialog/DialogInterface9.DialogInterface9_C" _returnvalue_2))
  (bind _output_get (set `self.DialogInterface` _returnvalue_3))
  (`TextBlock.SetText` (`/Game/Dialog/DialogInterface9.Text_Block_1` _output_get) (`self.Header Start`))
  (`UserWidget.AddToViewport` _output_get 0)
  (set `PlayerController.bShowMouseCursor` true _returnvalue_2))

(event `self.ReceiveActorEndOverlap`
  (params (OtherActor :type "Actor Object Reference"))
  (bind _returnvalue (`GameplayStatics.GetPlayerController` 0))
  ;[1 1 1] Handle input and camera
  (`Widget.RemoveFromParent` (`self.DialogInterface`) :!label _label)
  (bind _returnvalue_2 (`self.getMainCharacter`))
  (`self.EnableInput` _returnvalue_2 _returnvalue)
  (set `PlayerController.bShowMouseCursor` false _returnvalue))

(event `Leave`
  ;[1 1 1] Handle input and camera
  (`self.endDialog`)
  (goto _label))

(event `GetNext`
  (bind _decisioninterface (`self.DecisionInterface`))
  (if (== (`self.HeaderIndex`) 0)
    (bind _returnvalue (`self.getMainCharacter`))
    (if (>= (`MainCharacter.Points` _returnvalue) 0)
      (bind _returnvalue_2 (`self.setHeaderIndex` 1))
      (set `self.HeaderIndex` _returnvalue_2)
      (else
        (bind _returnvalue_3 (`self.setHeaderIndex` 2))
        (set `self.HeaderIndex` _returnvalue_3)))
    (set `self.NPCCurrentResponse` (select `int` (`self.HeaderIndex`) :`0` (`self.Header Start`) :`1` (`self.Header 1`) :`2` (`self.Header 2`) :`3` (`self.Header 3`) :`4` (`self.Header 4`) :`5` (`self.Header 5`) :`6` (`self.Header 6`) :`7` (`self.Header 7`) :`8` (`self.Header 8`) :`9` (`self.Header 9`) :`10` (`self.Header 12`) :`11` (`self.Header 13`) :`12` (`self.Header 14`) :`13` (`self.Header 15`) :`14` (`self.Header16`) :`15` (`self.Header17`) :`16` (`self.Header18`) :`17` (`self.Header19`) :`18` (`self.Header20`) :`19` (`self.Header21`) :`20` (`self.Header22`) :`21` (`self.Header23`) :`22` (`self.Header24`) :`23` (`self.Header25`) :`24` (`self.Header10`) :`25` (`self.Header11`) :`26` (`self.Header26`) :`27` (`self.Header27`) :`28` (`self.Header28`) :`29` (`self.Header29`) :`30` (`self.Header30`) :`31` (`self.Header31`) :`32` (`self.DecisionHeader`) :`33` (`self.DecisionHeader1`)) :!label _label_2)
    (elif (== (`self.HeaderIndex`) 1)
      (bind _returnvalue_4 (`self.getMainCharacter`))
      (if (`MainCharacter.bWantSacrifice` _returnvalue_4)
        (bind _returnvalue_5 (`self.setHeaderIndex` 3))
        (set `self.HeaderIndex` _returnvalue_5)
        (goto _label_2)
        (else
          (bind _returnvalue_6 (`self.setHeaderIndex` 4))
          (set `self.HeaderIndex` _returnvalue_6)
          (goto _label_2)))
      (elif (== (`self.HeaderIndex`) 2)
        (bind _returnvalue_7 (`self.getMainCharacter`))
        (if (`MainCharacter.bWantSacrifice` _returnvalue_7)
          (bind _returnvalue_8 (`self.setHeaderIndex` 3))
          (set `self.HeaderIndex` _returnvalue_8)
          (goto _label_2)
          (else
            (bind _returnvalue_9 (`self.setHeaderIndex` 4))
            (set `self.HeaderIndex` _returnvalue_9)
            (goto _label_2)))
        (elif (== (`self.HeaderIndex`) 3)
          (bind _returnvalue_10 (`self.getMainCharacter`))
          (if (`MainCharacter.bWasCurious` _returnvalue_10)
            (bind _returnvalue_11 (`self.setHeaderIndex` 5))
            (set `self.HeaderIndex` _returnvalue_11)
            (goto _label_2)
            (else
              (bind _returnvalue_12 (`self.setHeaderIndex` 6))
              (set `self.HeaderIndex` _returnvalue_12)
              (goto _label_2)))
          (elif (== (`self.HeaderIndex`) 4)
            (bind _returnvalue_13 (`self.getMainCharacter`))
            (if (`MainCharacter.bWasCurious` _returnvalue_13)
              (bind _returnvalue_14 (`self.setHeaderIndex` 5))
              (set `self.HeaderIndex` _returnvalue_14)
              (goto _label_2)
              (else
                (bind _returnvalue_15 (`self.setHeaderIndex` 6))
                (set `self.HeaderIndex` _returnvalue_15)
                (goto _label_2)))
            (elif (== (`self.HeaderIndex`) 5)
              (bind _returnvalue_16 (`self.getMainCharacter`))
              (if (`MainCharacter.bFlowersWasTaken` _returnvalue_16)
                (bind _returnvalue_17 (`self.setHeaderIndex` 7))
                (set `self.HeaderIndex` _returnvalue_17)
                (goto _label_2)
                (else
                  (bind _returnvalue_18 (`self.setHeaderIndex` 24))
                  (set `self.HeaderIndex` _returnvalue_18)
                  (goto _label_2)))
              (elif (== (`self.HeaderIndex`) 6)
                (bind _returnvalue_19 (`self.getMainCharacter`))
                (if (`MainCharacter.bFlowersWasTaken` _returnvalue_19)
                  (bind _returnvalue_20 (`self.setHeaderIndex` 7))
                  (set `self.HeaderIndex` _returnvalue_20)
                  (goto _label_2)
                  (else
                    (bind _returnvalue_21 (`self.setHeaderIndex` 24))
                    (set `self.HeaderIndex` _returnvalue_21)
                    (goto _label_2)))
                (elif (== (`self.HeaderIndex`) 7)
                  (bind _returnvalue_22 (`self.getMainCharacter`))
                  (if (`MainCharacter.bForcedToTakeCare` _returnvalue_22)
                    (bind _returnvalue_23 (`self.setHeaderIndex` 8))
                    (set `self.HeaderIndex` _returnvalue_23)
                    (goto _label_2)
                    (else
                      (bind _returnvalue_24 (`self.setHeaderIndex` 28))
                      (set `self.HeaderIndex` _returnvalue_24)
                      (goto _label_2)))
                  (elif (== (`self.HeaderIndex`) 24)
                    (bind _returnvalue_25 (`self.getMainCharacter`))
                    (if (`MainCharacter.bForcedToTakeCare` _returnvalue_25)
                      (bind _returnvalue_26 (`self.setHeaderIndex` 8))
                      (set `self.HeaderIndex` _returnvalue_26)
                      (goto _label_2)
                      (else
                        (bind _returnvalue_27 (`self.setHeaderIndex` 28))
                        (set `self.HeaderIndex` _returnvalue_27)
                        (goto _label_2)))
                    (elif (== (`self.HeaderIndex`) 8)
                      (bind _returnvalue_28 (`self.getMainCharacter`))
                      (if (`MainCharacter.bKilledIll` _returnvalue_28)
                        (bind _returnvalue_29 (`self.setHeaderIndex` 9))
                        (set `self.HeaderIndex` _returnvalue_29)
                        (goto _label_2)
                        (else
                          (bind _returnvalue_30 (`self.setHeaderIndex` 10))
                          (set `self.HeaderIndex` _returnvalue_30)
                          (goto _label_2)))
                      (elif (== (`self.HeaderIndex`) 28)
                        (bind _returnvalue_31 (`self.getMainCharacter`))
                        (if (`MainCharacter.bKilledIll` _returnvalue_31)
                          (bind _returnvalue_32 (`self.setHeaderIndex` 9))
                          (set `self.HeaderIndex` _returnvalue_32)
                          (goto _label_2)
                          (else
                            (bind _returnvalue_33 (`self.setHeaderIndex` 10))
                            (set `self.HeaderIndex` _returnvalue_33)
                            (goto _label_2)))
                        (elif (== (`self.HeaderIndex`) 9)
                          (bind _returnvalue_34 (`self.getMainCharacter`))
                          (if (`MainCharacter.bWonGame` _returnvalue_34)
                            (bind _returnvalue_35 (`self.setHeaderIndex` 11))
                            (set `self.HeaderIndex` _returnvalue_35)
                            (goto _label_2)
                            (else
                              (bind _returnvalue_36 (`self.setHeaderIndex` 26))
                              (set `self.HeaderIndex` _returnvalue_36)
                              (goto _label_2)))
                          (elif (== (`self.HeaderIndex`) 10)
                            (bind _returnvalue_37 (`self.getMainCharacter`))
                            (if (`MainCharacter.bWonGame` _returnvalue_37)
                              (bind _returnvalue_38 (`self.setHeaderIndex` 11))
                              (set `self.HeaderIndex` _returnvalue_38)
                              (goto _label_2)
                              (else
                                (bind _returnvalue_39 (`self.setHeaderIndex` 26))
                                (set `self.HeaderIndex` _returnvalue_39)
                                (goto _label_2)))
                            (elif (== (`self.HeaderIndex`) 11)
                              (bind _returnvalue_40 (`self.getMainCharacter`))
                              (if (`MainCharacter.bWantToAchievePurpose` _returnvalue_40)
                                (bind _returnvalue_41 (`self.setHeaderIndex` 12))
                                (set `self.HeaderIndex` _returnvalue_41)
                                (goto _label_2)
                                (else
                                  (bind _returnvalue_42 (`self.setHeaderIndex` 27))
                                  (set `self.HeaderIndex` _returnvalue_42)
                                  (goto _label_2)))
                              (elif (== (`self.HeaderIndex`) 26)
                                (bind _returnvalue_43 (`self.getMainCharacter`))
                                (if (`MainCharacter.bWantToAchievePurpose` _returnvalue_43)
                                  (bind _returnvalue_44 (`self.setHeaderIndex` 12))
                                  (set `self.HeaderIndex` _returnvalue_44)
                                  (goto _label_2)
                                  (else
                                    (bind _returnvalue_45 (`self.setHeaderIndex` 27))
                                    (set `self.HeaderIndex` _returnvalue_45)
                                    (goto _label_2)))
                                (elif (== (`self.HeaderIndex`) 12)
                                  (bind _returnvalue_46 (`self.getMainCharacter`))
                                  (if (`MainCharacter.bFrustrating` _returnvalue_46)
                                    (bind _returnvalue_47 (`self.setHeaderIndex` 13))
                                    (set `self.HeaderIndex` _returnvalue_47)
                                    (goto _label_2)
                                    (else
                                      (bind _returnvalue_48 (`self.setHeaderIndex` 29))
                                      (set `self.HeaderIndex` _returnvalue_48)
                                      (goto _label_2)))
                                  (elif (== (`self.HeaderIndex`) 27)
                                    (bind _returnvalue_49 (`self.getMainCharacter`))
                                    (if (`MainCharacter.bFrustrating` _returnvalue_49)
                                      (bind _returnvalue_50 (`self.setHeaderIndex` 13))
                                      (set `self.HeaderIndex` _returnvalue_50)
                                      (goto _label_2)
                                      (else
                                        (bind _returnvalue_51 (`self.setHeaderIndex` 29))
                                        (set `self.HeaderIndex` _returnvalue_51)
                                        (goto _label_2)))
                                    (elif (== (`self.HeaderIndex`) 13)
                                      (bind _returnvalue_52 (`self.getMainCharacter`))
                                      (if (`MainCharacter.bGaveUp` _returnvalue_52)
                                        (bind _returnvalue_53 (`self.setHeaderIndex` 14))
                                        (set `self.HeaderIndex` _returnvalue_53)
                                        (goto _label_2)
                                        (else
                                          (bind _returnvalue_54 (`self.setHeaderIndex` 30))
                                          (set `self.HeaderIndex` _returnvalue_54)
                                          (goto _label_2)))
                                      (elif (== (`self.HeaderIndex`) 29)
                                        (bind _returnvalue_55 (`self.getMainCharacter`))
                                        (if (`MainCharacter.bGaveUp` _returnvalue_55)
                                          (bind _returnvalue_56 (`self.setHeaderIndex` 14))
                                          (set `self.HeaderIndex` _returnvalue_56)
                                          (goto _label_2)
                                          (else
                                            (bind _returnvalue_57 (`self.setHeaderIndex` 30))
                                            (set `self.HeaderIndex` _returnvalue_57)
                                            (goto _label_2)))
                                        (elif (== (`self.HeaderIndex`) 14)
                                          (bind _returnvalue_58 (`self.getMainCharacter`))
                                          (if (`MainCharacter.bFlowersWasGiven` _returnvalue_58)
                                            (bind _returnvalue_59 (`self.setHeaderIndex` 23))
                                            (set `self.HeaderIndex` _returnvalue_59)
                                            (goto _label_2)
                                            (else
                                              (bind _returnvalue_60 (`self.setHeaderIndex` 31))
                                              (set `self.HeaderIndex` _returnvalue_60)
                                              (goto _label_2)))
                                          (elif (== (`self.HeaderIndex`) 30)
                                            (bind _returnvalue_61 (`self.getMainCharacter`))
                                            (if (`MainCharacter.bFlowersWasGiven` _returnvalue_61)
                                              (bind _returnvalue_62 (`self.setHeaderIndex` 23))
                                              (set `self.HeaderIndex` _returnvalue_62)
                                              (goto _label_2)
                                              (else
                                                (bind _returnvalue_63 (`self.setHeaderIndex` 31))
                                                (set `self.HeaderIndex` _returnvalue_63)
                                                (goto _label_2)))
                                            (elif (== (`self.HeaderIndex`) 23)
                                              (bind _returnvalue_64 (`self.getMainCharacter`))
                                              (bind _returnvalue_65 (`|CreateWidget` "/Game/Dialog/DecisionInterface.DecisionInterface_C" (`GameplayStatics.GetPlayerController` _returnvalue_64)))
                                              (bind _output_get (set `self.DecisionInterface` _returnvalue_65))
                                              (`TextBlock.SetText` (`/Game/Dialog/DecisionInterface.Text_Block_1` _output_get) (`self.DecisionHeader`))
                                              (`TextBlock.SetText` (`/Game/Dialog/DecisionInterface.Yes` _output_get) (`self.OdpYes`))
                                              (`TextBlock.SetText` (`/Game/Dialog/DecisionInterface.No` _output_get) (`self.OdpNo`))
                                              (bind _returnvalue_66 (`self.setHeaderIndex` 32))
                                              (set `self.HeaderIndex` _returnvalue_66)
                                              (`Widget.RemoveFromParent` (`self.DialogInterface`))
                                              (`UserWidget.AddToViewport` _returnvalue_65 0)
                                              (`UserWidget.AddToViewport` _output_get 0)
                                              (goto _label_2)
                                              (elif (== (`self.HeaderIndex`) 31)
                                                (bind _returnvalue_67 (`self.getMainCharacter`))
                                                (bind _returnvalue_68 (`|CreateWidget` "/Game/Dialog/DecisionInterface.DecisionInterface_C" (`GameplayStatics.GetPlayerController` _returnvalue_67)))
                                                (bind _output_get_2 (set `self.DecisionInterface` _returnvalue_68))
                                                (`TextBlock.SetText` (`/Game/Dialog/DecisionInterface.Text_Block_1` _output_get_2) (`self.DecisionHeader`))
                                                (`TextBlock.SetText` (`/Game/Dialog/DecisionInterface.Yes` _output_get_2) (`self.OdpYes`))
                                                (`TextBlock.SetText` (`/Game/Dialog/DecisionInterface.No` _output_get_2) (`self.OdpNo`))
                                                (bind _returnvalue_69 (`self.setHeaderIndex` 32))
                                                (set `self.HeaderIndex` _returnvalue_69)
                                                (`Widget.RemoveFromParent` (`self.DialogInterface`))
                                                (`UserWidget.AddToViewport` (`self.DecisionInterface`) 0)
                                                (goto _label_2)
                                                (elif (== (`self.HeaderIndex`) 32)
                                                  (if (== (`self.ArrayIndex`) 0)
                                                    (bind _returnvalue_70 (`self.setHeaderIndex` 33))
                                                    (set `self.HeaderIndex` _returnvalue_70)
                                                    (bind _output_get_3 (set `self.OdpYes` "Chcę uleczyć siostrę."))
                                                    (bind _output_get_4 (set `self.OdpNo` "Chcę spełnić własne życzenie"))
                                                    (`TextBlock.SetText` (`/Game/Dialog/DecisionInterface.Yes` _decisioninterface) _output_get_3)
                                                    (`TextBlock.SetText` (`/Game/Dialog/DecisionInterface.No` _decisioninterface) _output_get_4)
                                                    (goto _label_2)
                                                    (elif (== (`self.ArrayIndex`) 1)
                                                      (bind _returnvalue_71 (`|CreateWidget` "/Game/Dialog/outro.outro_C"))
                                                      (bind _output_get_5 (set `self.outro` _returnvalue_71))
                                                      (`TextBlock.SetText` (`/Game/Dialog/outro.Text` _output_get_5) "Zdecydowałeś, że nie oddasz słoja.")
                                                      (`TextBlock.SetText` (`/Game/Dialog/outro.Text1` _output_get_5) "Zachowałeś życie.")
                                                      (`TextBlock.SetText` (`/Game/Dialog/outro.Text2` _output_get_5) "Twoje czyny miały znaczący wpływ na Krainę Marzeń,")
                                                      (`TextBlock.SetText` (`/Game/Dialog/outro.Text3` _output_get_5) " zacząłeś dostrzegać to, czego wcześniej nie widziałeś.")
                                                      (`TextBlock.SetText` (`/Game/Dialog/outro.Text4` _output_get_5) "Twoi rodzice zaczęli poświęcać Ci więcej uwagi, a Ty stałeś się bardziej życzliwy w stosunku do innych.")
                                                      (`TextBlock.SetText` (`/Game/Dialog/outro.Text5` _output_get_5) "Twoja siostra zmarła, zanim się obudziłeś. Nie zdążyłeś się z nią pożegnać.")
                                                      (`Widget.RemoveFromParent` (`self.DecisionInterface`))
                                                      (`UserWidget.AddToViewport` _output_get_5 0)
                                                      (`GameplayStatics.PlaySound2D` "/Game/Movies/197492__palkonimo__heart-rate.197492__palkonimo__heart-rate")
                                                      (`KismetSystemLibrary.Delay` 20.0)
                                                      (`KismetSystemLibrary.QuitGame` null "Quit")))
                                                  (elif (== (`self.HeaderIndex`) 33)
                                                    (if (== (`self.ArrayIndex`) 0)
                                                      (bind _returnvalue_72 (`|CreateWidget` "/Game/Dialog/outro.outro_C"))
                                                      (bind _output_get_6 (set `self.outro` _returnvalue_72))
                                                      (`TextBlock.SetText` (`/Game/Dialog/outro.Text` _output_get_6) "Zdecydowałeś, że oddasz słoj..")
                                                      (`TextBlock.SetText` (`/Game/Dialog/outro.Text1` _output_get_6) "Swoje życzenie wykorzystałeś, ratując siostrze życie.")
                                                      (`TextBlock.SetText` (`/Game/Dialog/outro.Text2` _output_get_6) "Zdążyłeś się obudzić i zobaczyć swoją siostrę żywą...")
                                                      (`TextBlock.SetText` (`/Game/Dialog/outro.Text3` _output_get_6) "Potem zmarłeś z myślą, że postąpiłeś dobrze.")
                                                      (`TextBlock.SetText` (`/Game/Dialog/outro.Text4` _output_get_6) "Duchy Krainy Marzeń zadecydowały, że zostaniesz Opiekunem.")
                                                      (`TextBlock.SetText` (`/Game/Dialog/outro.Text5` _output_get_6) "Od tej pory wystawiasz na próbę kolejnych śmiałków i bacznie obserwujesz swoją siostrę.")
                                                      (`Widget.RemoveFromParent` (`self.DecisionInterface`))
                                                      (`UserWidget.AddToViewport` _output_get_6 0)
                                                      (`KismetSystemLibrary.Delay` 20.0)
                                                      (`KismetSystemLibrary.QuitGame` null "Quit")
                                                      (elif (== (`self.ArrayIndex`) 1)
                                                        (bind _returnvalue_73 (`|CreateWidget` "/Game/Dialog/outro.outro_C"))
                                                        (bind _output_get_7 (set `self.outro` _returnvalue_73))
                                                        (`TextBlock.SetText` (`/Game/Dialog/outro.Text` _output_get_7) "Zdecydowałeś, że oddasz słój.")
                                                        (`TextBlock.SetText` (`/Game/Dialog/outro.Text1` _output_get_7) "Swoje życzenie przeznaczyłeś na swoją własną zachciankę,")
                                                        (`TextBlock.SetText` (`/Game/Dialog/outro.Text2` _output_get_7) "Twoje czyny miały znaczący wpływ na Krainę Marzeń,")
                                                        (`TextBlock.SetText` (`/Game/Dialog/outro.Text3` _output_get_7) "Nie zdążyłeś pożegnać się z siostrą.")
                                                        (`TextBlock.SetText` (`/Game/Dialog/outro.Text4` _output_get_7) "Zaraz po spełnieniu życzenia, umarłeś.")
                                                        (`TextBlock.SetText` (`/Game/Dialog/outro.Text5` _output_get_7) "Duchy zmusiły Cię do tego, byś został opiekunem, Zostałeś najgorszym i najcięższym wyzwaniem dla kolejnych śmiałków, chcących spełnić swoje marzenia. WIelu przez Ciebie zawiodło.")
                                                        (`Widget.RemoveFromParent` (`self.DecisionInterface`))
                                                        (`UserWidget.AddToViewport` _output_get_7 0)
                                                        (`GameplayStatics.PlaySound2D` "/Game/Movies/197492__palkonimo__heart-rate.197492__palkonimo__heart-rate")
                                                        (`KismetSystemLibrary.Delay` 20.0)
                                                        (`KismetSystemLibrary.QuitGame` null "Quit")))))))))))))))))))))))))))))

(fn `UserConstructionScript`
  ;[1 1 1] Header Configuration
  (bind _output_get (set `self.Header Start` "Witaj chłopcze. Jestem Drzewem Mądrości. Widzę, że udało Ci się znależć do mnie drogę. Wiem, że była trudna, mozolna... Cieszę się, że Ci się udało. Pozwól, że wydam teraz swój osąd..."))
  (set `self.Header 1` "Zebrałeś więcej kryształów kolorowych niż czarnych. To bardzo dobrze! Kierowałeś się w większości dobrem. Jednakże nie tylko kryształy przesądzą o Twym losie. Pozwól, że przeanalizuję Twoje dokonania w naszym świecie.")
  (set `self.Header 2` "Zebrałeś więcej kryształów czarnych niż kolorowych.... To smutne. Kierowałeś się złem. Jednakże nie tylko kryształy przesądzą o Twym losie. Pozwól, że przeanalizuję Twoje dokonania w naszym świecie.")
  (set `self.Header 3` "Wykazałeś chęć poświęcenia się dla siostry. To bardzo szlachetne. Opiekunowie byli zachwyceni Twoją postawą. ")
  (set `self.Header 4` "Nie wykazałeś chęci poświęcenia się dla siostry. Wszyscy byliśmy rozczarowani....")
  (set `self.Header 5` "Byłeś ciekawy. Interesował Cię nasz świat i to, jak funkcjonuje. To bardzo przydatna cecha.")
  (set `self.Header 6` "Ani razu nie dopytałeś o szczegóły, dotyczące naszej krainy. ")
  (set `self.Header 7` "Zabrałeś jednemu opiekunowi kwiaty, skazując tym samym niewinne istoty na cierpienie i śmierć. Toż to okrutne! Okrutne! Takiego uczynku się nie wybacza.")
  (set `self.Header 8` "Przekonałeś opiekuna, by wziął odpowiedzialność za swoich podopiecznych. Postąpiłeś odpowiedzialnie i rozsądnie. Nie szedłeś na skróty. ")
  (set `self.Header 9` "Zabiłeś chore istoty dla dobra ogółu. Chyba nikt nie jest w stanie określić, czy to dobry, czy zły uczynek. Niemniej jednak istniało lepsze wyjście z tej sytuacji. Postąpiłeś rozsądnie, ale bez serca.")
  (set `self.Header 12` "Może zabicie chorych królików byłoby lepszym rozwiązaniem?")
  (set `self.Header 13` "Wygrałeś grę w pytania z tym złośliwym dup... Z jednym z opiekunów. Godne podziwu, że udało Ci się nie ponieść emocjom.")
  (set `self.Header 14` "Byłeś zdeterminowany, by osiągnąć swój cel.")
  (set `self.Header 15` "Straciłeś nad sobą panowanie podczas rozmowy z jednym z opiekunów. Smutne jest to, że nie potrafisz kontrolować należycie emocji.")
  (set `self.Header16` "Postanowiłeś się poddać w połowie drogi")
  (set `self.Header17` "Czułeś się porzucony, samotny, niekochany. Nikt nie poświęcał Ci należytej uwagi.")
  (set `self.Header18` "Stwierdziłeś, że wygodniej byłoby, gdyby Twoja siostra nigdy nie istniała. ")
  (set `self.Header19` "Stwierdziłeś, że wolałbyś, żeby Twoja siostra umarła. Zrezygnowałeś z leczenia jej.")
  (set `self.Header20` "Podczas próby z wybraniem właściwej według Ciebie ścieżki, odpowiedziałeś, że zdecydowanie wolisz dawać, niż brać.")
  (set `self.Header21` "Podczas próby z wybraniem właściwej według Ciebie ścieżki, odpowiedziałeś, że zdecydowanie wolisz brać, niż dawać.")
  (set `self.Header22` "W rozmowie z matką uznałeś, że gdybyś był na jej miejscu, starałbyś się uszczęśliwiać chore dziecko do końca jego dni. Nieważne jak krótkie byłoby jego życie.")
  (set `self.Header23` "W rozmowie z matką uznałeś, że gdybyś był na jej miejscu, nie chciałbyś marnować swojego czasu, cierpliwości i energii na zajmowaniu się dzieckiem, które i tak prędzej czy później by zmarło.")
  (set `self.Header24` "Za wszelką cenę chciałeś czuć się ważny.")
  (set `self.Header25` "Pomimo uśmiercenia niewinnych istot i zabrania im jedynego źródła pożywienia, ciągle wierzyłeś, że zjawy, które widzisz są prawdziwe. Kwiaty, które zerwałeś postanowiłeś oddać zjawie, imitującej Twoją siostrę. ")
  (set `self.Header10` "Nie zdecydowałeś się odebrać kwiatów opiekunowi, by podarować je siostrze.")
  (set `self.Header11` "Wszystkie króliki umarły przez Ciebie.")
  (set `self.Header26` "Nie udało Ci się wygrać gry w pytania z jednym z opiekunów")
  (set `self.Header27` "Nie byłeś zdecydowany by osiągnąć swój cel")
  (set `self.Header28` "Nie udało Ci się przekonać opiekuna, by zajął się podopiecznymi")
  (set `self.Header29` "Nie zdenerwowałeś się podczas żadnej rozmowy z opiekunem. Umiesz opanować emocje.")
  (set `self.Header30` "Byłeś zdeterminowany")
  (set `self.Header31` "Nie zdecydowałeś się oddać kwiatów siostrze")
  (set `self.DecisionHeader` "Więc, chcesz oddać słoik, czy wolisz zrezygnować z życzenia?")
  (set `self.OdpYes` "[Oddaj słoik]")
  (set `self.OdpNo` "[Nie oddawaj słoika]")
  (set `self.DecisionHeader1` "Chcesz uleczyć siostrę, czy spełnić swoje życzenie?")
  (set `self.NPCCurrentResponse` _output_get)
  (set `self.HeaderIndex` 0))