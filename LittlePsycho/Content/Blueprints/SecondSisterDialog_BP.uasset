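; Overlap-triggered dialog actor for the player's second conversation with the sick sister, about spending a life-costing wish, in hardcoded Polish.
; Overlap creates the dialog widget, disables player input and shows the cursor; Leave or end overlap reverses this.
; Answer events set the chosen number, then a nested branch chain advances HeaderIndex (NPC line) and ArrayIndex (reply set).
; Each choice varies the sister's response, but all paths share reply sets per stage, and final answers leave.
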(event `self.ReceiveActorBeginOverlap`
  (params (OtherActor :type "Actor Object Reference"))
  ;[1 1 1] Handle input and camera
  (bind _asmain_character (cast `MainCharacter` OtherActor))
  (bind _returnvalue (`self.setMainCharacter` _asmain_character))
  (bind _returnvalue_2 (`GameplayStatics.GetPlayerController` _returnvalue))
  (`self.DisableInput` _returnvalue _returnvalue_2)
  (bind _returnvalue_3 (`|CreateWidget` "/Game/Dialog/DialogInterface11.DialogInterface11_C" _returnvalue_2))
  (bind _output_get (set `self.DialogInterface` _returnvalue_3))
  (`TextBlock.SetText` (`/Game/Dialog/DialogInterface11.Text_Block_1` _output_get) "")
  (set `self.ButtonText` (`|MakeArray` (`self.Odp0.1`) (`self.Odp0.2`) (`self.Odp0.3`)))
  (`UserWidget.AddToViewport` _output_get 0)
  (set `PlayerController.bShowMouseCursor` true _returnvalue_2))

(event `self.ReceiveActorEndOverlap`
  (params (OtherActor :type "Actor Object Reference"))
  (bind _returnvalue (`GameplayStatics.GetPlayerController` 0))
  ;[1 1 1] Handle input and camera
  (`Widget.RemoveFromParent` (`self.DialogInterface`) :!label _label)
  (bind _returnvalue_2 (`self.getMainCharacter`))
  (`self.EnableInput` _returnvalue_2 _returnvalue)
  (set `PlayerController.bShowMouseCursor` false _returnvalue))

(event `Leave`
  ;[1 1 1] Handle input and camera
  (`self.endDialog`)
  (goto _label))

(event `Answer1`
  (`self.setChosenNumber` 0)
  (if (== (`self.HeaderIndex`) 0) :!label _label_2
    (bind _returnvalue (`self.isDialogDataAccurate` 0))
    (if _returnvalue
      (bind _returnvalue_2 (`self.setHeaderIndex` 1))
      (set `self.HeaderIndex` _returnvalue_2)
      (bind _returnvalue_3 (`self.setArrayIndex` 1))
      (set `self.ArrayIndex` _returnvalue_3)
      (set `self.ButtonText` (select `int` (`self.ArrayIndex`) :`0` (`|MakeArray` (`self.Odp0.1`) (`self.Odp0.2`) (`self.Odp0.3`)) :`1` (`|MakeArray` (`self.Odp1.1`) (`self.Odp1.2`) (`self.Odp1.3`)) :`2` (`|MakeArray` (`self.Odp3.1`) (`self.Odp3.2`) (`self.Odp3.3`)) :`3` (`|MakeArray` (`self.Odp4.1`) (`self.Odp4.2`) (`self.Odp4.3`)) :`4` (`|MakeArray` (`self.Odp5.1`) (`self.Odp5.2`) (`self.Odp5.3`))) :!label _label_3)
      (set `self.CurrentNPCResponse` (select `int` (`self.HeaderIndex`) :`0` (`self.HeaderStart`) :`1` (`self.Header1`) :`2` (`self.Header2`) :`3` (`self.Header3`) :`4` (`self.Header4`) :`5` (`self.Header5`) :`6` (`self.Header7`) :`7` (`self.Header8`) :`8` (`self.Header9`) :`9` (`self.Header10`) :`10` (`self.Header11a`) :`11` (`self.Header11b`) :`12` (`self.Header12`)))
      (else
        (bind _returnvalue_4 (`self.isDialogDataAccurate` 1))
        (if _returnvalue_4
          (bind _returnvalue_5 (`self.setHeaderIndex` 2))
          (set `self.HeaderIndex` _returnvalue_5)
          (bind _returnvalue_6 (`self.setArrayIndex` 1))
          (set `self.ArrayIndex` _returnvalue_6)
          (goto _label_3)
          (else
            (bind _returnvalue_7 (`self.isDialogDataAccurate` 2))
            (if _returnvalue_7
              (bind _returnvalue_8 (`self.setHeaderIndex` 3))
              (set `self.HeaderIndex` _returnvalue_8)
              (bind _returnvalue_9 (`self.setArrayIndex` 1))
              (set `self.ArrayIndex` _returnvalue_9)
              (goto _label_3))))))
    (elif (== (`self.HeaderIndex`) 1)
      (bind _returnvalue_10 (`self.isDialogDataAccurate` 0))
      (if _returnvalue_10
        (bind _returnvalue_11 (`self.setHeaderIndex` 4))
        (set `self.HeaderIndex` _returnvalue_11)
        (bind _returnvalue_12 (`self.setArrayIndex` 2))
        (set `self.ArrayIndex` _returnvalue_12)
        (goto _label_3)
        (else
          (bind _returnvalue_13 (`self.isDialogDataAccurate` 1))
          (if _returnvalue_13
            (bind _returnvalue_14 (`self.setHeaderIndex` 5))
            (set `self.HeaderIndex` _returnvalue_14)
            (bind _returnvalue_15 (`self.setArrayIndex` 2))
            (set `self.ArrayIndex` _returnvalue_15)
            (goto _label_3)
            (else
              (bind _returnvalue_16 (`self.isDialogDataAccurate` 2))
              (if _returnvalue_16
                (bind _returnvalue_17 (`self.setHeaderIndex` 6))
                (set `self.HeaderIndex` _returnvalue_17)
                (bind _returnvalue_18 (`self.setArrayIndex` 2))
                (set `self.ArrayIndex` _returnvalue_18)
                (goto _label_3))))))
      (elif (== (`self.HeaderIndex`) 2)
        (bind _returnvalue_19 (`self.isDialogDataAccurate` 0))
        (if _returnvalue_19
          (bind _returnvalue_20 (`self.setHeaderIndex` 4))
          (set `self.HeaderIndex` _returnvalue_20)
          (bind _returnvalue_21 (`self.setArrayIndex` 2))
          (set `self.ArrayIndex` _returnvalue_21)
          (goto _label_3)
          (else
            (bind _returnvalue_22 (`self.isDialogDataAccurate` 1))
            (if _returnvalue_22
              (bind _returnvalue_23 (`self.setHeaderIndex` 5))
              (set `self.HeaderIndex` _returnvalue_23)
              (bind _returnvalue_24 (`self.setArrayIndex` 2))
              (set `self.ArrayIndex` _returnvalue_24)
              (goto _label_3)
              (else
                (bind _returnvalue_25 (`self.isDialogDataAccurate` 2))
                (if _returnvalue_25
                  (bind _returnvalue_26 (`self.setHeaderIndex` 6))
                  (set `self.HeaderIndex` _returnvalue_26)
                  (bind _returnvalue_27 (`self.setArrayIndex` 2))
                  (set `self.ArrayIndex` _returnvalue_27)
                  (goto _label_3))))))
        (elif (== (`self.HeaderIndex`) 3)
          (bind _returnvalue_28 (`self.isDialogDataAccurate` 0))
          (if _returnvalue_28
            (bind _returnvalue_29 (`self.setHeaderIndex` 4))
            (set `self.HeaderIndex` _returnvalue_29)
            (bind _returnvalue_30 (`self.setArrayIndex` 2))
            (set `self.ArrayIndex` _returnvalue_30)
            (goto _label_3)
            (else
              (bind _returnvalue_31 (`self.isDialogDataAccurate` 1))
              (if _returnvalue_31
                (bind _returnvalue_32 (`self.setHeaderIndex` 5))
                (set `self.HeaderIndex` _returnvalue_32)
                (bind _returnvalue_33 (`self.setArrayIndex` 2))
                (set `self.ArrayIndex` _returnvalue_33)
                (goto _label_3)
                (else
                  (bind _returnvalue_34 (`self.isDialogDataAccurate` 2))
                  (if _returnvalue_34
                    (bind _returnvalue_35 (`self.setHeaderIndex` 6))
                    (set `self.HeaderIndex` _returnvalue_35)
                    (bind _returnvalue_36 (`self.setArrayIndex` 2))
                    (set `self.ArrayIndex` _returnvalue_36)
                    (goto _label_3))))))
          (elif (== (`self.HeaderIndex`) 4)
            (bind _returnvalue_37 (`self.isDialogDataAccurate` 0))
            (if _returnvalue_37
              (bind _returnvalue_38 (`self.setHeaderIndex` 7))
              (set `self.HeaderIndex` _returnvalue_38)
              (bind _returnvalue_39 (`self.setArrayIndex` 3))
              (set `self.ArrayIndex` _returnvalue_39)
              (goto _label_3)
              (else
                (bind _returnvalue_40 (`self.isDialogDataAccurate` 1))
                (if _returnvalue_40
                  (bind _returnvalue_41 (`self.setHeaderIndex` 8))
                  (set `self.HeaderIndex` _returnvalue_41)
                  (bind _returnvalue_42 (`self.setArrayIndex` 3))
                  (set `self.ArrayIndex` _returnvalue_42)
                  (goto _label_3)
                  (else
                    (bind _returnvalue_43 (`self.isDialogDataAccurate` 2))
                    (if _returnvalue_43
                      (bind _returnvalue_44 (`self.setHeaderIndex` 9))
                      (set `self.HeaderIndex` _returnvalue_44)
                      (bind _returnvalue_45 (`self.setArrayIndex` 3))
                      (set `self.ArrayIndex` _returnvalue_45)
                      (goto _label_3))))))
            (elif (== (`self.HeaderIndex`) 5)
              (bind _returnvalue_46 (`self.isDialogDataAccurate` 0))
              (if _returnvalue_46
                (bind _returnvalue_47 (`self.setHeaderIndex` 7))
                (set `self.HeaderIndex` _returnvalue_47)
                (bind _returnvalue_48 (`self.setArrayIndex` 3))
                (set `self.ArrayIndex` _returnvalue_48)
                (goto _label_3)
                (else
                  (bind _returnvalue_49 (`self.isDialogDataAccurate` 1))
                  (if _returnvalue_49
                    (bind _returnvalue_50 (`self.setHeaderIndex` 8))
                    (set `self.HeaderIndex` _returnvalue_50)
                    (bind _returnvalue_51 (`self.setArrayIndex` 3))
                    (set `self.ArrayIndex` _returnvalue_51)
                    (goto _label_3)
                    (else
                      (bind _returnvalue_52 (`self.isDialogDataAccurate` 2))
                      (if _returnvalue_52
                        (bind _returnvalue_53 (`self.setHeaderIndex` 9))
                        (set `self.HeaderIndex` _returnvalue_53)
                        (bind _returnvalue_54 (`self.setArrayIndex` 3))
                        (set `self.ArrayIndex` _returnvalue_54)
                        (goto _label_3))))))
              (elif (== (`self.HeaderIndex`) 6)
                (bind _returnvalue_55 (`self.isDialogDataAccurate` 0))
                (if _returnvalue_55
                  (bind _returnvalue_56 (`self.setHeaderIndex` 7))
                  (set `self.HeaderIndex` _returnvalue_56)
                  (bind _returnvalue_57 (`self.setArrayIndex` 3))
                  (set `self.ArrayIndex` _returnvalue_57)
                  (goto _label_3)
                  (else
                    (bind _returnvalue_58 (`self.isDialogDataAccurate` 1))
                    (if _returnvalue_58
                      (bind _returnvalue_59 (`self.setHeaderIndex` 8))
                      (set `self.HeaderIndex` _returnvalue_59)
                      (bind _returnvalue_60 (`self.setArrayIndex` 3))
                      (set `self.ArrayIndex` _returnvalue_60)
                      (goto _label_3)
                      (else
                        (bind _returnvalue_61 (`self.isDialogDataAccurate` 2))
                        (if _returnvalue_61
                          (bind _returnvalue_62 (`self.setHeaderIndex` 9))
                          (set `self.HeaderIndex` _returnvalue_62)
                          (bind _returnvalue_63 (`self.setArrayIndex` 3))
                          (set `self.ArrayIndex` _returnvalue_63)
                          (goto _label_3))))))
                (elif (== (`self.HeaderIndex`) 7)
                  (bind _returnvalue_64 (`self.isDialogDataAccurate` 0))
                  (if _returnvalue_64
                    (bind _returnvalue_65 (`self.setHeaderIndex` 10))
                    (set `self.HeaderIndex` _returnvalue_65)
                    (bind _returnvalue_66 (`self.setArrayIndex` 4))
                    (set `self.ArrayIndex` _returnvalue_66)
                    (goto _label_3)
                    (else
                      (bind _returnvalue_67 (`self.isDialogDataAccurate` 1))
                      (if _returnvalue_67
                        (bind _returnvalue_68 (`self.setHeaderIndex` 11))
                        (set `self.HeaderIndex` _returnvalue_68)
                        (bind _returnvalue_69 (`self.setArrayIndex` 4))
                        (set `self.ArrayIndex` _returnvalue_69)
                        (goto _label_3)
                        (else
                          (bind _returnvalue_70 (`self.isDialogDataAccurate` 2))
                          (if _returnvalue_70
                            (bind _returnvalue_71 (`self.setHeaderIndex` 12))
                            (set `self.HeaderIndex` _returnvalue_71)
                            (bind _returnvalue_72 (`self.setArrayIndex` 4))
                            (set `self.ArrayIndex` _returnvalue_72)
                            (goto _label_3))))))
                  (elif (== (`self.HeaderIndex`) 8)
                    (bind _returnvalue_73 (`self.isDialogDataAccurate` 0))
                    (if _returnvalue_73
                      (bind _returnvalue_74 (`self.setHeaderIndex` 10))
                      (set `self.HeaderIndex` _returnvalue_74)
                      (bind _returnvalue_75 (`self.setArrayIndex` 4))
                      (set `self.ArrayIndex` _returnvalue_75)
                      (goto _label_3)
                      (else
                        (bind _returnvalue_76 (`self.isDialogDataAccurate` 1))
                        (if _returnvalue_76
                          (bind _returnvalue_77 (`self.setHeaderIndex` 11))
                          (set `self.HeaderIndex` _returnvalue_77)
                          (bind _returnvalue_78 (`self.setArrayIndex` 4))
                          (set `self.ArrayIndex` _returnvalue_78)
                          (goto _label_3)
                          (else
                            (bind _returnvalue_79 (`self.isDialogDataAccurate` 2))
                            (if _returnvalue_79
                              (bind _returnvalue_80 (`self.setHeaderIndex` 12))
                              (set `self.HeaderIndex` _returnvalue_80)
                              (bind _returnvalue_81 (`self.setArrayIndex` 4))
                              (set `self.ArrayIndex` _returnvalue_81)
                              (goto _label_3))))))
                    (elif (== (`self.HeaderIndex`) 9)
                      (bind _returnvalue_82 (`self.isDialogDataAccurate` 0))
                      (if _returnvalue_82
                        (bind _returnvalue_83 (`self.setHeaderIndex` 10))
                        (set `self.HeaderIndex` _returnvalue_83)
                        (bind _returnvalue_84 (`self.setArrayIndex` 4))
                        (set `self.ArrayIndex` _returnvalue_84)
                        (goto _label_3)
                        (else
                          (bind _returnvalue_85 (`self.isDialogDataAccurate` 1))
                          (if _returnvalue_85
                            (bind _returnvalue_86 (`self.setHeaderIndex` 11))
                            (set `self.HeaderIndex` _returnvalue_86)
                            (bind _returnvalue_87 (`self.setArrayIndex` 4))
                            (set `self.ArrayIndex` _returnvalue_87)
                            (goto _label_3)
                            (else
                              (bind _returnvalue_88 (`self.isDialogDataAccurate` 2))
                              (if _returnvalue_88
                                (bind _returnvalue_89 (`self.setHeaderIndex` 12))
                                (set `self.HeaderIndex` _returnvalue_89)
                                (bind _returnvalue_90 (`self.setArrayIndex` 4))
                                (set `self.ArrayIndex` _returnvalue_90)
                                (goto _label_3))))))
                      (elif (== (`self.HeaderIndex`) 10)
                        (bind _returnvalue_91 (`self.isDialogDataAccurate` 0))
                        (if _returnvalue_91
                          (`self.Leave`)
                          (else
                            (bind _returnvalue_92 (`self.isDialogDataAccurate` 1))
                            (if _returnvalue_92
                              (`self.Leave`)
                              (else
                                (bind _returnvalue_93 (`self.isDialogDataAccurate` 2))
                                (if _returnvalue_93
                                  (`self.Leave`))))))
                        (elif (== (`self.HeaderIndex`) 11)
                          (bind _returnvalue_94 (`self.isDialogDataAccurate` 0))
                          (if _returnvalue_94
                            (`self.Leave`)
                            (else
                              (bind _returnvalue_95 (`self.isDialogDataAccurate` 1))
                              (if _returnvalue_95
                                (`self.Leave`)
                                (else
                                  (bind _returnvalue_96 (`self.isDialogDataAccurate` 2))
                                  (if _returnvalue_96
                                    (`self.Leave`))))))
                          (elif (== (`self.HeaderIndex`) 12)
                            (bind _returnvalue_97 (`self.isDialogDataAccurate` 0))
                            (if _returnvalue_97
                              (`self.Leave`)
                              (else
                                (bind _returnvalue_98 (`self.isDialogDataAccurate` 1))
                                (if _returnvalue_98
                                  (`self.Leave`)
                                  (else
                                    (bind _returnvalue_99 (`self.isDialogDataAccurate` 2))
                                    (if _returnvalue_99
                                      (`self.Leave`))))))))))))))))))))

(event `Answer2`
  (`self.setChosenNumber` 1)
  (goto _label_2))

(event `Answer3`
  (`self.setChosenNumber` 2)
  (goto _label_2))

(fn `UserConstructionScript`
  ;[1 1 1] Header Configuration
  (bind _output_get (set `self.HeaderStart` "Tu jesteś! Od kiedy tylko tu wróciłam, próbowałam Cię znaleźć!"))
  (set `self.Header1` "Na razie tak. Na razie... Jest źle, bracie, bardzo. Mój czas powoli się kończy. Spotkałam jednego z duchów, które tu żyją. Powiedział, że znaleźliśmy się tu, bo bardzo pragnąłeś, bym wyzdrowiała. Ale powiedział też, że... Życzenie możesz wykorzystać jak tylko chcesz, a za jego spełnienie musisz zapłacić swoim własnym życiem. To chore! Nie chcę, żebyśmy musieli wybierać pomiędzy moim życiem, a Twoim!")
  (set `self.Header2` "To nie ode mnie zależy, tylko od mojego stanu zdrowia. Przykro mi bracie, że musisz działać sam, gdybym mogła, wolałabym sama walczyć o swoje życie... Ech... Jest źle, bracie, bardzo. Mój czas powoli się kończy. Spotkałam jednego z duchów, które tu żyją. Powiedział, że znaleźliśmy się tu, bo bardzo pragnąłeś bym wyzdrowiała. Ale powiedział też, że... Życzenie możesz wykorzystać jak tylko chcesz, a za jego spełnienie musisz zapłacić swoim własnym życiem. To chore! Nie chcę, żebyśmy musieli wybierać pomiędzy moim życiem, a Twoim!")
  (set `self.Header3` "Powiedzmy, że mój stan się trochę ustabilizował, z tego co zrozumiałam. To strasznie bolesne. Ech... Bracie, jest źle, bardzo. Mój czas powoli się kończy. Spotkałam jednego z duchów, które tu żyją. Powiedział, że znaleźliśmy się tu, bo bardzo pragnąłeś, bym wyzdrowiała. Ale powiedział też, że... Życzenie możesz wykorzystać jak tylko chcesz, a za jego spełnienie musisz zapłacić swoim własnym życiem. To chore! Nie chcę, żebyśmy musieli wybierać pomiędzy moim życiem, a Twoim!")
  (set `self.Header4` "Wiem. Nie będę Cię winić, jeśli zużyjesz życzenie na coś innego. I tak będę... martwa, prawda? Ty jesteś zdrowy, młody, dasz sobie radę. Należy Ci się życie. To mnie spotkała choroba. To... Nie mogę Cię prosić, byś się dla mnie poświęcał.")
  (set `self.Header5` "Co? Nie! Nie będę Cię winić, jeśli zużyjesz życzenie na coś innego, czy jeśli w ogóle nie skorzystasz z życzenia.  Należy Ci się życie. To mnie spotkała choroba. To... Nie mogę... Nawet nigdy nie chciałam, żebyś się dla mnie poświęcał.")
  (set `self.Header7` "Musisz żyć! Wspierać rodziców, kiedy odejdę. Szczególnie musisz być podporą dla mamy. Już teraz odchodzi od zmysłów, a co dopiero, kiedy umrę. Nie przejmuj się mną. Nigdy nie chciałam, żebyś się dla mnie poświęcał.")
  (set `self.Header8` "Pamiętaj, cokolwiek wybierzesz, jesteś moim bratem i bardzo Cię kocham. I nie będę Ci nic miała za złe.")
  (set `self.Header9` "Rozumiem. Cokolwiek wybierzesz, jesteś moim bratem, nie będę Ci miała niczego za złe. Kocham Cię bardzo.")
  (set `self.Header10` "Proszę, nie! Postaw na swoje życie! Nie będę Ci miała tego za złe. Bardzo Cię kocham, nie chcę, żebyś się poświęcał! Błagam!")
  (set `self.Header11a` "Ugh... Słabo mi znowu...  Pamiętaj, że jestem z Tobą.  ")
  (set `self.Header11b` "Wiem, przepraszam...Ugh... Słabo mi znowu...  Pamiętaj, że jestem z Tobą.  ")
  (set `self.Header12` "Ale też chcę, żebyś i Ty żył... Ugh... Słabo mi znowu...  Pamiętaj, że jestem z Tobą.  ")
  (set `self.CurrentNPCResponse` _output_get)
  ;[1 1 1] Dialog Data Configuration
  (set `self.Odp0.1` "Wszystko w porządku?")
  (set `self.Odp0.2` "To jakiś żart? Będziesz tak znikać i się pojawiać cały czas?")
  (set `self.Odp0.3` "Trochę nie rozumiem, co tu znowu robisz.")
  (set `self.Odp1.1` "My? Przecież wszystko robię sam. I to do mnie należy życzenie.")
  (set `self.Odp1.2` "I nie będziemy. Twoje zdrowie jest ważniejsze.")
  (set `self.Odp1.3` "Masz rację. Nie oddam duszy. Nie zużyję życzenia.")
  (set `self.Odp3.1` "Ostateczną decyzję podejmę i tak przy Drzewie Mądrości. Muszę się jeszcze zastanowić.")
  (set `self.Odp3.2` "Zrobię, co będę uważał za słuszne, nie interesuje mnie twoje zdanie.")
  (set `self.Odp3.3` "Jesteś moją małą siostrzyczką, jestem gotów oddać życie za ciebie. Będzie dobrze, zobaczysz.")
  (set `self.Odp4.1` "Też Cię kocham.")
  (set `self.Odp4.2` "Nie jestem w stanie już odwzajemniać tak uczuć względem ciebie, jak kiedyś, przepraszam.")
  (set `self.Odp4.3` "Wiem, że chcesz żyć. ")
  (set `self.Odp5.1` "Bez sensu. [Odejdź]")
  (set `self.Odp5.2` "Muszę się pospieszyć. [Odejdź]")
  (set `self.Odp5.3` "Uratuję cię. [Odejdź]")
  (set `self.HeaderIndex` 0)
  (set `self.ArrayIndex` 0))