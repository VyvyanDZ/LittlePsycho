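; Dialog actor for the Polish-language "loss" (strata) conversation, opening a choice widget on player overlap and swapping character input for the cursor.
; Construction script fills the lines; three answer events feed one nested-branch state machine, using HeaderIndex for NPC responses and ArrayIndex for options.
; One answer awards the player points and the Generous flag.
; Final answers destroy KorzyscDialog_BP (benefit dialog) actors and call Leave, which closes the widget and restores input.
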(event `self.ReceiveActorBeginOverlap`
  (params (OtherActor :type "Actor Object Reference"))
  ;[1 1 1] Handle input and camera
  (bind _asmain_character (cast `MainCharacter` OtherActor))
  (bind _returnvalue (`self.setMainCharacter` _asmain_character))
  (bind _returnvalue_2 (`GameplayStatics.GetPlayerController` _returnvalue))
  (`self.DisableInput` _returnvalue _returnvalue_2)
  (bind _returnvalue_3 (`|CreateWidget` "/Game/Dialog/DialogInterface5.DialogInterface5_C" _returnvalue_2))
  (bind _output_get (set `self.DialogInterface` _returnvalue_3))
  (`TextBlock.SetText` (`/Game/Dialog/DialogInterface5.Text_Block_1` _output_get) (`self.Header Start`))
  (set `self.ButtonText` (select `int` (`self.ArrayIndex`) :`0` (`|MakeArray` (`self.Odp 0.1`) (`self.Odp 0.2`) (`self.Odp 0.3`)) :`1` (`|MakeArray` (`self.Odp 1.1`) (`self.Odp 1.2`) (`self.Odp 1.3`)) :`2` (`|MakeArray` (`self.Odp 2.1`) (`self.Odp 2.2`) (`self.Odp 2.3`)) :`3` (`|MakeArray` (`self.Odp4.1`) (`self.Odp4.2`) (`self.Odp4.3`)) :`4` (`|MakeArray` (`self.Odp 7.1`) (`self.Odp 7.2`) (`self.Odp 7.3`)) :`5` (`|MakeArray` (`self.Odp 8.1`) (`self.Odp 8.2`) (`self.Odp 8.3`)) :`6` (`|MakeArray` (`self.Odp15.1`) (`self.Odp15.2`) (`self.Odp15.3`))))
  (`UserWidget.AddToViewport` _output_get 0)
  (set `PlayerController.bShowMouseCursor` true _returnvalue_2))

(event `self.ReceiveActorEndOverlap`
  (params (OtherActor :type "Actor Object Reference"))
  (bind _returnvalue (`GameplayStatics.GetPlayerController` 0))
  ;[1 1 1] Handle input and camera
  (`Widget.RemoveFromParent` (`self.DialogInterface`) :!label _label)
  (bind _returnvalue_2 (`self.getMainCharacter`))
  (`self.EnableInput` _returnvalue_2 _returnvalue)
  (set `PlayerController.bShowMouseCursor` false _returnvalue))

(event `Leave`
  ;[1 1 1] Handle input and camera
  (`self.endDialog`)
  (goto _label))

(event `Answer1`
  (`self.setChosenNumber` 0)
  (if (== (`self.HeaderIndex`) 0) :!label _label_2
    (bind _returnvalue (`self.isDialogDataAccurate` 0))
    (if _returnvalue
      (bind _returnvalue_2 (`self.setHeaderIndex` 1))
      (set `self.HeaderIndex` _returnvalue_2)
      (bind _returnvalue_3 (`self.setArrayIndex` 1))
      (set `self.ArrayIndex` _returnvalue_3)
      (set `self.ButtonText` (select `int` (`self.ArrayIndex`) :`0` (`|MakeArray` (`self.Odp 0.1`) (`self.Odp 0.2`) (`self.Odp 0.3`)) :`1` (`|MakeArray` (`self.Odp 1.1`) (`self.Odp 1.2`) (`self.Odp 1.3`)) :`2` (`|MakeArray` (`self.Odp 2.1`) (`self.Odp 2.2`) (`self.Odp 2.3`)) :`3` (`|MakeArray` (`self.Odp4.1`) (`self.Odp4.2`) (`self.Odp4.3`)) :`4` (`|MakeArray` (`self.Odp 7.1`) (`self.Odp 7.2`) (`self.Odp 7.3`)) :`5` (`|MakeArray` (`self.Odp 8.1`) (`self.Odp 8.2`) (`self.Odp 8.3`)) :`6` (`|MakeArray` (`self.Odp15.1`) (`self.Odp15.2`) (`self.Odp15.3`))) :!label _label_3)
      (set `self.CurrentNPCResponse` (select `int` (`self.HeaderIndex`) :`0` (`self.Header Start`) :`1` (`self.Header 1`) :`2` (`self.Header 2`) :`3` (`self.Header 3`) :`4` (`self.Header 4`) :`5` (`self.Header 5`) :`6` (`self.Header 6`) :`7` (`self.Header 7`) :`8` (`self.Header 8`) :`9` (`self.Header 9`) :`10` (`self.Header 12`) :`11` (`self.Header 13`) :`12` (`self.Header 14`) :`13` (`self.Header 15`)))
      (else
        (bind _returnvalue_4 (`self.isDialogDataAccurate` 1))
        (if _returnvalue_4
          (bind _returnvalue_5 (`self.setHeaderIndex` 2))
          (set `self.HeaderIndex` _returnvalue_5)
          (bind _returnvalue_6 (`self.setArrayIndex` 2))
          (set `self.ArrayIndex` _returnvalue_6)
          (goto _label_3)
          (else
            (bind _returnvalue_7 (`self.isDialogDataAccurate` 2))
            (if _returnvalue_7
              (bind _returnvalue_8 (`self.setHeaderIndex` 3))
              (set `self.HeaderIndex` _returnvalue_8)
              (bind _returnvalue_9 (`self.setArrayIndex` 2))
              (set `self.ArrayIndex` _returnvalue_9)
              (goto _label_3))))))
    (elif (== (`self.HeaderIndex`) 1)
      (bind _returnvalue_10 (`self.isDialogDataAccurate` 0))
      (if _returnvalue_10
        (bind _returnvalue_11 (`self.setHeaderIndex` 4))
        (set `self.HeaderIndex` _returnvalue_11)
        (bind _returnvalue_12 (`self.setArrayIndex` 3))
        (set `self.ArrayIndex` _returnvalue_12)
        (goto _label_3)
        (else
          (bind _returnvalue_13 (`self.isDialogDataAccurate` 1))
          (if _returnvalue_13
            (bind _returnvalue_14 (`self.setHeaderIndex` 5))
            (set `self.HeaderIndex` _returnvalue_14)
            (bind _returnvalue_15 (`self.setArrayIndex` 3))
            (set `self.ArrayIndex` _returnvalue_15)
            (goto _label_3)
            (else
              (bind _returnvalue_16 (`self.isDialogDataAccurate` 2))
              (if _returnvalue_16
                (bind _returnvalue_17 (`self.setHeaderIndex` 6))
                (set `self.HeaderIndex` _returnvalue_17)
                (bind _returnvalue_18 (`self.setArrayIndex` 3))
                (set `self.ArrayIndex` _returnvalue_18)
                (goto _label_3))))))
      (elif (== (`self.HeaderIndex`) 2)
        (bind _returnvalue_19 (`self.isDialogDataAccurate` 0))
        (if _returnvalue_19
          (bind _returnvalue_20 (`self.setHeaderIndex` 7))
          (set `self.HeaderIndex` _returnvalue_20)
          (bind _returnvalue_21 (`self.setArrayIndex` 4))
          (set `self.ArrayIndex` _returnvalue_21)
          (goto _label_3)
          (else
            (bind _returnvalue_22 (`self.isDialogDataAccurate` 1))
            (if _returnvalue_22
              (bind _returnvalue_23 (`self.setHeaderIndex` 8))
              (set `self.HeaderIndex` _returnvalue_23)
              (bind _returnvalue_24 (`self.setArrayIndex` 5))
              (set `self.ArrayIndex` _returnvalue_24)
              (goto _label_3)
              (else
                (bind _returnvalue_25 (`self.isDialogDataAccurate` 2))
                (if _returnvalue_25
                  (bind _returnvalue_26 (`self.setHeaderIndex` 9))
                  (set `self.HeaderIndex` _returnvalue_26)
                  (bind _returnvalue_27 (`self.setArrayIndex` 4))
                  (set `self.ArrayIndex` _returnvalue_27)
                  (goto _label_3))))))
        (elif (== (`self.HeaderIndex`) 3)
          (bind _returnvalue_28 (`self.isDialogDataAccurate` 0))
          (if _returnvalue_28
            (bind _returnvalue_29 (`self.setHeaderIndex` 7))
            (set `self.HeaderIndex` _returnvalue_29)
            (bind _returnvalue_30 (`self.setArrayIndex` 4))
            (set `self.ArrayIndex` _returnvalue_30)
            (goto _label_3)
            (else
              (bind _returnvalue_31 (`self.isDialogDataAccurate` 1))
              (if _returnvalue_31
                (bind _returnvalue_32 (`self.setHeaderIndex` 8))
                (set `self.HeaderIndex` _returnvalue_32)
                (bind _returnvalue_33 (`self.setArrayIndex` 5))
                (set `self.ArrayIndex` _returnvalue_33)
                (goto _label_3)
                (else
                  (bind _returnvalue_34 (`self.isDialogDataAccurate` 2))
                  (if _returnvalue_34
                    (bind _returnvalue_35 (`self.setHeaderIndex` 9))
                    (set `self.HeaderIndex` _returnvalue_35)
                    (bind _returnvalue_36 (`self.setArrayIndex` 4))
                    (set `self.ArrayIndex` _returnvalue_36)
                    (goto _label_3))))))
          (elif (== (`self.HeaderIndex`) 4)
            (bind _returnvalue_37 (`self.isDialogDataAccurate` 0))
            (if _returnvalue_37
              (bind _returnvalue_38 (`self.setHeaderIndex` 2))
              (set `self.HeaderIndex` _returnvalue_38)
              (bind _returnvalue_39 (`self.setArrayIndex` 2))
              (set `self.ArrayIndex` _returnvalue_39)
              (goto _label_3)
              (else
                (bind _returnvalue_40 (`self.isDialogDataAccurate` 1))
                (if _returnvalue_40
                  (bind _returnvalue_41 (`self.setHeaderIndex` 3))
                  (set `self.HeaderIndex` _returnvalue_41)
                  (bind _returnvalue_42 (`self.setArrayIndex` 2))
                  (set `self.ArrayIndex` _returnvalue_42)
                  (goto _label_3)
                  (else
                    (bind _returnvalue_43 (`self.isDialogDataAccurate` 2))
                    (if _returnvalue_43
                      (bind _returnvalue_44 (`self.setHeaderIndex` 10))
                      (set `self.HeaderIndex` _returnvalue_44)
                      (bind _returnvalue_45 (`self.setArrayIndex` 4))
                      (set `self.ArrayIndex` _returnvalue_45)
                      (bind _returnvalue_46 (`self.getMainCharacter`))
                      (set `MainCharacter.Points` (+ (`MainCharacter.Points` _returnvalue_46) 35) _returnvalue_46)
                      (set `MainCharacter.bGenerous` true _returnvalue_46)
                      (goto _label_3))))))
            (elif (== (`self.HeaderIndex`) 5)
              (bind _returnvalue_47 (`self.isDialogDataAccurate` 0))
              (if _returnvalue_47
                (bind _returnvalue_48 (`self.setHeaderIndex` 2))
                (set `self.HeaderIndex` _returnvalue_48)
                (bind _returnvalue_49 (`self.setArrayIndex` 2))
                (set `self.ArrayIndex` _returnvalue_49)
                (goto _label_3)
                (else
                  (bind _returnvalue_50 (`self.isDialogDataAccurate` 1))
                  (if _returnvalue_50
                    (bind _returnvalue_51 (`self.setHeaderIndex` 3))
                    (set `self.HeaderIndex` _returnvalue_51)
                    (bind _returnvalue_52 (`self.setArrayIndex` 2))
                    (set `self.ArrayIndex` _returnvalue_52)
                    (goto _label_3)
                    (else
                      (bind _returnvalue_53 (`self.isDialogDataAccurate` 2))
                      (if _returnvalue_53
                        (bind _returnvalue_54 (`self.setHeaderIndex` 10))
                        (set `self.HeaderIndex` _returnvalue_54)
                        (bind _returnvalue_55 (`self.setArrayIndex` 4))
                        (set `self.ArrayIndex` _returnvalue_55)
                        (goto _label_3))))))
              (elif (== (`self.HeaderIndex`) 6)
                (bind _returnvalue_56 (`self.isDialogDataAccurate` 0))
                (if _returnvalue_56
                  (bind _returnvalue_57 (`self.setHeaderIndex` 2))
                  (set `self.HeaderIndex` _returnvalue_57)
                  (bind _returnvalue_58 (`self.setArrayIndex` 2))
                  (set `self.ArrayIndex` _returnvalue_58)
                  (goto _label_3)
                  (else
                    (bind _returnvalue_59 (`self.isDialogDataAccurate` 1))
                    (if _returnvalue_59
                      (bind _returnvalue_60 (`self.setHeaderIndex` 3))
                      (set `self.HeaderIndex` _returnvalue_60)
                      (bind _returnvalue_61 (`self.setArrayIndex` 2))
                      (set `self.ArrayIndex` _returnvalue_61)
                      (goto _label_3)
                      (else
                        (bind _returnvalue_62 (`self.isDialogDataAccurate` 2))
                        (if _returnvalue_62
                          (bind _returnvalue_63 (`self.setHeaderIndex` 10))
                          (set `self.HeaderIndex` _returnvalue_63)
                          (bind _returnvalue_64 (`self.setArrayIndex` 4))
                          (set `self.ArrayIndex` _returnvalue_64)
                          (goto _label_3))))))
                (elif (== (`self.HeaderIndex`) 7)
                  (bind _returnvalue_65 (`self.isDialogDataAccurate` 0))
                  (if _returnvalue_65
                    (bind _outactors (`GameplayStatics.GetAllActorsOfClass` "/Script/LittlePsycho.DialogActor"))
                    (for _array_element _outactors
                      (bind _askorzysc_dialog_bp (cast `/Game/Blueprints/KorzyscDialog_BP` _array_element))
                      (`self.K2_DestroyActor` _askorzysc_dialog_bp)
                      (`self.Leave`))
                    (else
                      (bind _returnvalue_66 (`self.isDialogDataAccurate` 1))
                      (if _returnvalue_66
                        (bind _outactors_2 (`GameplayStatics.GetAllActorsOfClass` "/Script/LittlePsycho.DialogActor"))
                        (for _array_element_2 _outactors_2
                          (bind _askorzysc_dialog_bp_2 (cast `/Game/Blueprints/KorzyscDialog_BP` _array_element_2))
                          (`self.K2_DestroyActor` _askorzysc_dialog_bp_2)
                          (`self.Leave`))
                        (else
                          (bind _returnvalue_67 (`self.isDialogDataAccurate` 2))
                          (if _returnvalue_67
                            (bind _outactors_3 (`GameplayStatics.GetAllActorsOfClass` "/Script/LittlePsycho.DialogActor"))
                            (for _array_element_3 _outactors_3
                              (bind _askorzysc_dialog_bp_3 (cast `/Game/Blueprints/KorzyscDialog_BP` _array_element_3))
                              (`self.K2_DestroyActor` _askorzysc_dialog_bp_3)
                              (`self.Leave`)))))))
                  (elif (== (`self.HeaderIndex`) 8)
                    (bind _returnvalue_68 (`self.isDialogDataAccurate` 0))
                    (if _returnvalue_68
                      (bind _returnvalue_69 (`self.setHeaderIndex` 11))
                      (set `self.HeaderIndex` _returnvalue_69)
                      (bind _returnvalue_70 (`self.setArrayIndex` 4))
                      (set `self.ArrayIndex` _returnvalue_70)
                      (goto _label_3)
                      (else
                        (bind _returnvalue_71 (`self.isDialogDataAccurate` 1))
                        (if _returnvalue_71
                          (bind _returnvalue_72 (`self.setHeaderIndex` 12))
                          (set `self.HeaderIndex` _returnvalue_72)
                          (bind _returnvalue_73 (`self.setArrayIndex` 4))
                          (set `self.ArrayIndex` _returnvalue_73)
                          (goto _label_3)
                          (else
                            (bind _returnvalue_74 (`self.isDialogDataAccurate` 2))
                            (if _returnvalue_74
                              (bind _returnvalue_75 (`self.setHeaderIndex` 13))
                              (set `self.HeaderIndex` _returnvalue_75)
                              (bind _returnvalue_76 (`self.setArrayIndex` 4))
                              (set `self.ArrayIndex` _returnvalue_76)
                              (goto _label_3))))))
                    (elif (== (`self.HeaderIndex`) 9)
                      (bind _returnvalue_77 (`self.isDialogDataAccurate` 0))
                      (if _returnvalue_77
                        (bind _outactors_4 (`GameplayStatics.GetAllActorsOfClass` "/Script/LittlePsycho.DialogActor"))
                        (for _array_element_4 _outactors_4
                          (bind _askorzysc_dialog_bp_4 (cast `/Game/Blueprints/KorzyscDialog_BP` _array_element_4))
                          (`self.K2_DestroyActor` _askorzysc_dialog_bp_4)
                          (`self.Leave`))
                        (else
                          (bind _returnvalue_78 (`self.isDialogDataAccurate` 1))
                          (if _returnvalue_78
                            (bind _outactors_5 (`GameplayStatics.GetAllActorsOfClass` "/Script/LittlePsycho.DialogActor"))
                            (for _array_element_5 _outactors_5
                              (bind _askorzysc_dialog_bp_5 (cast `/Game/Blueprints/KorzyscDialog_BP` _array_element_5))
                              (`self.K2_DestroyActor` _askorzysc_dialog_bp_5)
                              (`self.Leave`))
                            (else
                              (bind _returnvalue_79 (`self.isDialogDataAccurate` 2))
                              (if _returnvalue_79
                                (bind _outactors_6 (`GameplayStatics.GetAllActorsOfClass` "/Script/LittlePsycho.DialogActor"))
                                (for _array_element_6 _outactors_6
                                  (bind _askorzysc_dialog_bp_6 (cast `/Game/Blueprints/KorzyscDialog_BP` _array_element_6))
                                  (`self.K2_DestroyActor` _askorzysc_dialog_bp_6)
                                  (`self.Leave`)))))))
                      (elif (== (`self.HeaderIndex`) 10)
                        (bind _returnvalue_80 (`self.isDialogDataAccurate` 0))
                        (if _returnvalue_80
                          (bind _outactors_7 (`GameplayStatics.GetAllActorsOfClass` "/Script/LittlePsycho.DialogActor"))
                          (for _array_element_7 _outactors_7
                            (bind _askorzysc_dialog_bp_7 (cast `/Game/Blueprints/KorzyscDialog_BP` _array_element_7))
                            (`self.K2_DestroyActor` _askorzysc_dialog_bp_7)
                            (`self.Leave`))
                          (else
                            (bind _returnvalue_81 (`self.isDialogDataAccurate` 1))
                            (if _returnvalue_81
                              (bind _outactors_8 (`GameplayStatics.GetAllActorsOfClass` "/Script/LittlePsycho.DialogActor"))
                              (for _array_element_8 _outactors_8
                                (bind _askorzysc_dialog_bp_8 (cast `/Game/Blueprints/KorzyscDialog_BP` _array_element_8))
                                (`self.K2_DestroyActor` _askorzysc_dialog_bp_8)
                                (`self.Leave`))
                              (else
                                (bind _returnvalue_82 (`self.isDialogDataAccurate` 2))
                                (if _returnvalue_82
                                  (bind _outactors_9 (`GameplayStatics.GetAllActorsOfClass` "/Script/LittlePsycho.DialogActor"))
                                  (for _array_element_9 _outactors_9
                                    (bind _askorzysc_dialog_bp_9 (cast `/Game/Blueprints/KorzyscDialog_BP` _array_element_9))
                                    (`self.K2_DestroyActor` _askorzysc_dialog_bp_9)
                                    (`self.Leave`)))))))
                        (elif (== (`self.HeaderIndex`) 11)
                          (bind _returnvalue_83 (`self.isDialogDataAccurate` 0))
                          (if _returnvalue_83
                            (bind _outactors_10 (`GameplayStatics.GetAllActorsOfClass` "/Script/LittlePsycho.DialogActor"))
                            (for _array_element_10 _outactors_10
                              (bind _askorzysc_dialog_bp_10 (cast `/Game/Blueprints/KorzyscDialog_BP` _array_element_10))
                              (`self.K2_DestroyActor` _askorzysc_dialog_bp_10)
                              (`self.Leave`))
                            (else
                              (bind _returnvalue_84 (`self.isDialogDataAccurate` 1))
                              (if _returnvalue_84
                                (bind _outactors_11 (`GameplayStatics.GetAllActorsOfClass` "/Script/LittlePsycho.DialogActor"))
                                (for _array_element_11 _outactors_11
                                  (bind _askorzysc_dialog_bp_11 (cast `/Game/Blueprints/KorzyscDialog_BP` _array_element_11))
                                  (`self.K2_DestroyActor` _askorzysc_dialog_bp_11)
                                  (`self.Leave`))
                                (else
                                  (bind _returnvalue_85 (`self.isDialogDataAccurate` 2))
                                  (if _returnvalue_85
                                    (bind _outactors_12 (`GameplayStatics.GetAllActorsOfClass` "/Script/LittlePsycho.DialogActor"))
                                    (for _array_element_12 _outactors_12
                                      (bind _askorzysc_dialog_bp_12 (cast `/Game/Blueprints/KorzyscDialog_BP` _array_element_12))
                                      (`self.K2_DestroyActor` _askorzysc_dialog_bp_12)
                                      (`self.Leave`)))))))
                          (elif (== (`self.HeaderIndex`) 12)
                            (bind _returnvalue_86 (`self.isDialogDataAccurate` 0))
                            (if _returnvalue_86
                              (bind _outactors_13 (`GameplayStatics.GetAllActorsOfClass` "/Script/LittlePsycho.DialogActor"))
                              (for _array_element_13 _outactors_13
                                (bind _askorzysc_dialog_bp_13 (cast `/Game/Blueprints/KorzyscDialog_BP` _array_element_13))
                                (`self.K2_DestroyActor` _askorzysc_dialog_bp_13)
                                (`self.Leave`))
                              (else
                                (bind _returnvalue_87 (`self.isDialogDataAccurate` 1))
                                (if _returnvalue_87
                                  (bind _outactors_14 (`GameplayStatics.GetAllActorsOfClass` "/Script/LittlePsycho.DialogActor"))
                                  (for _array_element_14 _outactors_14
                                    (bind _askorzysc_dialog_bp_14 (cast `/Game/Blueprints/KorzyscDialog_BP` _array_element_14))
                                    (`self.K2_DestroyActor` _askorzysc_dialog_bp_14)
                                    (`self.Leave`))
                                  (else
                                    (bind _returnvalue_88 (`self.isDialogDataAccurate` 2))
                                    (if _returnvalue_88
                                      (bind _outactors_15 (`GameplayStatics.GetAllActorsOfClass` "/Script/LittlePsycho.DialogActor"))
                                      (for _array_element_15 _outactors_15
                                        (bind _askorzysc_dialog_bp_15 (cast `/Game/Blueprints/KorzyscDialog_BP` _array_element_15))
                                        (`self.K2_DestroyActor` _askorzysc_dialog_bp_15)
                                        (`self.Leave`)))))))
                            (elif (== (`self.HeaderIndex`) 13)
                              (bind _returnvalue_89 (`self.isDialogDataAccurate` 0))
                              (if _returnvalue_89
                                (bind _outactors_16 (`GameplayStatics.GetAllActorsOfClass` "/Script/LittlePsycho.DialogActor"))
                                (for _array_element_16 _outactors_16
                                  (bind _askorzysc_dialog_bp_16 (cast `/Game/Blueprints/KorzyscDialog_BP` _array_element_16))
                                  (`self.K2_DestroyActor` _askorzysc_dialog_bp_16)
                                  (`self.Leave`))
                                (else
                                  (bind _returnvalue_90 (`self.isDialogDataAccurate` 1))
                                  (if _returnvalue_90
                                    (bind _outactors_17 (`GameplayStatics.GetAllActorsOfClass` "/Script/LittlePsycho.DialogActor"))
                                    (for _array_element_17 _outactors_17
                                      (bind _askorzysc_dialog_bp_17 (cast `/Game/Blueprints/KorzyscDialog_BP` _array_element_17))
                                      (`self.K2_DestroyActor` _askorzysc_dialog_bp_17)
                                      (`self.Leave`))
                                    (else
                                      (bind _returnvalue_91 (`self.isDialogDataAccurate` 2))
                                      (if _returnvalue_91
                                        (bind _outactors_18 (`GameplayStatics.GetAllActorsOfClass` "/Script/LittlePsycho.DialogActor"))
                                        (for _array_element_18 _outactors_18
                                          (bind _askorzysc_dialog_bp_18 (cast `/Game/Blueprints/KorzyscDialog_BP` _array_element_18))
                                          (`self.K2_DestroyActor` _askorzysc_dialog_bp_18)
                                          (`self.Leave`))))))))))))))))))))))

(event `Answer2`
  (`self.setChosenNumber` 1)
  (goto _label_2))

(event `Answer3`
  (`self.setChosenNumber` 2)
  (goto _label_2))

(fn `UserConstructionScript`
  ;[1 1 1] Header Configuration
  (bind _output_get (set `self.Header Start` "Dlaczego wybrałeś stratę?"))
  (set `self.Header 1` "Świadomy czy nie, to nadal był wybór, którego konsekwencje musisz ponieść.")
  (set `self.Header 2` "To prawda. Aczkolwiek nie zawsze. Co jesteś gotów stracić, by móc uleczyć siostrę?")
  (set `self.Header 3` "To prawda. Co jesteś gotów stracić, by móc uleczyć siostrę?")
  (set `self.Header 4` "A więc, ponawiam pytanie: Dlaczego wybrałeś stratę? Jeśli odpowiesz, będziesz mógł pójść dalej.")
  (set `self.Header 5` "Zaliczoną próbę, czyż nie? A więc, ponawiam pytanie: Dlaczego wybrałeś stratę? Jeśli odpowiesz, będziesz mógł pójść dalej.")
  (set `self.Header 6` "Niech to będzie niespodzianka. A więc, ponawiam pytanie: Dlaczego wybrałeś stratę? Jeśli odpowiesz, będziesz mógł pójść dalej.")
  (set `self.Header 7` "Rozumiem, kroczysz dobrą ścieżką.")
  (set `self.Header 8` "Nie do końca takie niemożliwe. Ale tę drogę musisz odkryć sam.")
  (set `self.Header 9` "To smutne. Nie podoba mi się Twoje postępowanie.")
  (set `self.Header 12` "Och, rozumiem. To dobrze.")
  (set `self.Header 13` "Nie musisz, ale nie mogę Ci pomóc. Idź już.")
  (set `self.Header 14` "Nie mogę. Idź już.")
  (set `self.Header 15` "Stracę wszystko.")
  (set `self.CurrentNPCResponse` _output_get)
  ;[1 1 1] Dialog Data Configuration
  (set `self.Odp 0.1` "Myślałem, że to wszystko jedno, w którą stronę pójdę.")
  (set `self.Odp 0.2` "Lepiej stracić i dać innej istocie szczęście.")
  (set `self.Odp 0.3` "Obecnie coraz mniej ludzi robi coś bezinteresownie.")
  (set `self.Odp 1.1` "No dobra, chociaż mało to ma sensu, bo to tylko sen.")
  (set `self.Odp 1.2` "A co będę miał z tego, że z tobą porozmawiam?")
  (set `self.Odp 1.3` "A jakie to będą konsekwencje?")
  (set `self.Odp 2.1` "Umowa była taka, że mam oddać życie za życzenie. I jestem gotów tyle dać.")
  (set `self.Odp 2.2` "Wolałbym stracić jak najmniej, ale wiem, że to niemożliwe.")
  (set `self.Odp 2.3` "Nic.")
  (set `self.Odp4.1` "Lepiej stracić i dać drugiej istocie szczęście.")
  (set `self.Odp4.2` "Obecnie coraz mniej ludzi robi coś bezinteresownie.")
  (set `self.Odp4.3` "Lubię dawać.")
  (set `self.Odp 7.1` "[Odejdź]")
  (set `self.Odp 7.2` "[Przebiegnij przez zjawę]")
  (set `self.Odp 7.3` "I tak to tylko sen. [Odejdź]")
  (set `self.Odp 8.1` "Istnieje inne wyjście? Naprawdę? Nie muszę umierać?")
  (set `self.Odp 8.2` "Nie pomożesz mi?")
  (set `self.Odp 8.3` "Przecież nic nie stracisz, pomagając mi.")
  (set `self.Odp15.1` "I ty śmiesz mnie pouczać o stracie i korzyści?! [Odejdź]")
  (set `self.Odp15.2` "Rozumiem. [Odejdź]")
  (set `self.Odp15.3` "I tyle jeśli chodzi o naukę. [Odejdź]")
  (set `self.HeaderIndex` 0)
  (set `self.ArrayIndex` 0))