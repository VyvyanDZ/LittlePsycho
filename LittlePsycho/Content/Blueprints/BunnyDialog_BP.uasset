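; Branching Polish-language NPC dialogue about a moral choice over sick rabbits and the flowers they eat.
; Overlap disables player input and opens DialogInterface2 with a cursor; leaving restores both.
; Three answer events share one hardcoded branch tree, using HeaderIndex and ArrayIndex to select NPC line and replies from construction-script strings.
; Choices can deduct MainCharacter Points and set outcome flags like KilledIll, LeaveAlone and FlowersWasTaken.
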(event `self.ReceiveActorBeginOverlap`
  (params (OtherActor :type "Actor Object Reference"))
  ;[1 1 1] Handle input and camera
  (bind _asmain_character (cast `MainCharacter` OtherActor))
  (bind _returnvalue (`self.setMainCharacter` _asmain_character))
  (bind _returnvalue_2 (`GameplayStatics.GetPlayerController` _returnvalue))
  (`self.DisableInput` _returnvalue _returnvalue_2)
  (bind _returnvalue_3 (`|CreateWidget` "/Game/Dialog/DialogInterface2.DialogInterface2_C" _returnvalue_2))
  (bind _output_get (set `self.DialogInterface` _returnvalue_3))
  (`TextBlock.SetText` (`/Game/Dialog/DialogInterface2.Text_Block_1` _output_get) "")
  (set `self.ButtonText` (select `int` (`self.ArrayIndex`) :`0` (`|MakeArray` (`self.Odp 0.1`) (`self.Odp 0.2`) (`self.Odp 0.3`)) :`1` (`|MakeArray` (`self.Odp 1.1`) (`self.Odp 1.2`) (`self.Odp 1.3`)) :`2` (`|MakeArray` (`self.Odp 2.1`) (`self.Odp 2.2`) (`self.Odp 2.3`)) :`3` (`|MakeArray` (`self.Odp4.1`) (`self.Odp4.2`) (`self.Odp4.3`)) :`4` (`|MakeArray` (`self.Odp 7.1`) (`self.Odp 7.2`) (`self.Odp 7.3`)) :`5` (`|MakeArray` (`self.Odp 9.1`) (`self.Odp 9.2`) (`self.Odp 9.3`)) :`6` (`|MakeArray` (`self.Odp 10.1`) (`self.Odp 10.2`) (`self.Odp 10.3`))))
  (`UserWidget.AddToViewport` _output_get 0)
  (set `PlayerController.bShowMouseCursor` true _returnvalue_2))

(event `self.ReceiveActorEndOverlap`
  (params (OtherActor :type "Actor Object Reference"))
  (bind _returnvalue (`GameplayStatics.GetPlayerController` 0))
  ;[1 1 1] Handle input and camera
  (`Widget.RemoveFromParent` (`self.DialogInterface`) :!label _label)
  (bind _returnvalue_2 (`self.getMainCharacter`))
  (`self.EnableInput` _returnvalue_2 _returnvalue)
  (set `PlayerController.bShowMouseCursor` false _returnvalue))

(event `Leave`
  ;[1 1 1] Handle input and camera
  (`self.endDialog`)
  (goto _label))

(event `Answer 1`
  (`self.setChosenNumber` 0)
  (if (== (`self.HeaderIndex`) 0) :!label _label_2
    (bind _returnvalue (`self.isDialogDataAccurate` 0))
    (if _returnvalue
      (bind _returnvalue_2 (`self.setHeaderIndex` 1))
      (set `self.HeaderIndex` _returnvalue_2)
      (bind _returnvalue_3 (`self.setArrayIndex` 1))
      (set `self.ArrayIndex` _returnvalue_3)
      (set `self.ButtonText` (select `int` (`self.ArrayIndex`) :`0` (`|MakeArray` (`self.Odp 0.1`) (`self.Odp 0.2`) (`self.Odp 0.3`)) :`1` (`|MakeArray` (`self.Odp 1.1`) (`self.Odp 1.2`) (`self.Odp 1.3`)) :`2` (`|MakeArray` (`self.Odp 2.1`) (`self.Odp 2.2`) (`self.Odp 2.3`)) :`3` (`|MakeArray` (`self.Odp4.1`) (`self.Odp4.2`) (`self.Odp4.3`)) :`4` (`|MakeArray` (`self.Odp 7.1`) (`self.Odp 7.2`) (`self.Odp 7.3`)) :`5` (`|MakeArray` (`self.Odp 9.1`) (`self.Odp 9.2`) (`self.Odp 9.3`)) :`6` (`|MakeArray` (`self.Odp 10.1`) (`self.Odp 10.2`) (`self.Odp 10.3`))) :!label _label_3)
      (set `self.CurrentNPCResponse` (select `int` (`self.HeaderIndex`) :`0` (`self.Header Start`) :`1` (`self.Header 1`) :`2` (`self.Header 2`) :`3` (`self.Header 3`) :`4` (`self.Header 4`) :`5` (`self.Header 5`) :`6` (`self.Header 7`) :`7` (`self.Header 8`) :`8` (`self.Header 9`) :`9` (`self.Header 10`)))
      (else
        (bind _returnvalue_4 (`self.isDialogDataAccurate` 1))
        (if _returnvalue_4
          (bind _returnvalue_5 (`self.setHeaderIndex` 2))
          (set `self.HeaderIndex` _returnvalue_5)
          (bind _returnvalue_6 (`self.setArrayIndex` 2))
          (set `self.ArrayIndex` _returnvalue_6)
          (goto _label_3)
          (else
            (bind _returnvalue_7 (`self.isDialogDataAccurate` 2))
            (if _returnvalue_7
              (bind _returnvalue_8 (`self.setHeaderIndex` 3))
              (set `self.HeaderIndex` _returnvalue_8)
              (bind _returnvalue_9 (`self.setArrayIndex` 2))
              (set `self.ArrayIndex` _returnvalue_9)
              (goto _label_3))))))
    (elif (== (`self.HeaderIndex`) 1)
      (bind _returnvalue_10 (`self.isDialogDataAccurate` 0))
      (if _returnvalue_10
        (bind _returnvalue_11 (`self.setHeaderIndex` 4))
        (set `self.HeaderIndex` _returnvalue_11)
        (bind _returnvalue_12 (`self.setArrayIndex` 3))
        (set `self.ArrayIndex` _returnvalue_12)
        (goto _label_3)
        (else
          (bind _returnvalue_13 (`self.isDialogDataAccurate` 1))
          (if _returnvalue_13
            (bind _returnvalue_14 (`self.setHeaderIndex` 5))
            (set `self.HeaderIndex` _returnvalue_14)
            (bind _returnvalue_15 (`self.setArrayIndex` 2))
            (set `self.ArrayIndex` _returnvalue_15)
            (goto _label_3)
            (else
              (bind _returnvalue_16 (`self.isDialogDataAccurate` 2))
              (if _returnvalue_16
                (bind _returnvalue_17 (`self.setHeaderIndex` 4))
                (set `self.HeaderIndex` _returnvalue_17)
                (bind _returnvalue_18 (`self.setArrayIndex` 3))
                (set `self.ArrayIndex` _returnvalue_18)
                (goto _label_3))))))
      (elif (== (`self.HeaderIndex`) 2)
        (bind _returnvalue_19 (`self.isDialogDataAccurate` 0))
        (if _returnvalue_19
          (bind _returnvalue_20 (`self.setHeaderIndex` 6))
          (set `self.HeaderIndex` _returnvalue_20)
          (bind _returnvalue_21 (`self.setArrayIndex` 4))
          (set `self.ArrayIndex` _returnvalue_21)
          (goto _label_3)
          (else
            (bind _returnvalue_22 (`self.isDialogDataAccurate` 1))
            (if _returnvalue_22
              (bind _returnvalue_23 (`self.setHeaderIndex` 7))
              (set `self.HeaderIndex` _returnvalue_23)
              (bind _returnvalue_24 (`self.setArrayIndex` 3))
              (set `self.ArrayIndex` _returnvalue_24)
              (goto _label_3)
              (else
                (bind _returnvalue_25 (`self.isDialogDataAccurate` 2))
                (if _returnvalue_25
                  (bind _returnvalue_26 (`self.setHeaderIndex` 8))
                  (set `self.HeaderIndex` _returnvalue_26)
                  (bind _returnvalue_27 (`self.setArrayIndex` 5))
                  (set `self.ArrayIndex` _returnvalue_27)
                  (goto _label_3))))))
        (elif (== (`self.HeaderIndex`) 3)
          (bind _returnvalue_28 (`self.isDialogDataAccurate` 0))
          (if _returnvalue_28
            (bind _returnvalue_29 (`self.setHeaderIndex` 6))
            (set `self.HeaderIndex` _returnvalue_29)
            (bind _returnvalue_30 (`self.setArrayIndex` 4))
            (set `self.ArrayIndex` _returnvalue_30)
            (goto _label_3)
            (else
              (bind _returnvalue_31 (`self.isDialogDataAccurate` 1))
              (if _returnvalue_31
                (bind _returnvalue_32 (`self.setHeaderIndex` 7))
                (set `self.HeaderIndex` _returnvalue_32)
                (bind _returnvalue_33 (`self.setArrayIndex` 3))
                (set `self.ArrayIndex` _returnvalue_33)
                (goto _label_3)
                (else
                  (bind _returnvalue_34 (`self.isDialogDataAccurate` 2))
                  (if _returnvalue_34
                    (bind _returnvalue_35 (`self.setHeaderIndex` 8))
                    (set `self.HeaderIndex` _returnvalue_35)
                    (bind _returnvalue_36 (`self.setArrayIndex` 5))
                    (set `self.ArrayIndex` _returnvalue_36)
                    (goto _label_3))))))
          (elif (== (`self.HeaderIndex`) 4)
            (bind _returnvalue_37 (`self.isDialogDataAccurate` 0))
            (if _returnvalue_37
              (bind _returnvalue_38 (`self.getMainCharacter`))
              (set `MainCharacter.Points` (- (`MainCharacter.Points` _returnvalue_38) 100) _returnvalue_38)
              (set `MainCharacter.bFlowersWasTaken` true _returnvalue_38)
              (set `MainCharacter.bLeaveAlone` true _returnvalue_38)
              (`self.Leave`)
              (else
                (bind _returnvalue_39 (`self.isDialogDataAccurate` 1))
                (if _returnvalue_39
                  (bind _returnvalue_40 (`self.setHeaderIndex` 9))
                  (set `self.HeaderIndex` _returnvalue_40)
                  (bind _returnvalue_41 (`self.setArrayIndex` 6))
                  (set `self.ArrayIndex` _returnvalue_41)
                  (bind _returnvalue_42 (`self.getMainCharacter`))
                  (set `MainCharacter.bForcedToTakeCare` true _returnvalue_42)
                  (goto _label_3)
                  (else
                    (bind _returnvalue_43 (`self.isDialogDataAccurate` 2))
                    (if _returnvalue_43
                      (bind _returnvalue_44 (`self.getMainCharacter`))
                      (set `MainCharacter.Points` (- (`MainCharacter.Points` _returnvalue_44) 50) _returnvalue_44)
                      (set `MainCharacter.bKilledIll` true _returnvalue_44)
                      (`self.Leave`))))))
            (elif (== (`self.HeaderIndex`) 5)
              (bind _returnvalue_45 (`self.isDialogDataAccurate` 0))
              (if _returnvalue_45
                (bind _returnvalue_46 (`self.setHeaderIndex` 6))
                (set `self.HeaderIndex` _returnvalue_46)
                (bind _returnvalue_47 (`self.setArrayIndex` 4))
                (set `self.ArrayIndex` _returnvalue_47)
                (goto _label_3)
                (else
                  (bind _returnvalue_48 (`self.isDialogDataAccurate` 1))
                  (if _returnvalue_48
                    (bind _returnvalue_49 (`self.setHeaderIndex` 7))
                    (set `self.HeaderIndex` _returnvalue_49)
                    (bind _returnvalue_50 (`self.setArrayIndex` 3))
                    (set `self.ArrayIndex` _returnvalue_50)
                    (goto _label_3)
                    (else
                      (bind _returnvalue_51 (`self.isDialogDataAccurate` 2))
                      (if _returnvalue_51
                        (bind _returnvalue_52 (`self.setHeaderIndex` 8))
                        (set `self.HeaderIndex` _returnvalue_52)
                        (bind _returnvalue_53 (`self.setArrayIndex` 5))
                        (set `self.ArrayIndex` _returnvalue_53)
                        (goto _label_3))))))
              (elif (== (`self.HeaderIndex`) 6)
                (bind _returnvalue_54 (`self.isDialogDataAccurate` 0))
                (if _returnvalue_54
                  (bind _returnvalue_55 (`self.getMainCharacter`))
                  (set `MainCharacter.Points` (- (`MainCharacter.Points` _returnvalue_55) 100) _returnvalue_55)
                  (set `MainCharacter.bLeaveAlone` true _returnvalue_55)
                  (`self.Leave`)
                  (else
                    (bind _returnvalue_56 (`self.isDialogDataAccurate` 1))
                    (if _returnvalue_56
                      (bind _returnvalue_57 (`self.setHeaderIndex` 9))
                      (set `self.HeaderIndex` _returnvalue_57)
                      (bind _returnvalue_58 (`self.setArrayIndex` 6))
                      (set `self.ArrayIndex` _returnvalue_58)
                      (bind _returnvalue_59 (`self.getMainCharacter`))
                      (set `MainCharacter.bForcedToTakeCare` true _returnvalue_59)
                      (goto _label_3)
                      (else
                        (bind _returnvalue_60 (`self.isDialogDataAccurate` 2))
                        (if _returnvalue_60
                          (bind _returnvalue_61 (`self.getMainCharacter`))
                          (set `MainCharacter.Points` (- (`MainCharacter.Points` _returnvalue_61) 50) _returnvalue_61)
                          (set `MainCharacter.bFlowersWasTaken` true _returnvalue_61)
                          (set `MainCharacter.bKilledIll` true _returnvalue_61)
                          (`self.Leave`))))))
                (elif (== (`self.HeaderIndex`) 7)
                  (bind _returnvalue_62 (`self.isDialogDataAccurate` 0))
                  (if _returnvalue_62
                    (bind _returnvalue_63 (`self.getMainCharacter`))
                    (set `MainCharacter.Points` (- (`MainCharacter.Points` _returnvalue_63) 100) _returnvalue_63)
                    (set `MainCharacter.bFlowersWasTaken` true _returnvalue_63)
                    (set `MainCharacter.bLeaveAlone` true _returnvalue_63)
                    (`self.Leave`)
                    (else
                      (bind _returnvalue_64 (`self.isDialogDataAccurate` 1))
                      (if _returnvalue_64
                        (bind _returnvalue_65 (`self.setHeaderIndex` 9))
                        (set `self.HeaderIndex` _returnvalue_65)
                        (bind _returnvalue_66 (`self.setArrayIndex` 6))
                        (set `self.ArrayIndex` _returnvalue_66)
                        (bind _returnvalue_67 (`self.getMainCharacter`))
                        (set `MainCharacter.bForcedToTakeCare` true _returnvalue_67)
                        (else
                          (bind _returnvalue_68 (`self.isDialogDataAccurate` 2))
                          (if _returnvalue_68
                            (bind _returnvalue_69 (`self.getMainCharacter`))
                            (set `MainCharacter.Points` (- (`MainCharacter.Points` _returnvalue_69) 50) _returnvalue_69)
                            (set `MainCharacter.bKilledIll` true _returnvalue_69)
                            (`self.Leave`))))))
                  (elif (== (`self.HeaderIndex`) 8)
                    (bind _returnvalue_70 (`self.isDialogDataAccurate` 0))
                    (if _returnvalue_70
                      (bind _returnvalue_71 (`self.getMainCharacter`))
                      (set `MainCharacter.Points` (- (`MainCharacter.Points` _returnvalue_71) 25) _returnvalue_71)
                      (set `MainCharacter.bKilledIll` true _returnvalue_71)
                      (`self.Leave`)
                      (else
                        (bind _returnvalue_72 (`self.isDialogDataAccurate` 1))
                        (if _returnvalue_72
                          (bind _returnvalue_73 (`self.setHeaderIndex` 9))
                          (set `self.HeaderIndex` _returnvalue_73)
                          (bind _returnvalue_74 (`self.setArrayIndex` 6))
                          (set `self.ArrayIndex` _returnvalue_74)
                          (bind _returnvalue_75 (`self.getMainCharacter`))
                          (set `MainCharacter.bForcedToTakeCare` true _returnvalue_75)
                          (goto _label_3)
                          (else
                            (bind _returnvalue_76 (`self.isDialogDataAccurate` 2))
                            (if _returnvalue_76
                              (bind _returnvalue_77 (`self.getMainCharacter`))
                              (set `MainCharacter.Points` (- (`MainCharacter.Points` _returnvalue_77) 50) _returnvalue_77)
                              (set `MainCharacter.bFlowersWasTaken` true _returnvalue_77)
                              (set `MainCharacter.bLeaveAlone` true _returnvalue_77)
                              (`self.Leave`))))))
                    (elif (== (`self.HeaderIndex`) 9)
                      (bind _returnvalue_78 (`self.isDialogDataAccurate` 0))
                      (if _returnvalue_78
                        (`self.Leave`)
                        (else
                          (bind _returnvalue_79 (`self.isDialogDataAccurate` 1))
                          (if _returnvalue_79
                            (bind _returnvalue_80 (`self.getMainCharacter`))
                            (set `MainCharacter.Points` (- (`MainCharacter.Points` _returnvalue_80) 10) _returnvalue_80)
                            (`self.Leave`)
                            (else
                              (bind _returnvalue_81 (`self.isDialogDataAccurate` 2))
                              (if _returnvalue_81
                                (bind _returnvalue_82 (`self.getMainCharacter`))
                                (set `MainCharacter.bWalkThroughSecond` true _returnvalue_82)
                                (`self.Leave`)))))))))))))))))

(event `Answer 2`
  (`self.setChosenNumber` 1)
  (goto _label_2))

(event `Answer 3`
  (`self.setChosenNumber` 2)
  (goto _label_2))

(fn `UserConstructionScript`
  ;[1 1 1] Header Configuration
  (bind _output_get (set `self.Header Start` "Czy możesz mi pomóc?"))
  (set `self.Header 1` "Z nieba mi spadłeś! Widzisz to malutkie stadko króliczków nieopodal? Opiekuję się nimi od jakiegoś czasu, ale niestety kilka z nich zachorowało. O, widzisz? Tamte dwa w rogu, przy tych kolorowych kwiatach.")
  (set `self.Header 2` "To nie wchodzi w grę. Nie poradzę sobie sama. Nie wiem kompletnie co robić! Jeśli odseparuję te dwa króliki, nie mam gwarancji, że przeżyją. Nie chcę też skracać ich cierpień, nie potrafię! Jeśli zostaną w stadzie, zachorują wszystkie. To moi przyjaciele, czuję się taka bezsilna!")
  (set `self.Header 3` "Wiem, przepraszam, że Cię zatrzymuję. Ale proszę, nie wiem kompletnie, co robić! Widzisz to malutkie stadko króliczków nieopodal? Opiekuję się nimi od jakiegoś czasu, ale niestety kilka z nich zachorowało. O, widzisz? Tamte dwa w rogu, przy tych kolorowych kwiatach.  Jeśli odseparuję te dwa króliki, nie mam gwarancji, że przeżyją. Nie chcę też skracać ich cierpień, nie potrafię! Jeśli zostaną w stadzie, zachorują wszystkie. To moi przyjaciele, czuję się taka bezsilna!")
  (set `self.Header 4` "Te króliki żywią się tylko tymi kwiatami. Bardzo się staram powiększyć ich liczbę, ale mi się nie udaje. Ledwo ich starcza... Naprawdę chciałabym, ale nie mogę Ci dać ani jednego. Proszę tylko o radę... Mogę odseparować chore osobniki, ale wtedy najpewniej ich należycie nie dopilnuję. Z kolei jeśli nic nie zrobię, prawdopodobnie zachoruje całe stado. A zabijanie... Wzdrygam się na samą myśl. Co proponujesz?")
  (set `self.Header 5` "Może możesz jakoś rozwiązać mój problem? Każde rozwiązanie ma złe i dobre strony, a jak sobie pomyślę, że musiałabym dla dobra stada poświęcić tych dwojga... Nie chcę nawet o tym myśleć, nie dam rady! To wykluczone! Z kolei odseparowanie też nie wchodzi w grę, bo bez tych kwiatów nie przeżyją. Żywią się tylko nimi. A jeśli zarażą pozostałych w stadzie... To chyba bardziej okropne od poświęcenia dla dobra ogółu.")
  (set `self.Header 7` "To dodatkowy czas, który muszę poświęcić na opiekę nad nimi. Muszę pójść, zająć się nimi, wrócić i dopilnować reszty stada, by nie dopadła ich zaraza. To bardzo ciężka praca.")
  (set `self.Header 8` "Więc co proponujesz?")
  (set `self.Header 9` "Jesteś pewny? To według Ciebie jedyne wyjście? Może to da się rozwiązać jakoś inaczej?")
  (set `self.Header 10` "Masz rację! Powinnam brać odpowiedzialność za swoich podopiecznych!")
  (set `self.CurrentNPCResponse` _output_get)
  ;[1 1 1] Dialog Data Configuration
  (set `self.Odp 0.1` "Oczywiście, w czym mogę pomóc?")
  (set `self.Odp 0.2` "To może zrobimy tak, ty mi zaliczysz próbę, a ja sobie pójdę...?")
  (set `self.Odp 0.3` "Nie mam na to czasu, muszę dostać się do Drzewa Mądrości, przesuń się!")
  (set `self.Odp 1.1` "Czy one jedzą te kolorowe kwiatki? Moja siostra je uwielbia. Pomogę Ci, jeśli oddasz mi jeden.")
  (set `self.Odp 1.2` "I...Jak mogę pomóc?")
  (set `self.Odp 1.3` "Myślałem, że masz jakiś problem, a tobie chodzi tylko o jakieś króliki? W zamian chcę otrzymać trochę tych kwiatów, które jedzą. Moja siostra bardzo je lubi.")
  (set `self.Odp 2.1` "Nie masz gwarancji, że przeżyją? A czemu po prostu nie będziesz im zrywać tych kwiatków i zanosić w nowe miejsce pobytu?")
  (set `self.Odp 2.2` "Nie można zabić tych zwierząt! Na pewno da się jakoś je uratować. Wymyślę coś wzamian za kilka ulubionych kwiatów mojej siostry.")
  (set `self.Odp 2.3` "Mogę ukrócić ich cierpienia, by nie umierały w męczarniach.")
  (set `self.Odp4.1` "Nic. Wezmę po prostu kwiaty, którymi się żywią i po kłopocie. To przecież tylko sen. [Zabierz kwiaty i zostaw zwierzęta na pastwę losu]")
  (set `self.Odp4.2` "Odseparujmy je. Niech nie rozprzestrzeniają choroby w stadzie. Będziesz im przynosić jedzenie. [Odseparuj zwierzęta od stada].")
  (set `self.Odp4.3` "Po prostu je zabiję. [Zabij chore króliki]")
  (set `self.Odp 7.1` "Skoro nie masz czasu się nimi zająć, zostaw je z resztą stada. [Nie rozdzielaj stada]")
  (set `self.Odp 7.2` "Dodatkowy czas? To przecież twoi podopieczni! Lamentujesz zamiast wziąć odpowiedzialność i zrobić coś konstruktywnego. Bierz się do roboty!")
  (set `self.Odp 7.3` "Więc najlepiej nic nie rób. Ja się tym zajmę. Będziesz miała nauczkę, żeby podejmować działania samodzielnie. [Zabij chore zwierzęta i zabierz część kwiatów dla siostry]")
  (set `self.Odp 9.1` "Nie, po prostu je zabiję. [Zabij chore króliki]")
  (set `self.Odp 9.2` "Odseparujmy je. Niech nie rozprzestrzeniają choroby w stadzie. Będziesz im przynosić jedzenie. [Odseparuj zwierzęta od stada]")
  (set `self.Odp 9.3` "Wiesz co, zmieniłem zdanie. Wezmę po prostu te kwiaty, mam te twoje króliki gdzieś. [Zabierz kwiaty i zostaw zwierzęta na pastwę losu]")
  (set `self.Odp 10.1` "[Odejdź]")
  (set `self.Odp 10.2` "Zawsze mam rację. [Odejdź]")
  (set `self.Odp 10.3` "Cieszę się, że mogłem pomóc [Odejdź]")
  (set `self.HeaderIndex` 0)
  (set `self.ArrayIndex` 0))